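; Test player character Blueprint with movement and camera input, altar-based respawn and a toggleable debug panel.
; Save point, position and level pass through the GameInstance interface, letting BeginPlay restore position and Respawn teleport or reload the saved level.
; CheckBehindDecor traces camera to mesh, using DoOnce-gated timelines to fade MPC_Occlusion parameters when "Decor"-tagged components block the view.
; ActiveAltar finds the nearest altar, but its activation call is disconnected.
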(event `InputAction|DebugInput`
  (params (Key :type "Key Structure"))
  (:`Pressed`
    (bind _isa (`/Engine/EditorBlueprintResources/StandardMacros.FlipFlop`)
      (:`A`
        _)
      (:`B`
        _))
    (`self.WidgetVisibility` (`/Game/BP/Widget/WBP_DebugPanel.B_Debug` (`self.DebugWidget`)) _isa)))

(event `self.ReceiveBeginPlay`
  (bind _returnvalue (`|CreateWidget` "/Game/BP/Widget/WBP_DebugPanel.WBP_DebugPanel_C" null self))
  (bind _output_get (set `self.DebugWidget` _returnvalue))
  (`UserWidget.AddToViewport` _output_get 0)
  (`self.SetupGameInstance`))

(event `Respawn`
  (bind _previous_level (`self.Previous Level`))
  (if (== _previous_level "None")
    (`/Engine/EditorBlueprintResources/StandardMacros.IsValid` (`self.LastSavePoint`) :!label _label
      (:`Is Valid`
        (`SceneComponent.K2_SetWorldLocation` (`self.CapsuleComponent`) (`self.RespawnPosition`) false true))
      (:`Is Not Valid`
        (`KismetSystemLibrary.PrintString` "No respawn Point Valid")))
    (else
      (bind _returnvalue (`GameplayStatics.GetCurrentLevelName` true))
      (if (`KismetStringLibrary.EqualEqual_StrStr` _returnvalue (`KismetStringLibrary.Conv_NameToString` _previous_level))
        (goto _label)
        (else
          (`GameplayStatics.OpenLevel` (`self.Previous Level`)))))))

(event `CheckBehindDecor`
  ;[1 1 1] CheckBehindDecor
  (bind _outhit (`KismetSystemLibrary.LineTraceSingle` (`SceneComponent.K2_GetComponentLocation` (`self.Camera`)) (`SceneComponent.K2_GetComponentLocation` (`self.Mesh`)) "TraceTypeQuery1"))
  (bind (_bblockinghit _binitialoverlap _time _distance _location _impactpoint _normal _impactnormal _physmat _hitactor _hitcomponent) (`GameplayStatics.BreakHitResult` _outhit))
  (if _bblockinghit
    (if (`ActorComponent.ComponentHasTag` _hitcomponent "Decor")
      (`KismetMaterialLibrary.SetScalarParameterValue` "/Game/Ressources/Materials/DissolveCam/MPC_Occlusion.MPC_Occlusion" "Collider?" 1.0)
      (`/Engine/EditorBlueprintResources/StandardMacros.DoOnce` false :!label _label_2
        (:`Completed`
          (bind (_direction _hardness) (`Timeline|FadeIn` :!via `PlayFromStart`)
            (:`Update`
              (`KismetMaterialLibrary.SetScalarParameterValue` "/Game/Ressources/Materials/DissolveCam/MPC_Occlusion.MPC_Occlusion" "hardness" _hardness))
            (:`Finished`
              (goto _label_3 :!via `Reset`))))))
    (else
      ;[1 1 1] Check si Deja Desactivé
      (bind _returnvalue (`KismetMaterialLibrary.GetScalarParameterValue` "/Game/Ressources/Materials/DissolveCam/MPC_Occlusion.MPC_Occlusion" "Collider?"))
      (if (not (== _returnvalue 0.0))
        (`/Engine/EditorBlueprintResources/StandardMacros.DoOnce` false :!label _label_3
          (:`Completed`
            (bind (_direction_2 _hardness_2 _collision) (`Timeline|FadeOut` :!via `PlayFromStart`)
              (:`Update`
                (`KismetMaterialLibrary.SetScalarParameterValue` "/Game/Ressources/Materials/DissolveCam/MPC_Occlusion.MPC_Occlusion" "Collider?" _collision)
                (`KismetMaterialLibrary.SetScalarParameterValue` "/Game/Ressources/Materials/DissolveCam/MPC_Occlusion.MPC_Occlusion" "hardness" _hardness_2))
              (:`Finished`
                (goto _label_2 :!via `Reset`)))))))))

(event `SaveAltar`
  (bind _returnvalue (`GameplayStatics.GetCurrentLevelName` true))
  (`/Game/BP/Data/BPI_PlayerInstance.SaveAltar` (`self.As BPI Player Instance`) (`KismetStringLibrary.Conv_StringToName` _returnvalue) (`self.RespawnPosition`) (`self.LastSavePoint`)))

(event `InputAxis|Vertical`
  (params (AxisValue :type "Float (single-precision)"))
  (bind (_returnvalue_roll _returnvalue_pitch _returnvalue_yaw) (`KismetMathLibrary.BreakRotator` (`self.GetControlRotation`)))
  ;[0 1 0.01606] Movement
  (`self.AddMovementInput` (`KismetMathLibrary.GetForwardVector` (`KismetMathLibrary.MakeRotator` 0.0 0.0 _returnvalue_yaw)) AxisValue))

(event `InputAxis|Turn`
  (params (AxisValue :type "Float (single-precision)"))
  ;[0 1 0.006503] Camera
  ;;[0.01644 1 0] Mousse
  (`self.AddControllerYawInput` AxisValue))

(event `InputAxis|TurnRate`
  (params (AxisValue :type "Float (single-precision)"))
  ;[0 1 0.006503] Camera
  ;;[0 1 0.04173] GamePad
  (`self.AddControllerYawInput` (* AxisValue (`self.baseTurnRate`) (`GameplayStatics.GetWorldDeltaSeconds`))))

(event `InputAxis|Horizontal`
  (params (AxisValue :type "Float (single-precision)"))
  (bind (_returnvalue_roll _returnvalue_pitch _returnvalue_yaw) (`KismetMathLibrary.BreakRotator` (`self.GetControlRotation`)))
  ;[0 1 0.01606] Movement
  (`self.AddMovementInput` (`KismetMathLibrary.GetRightVector` (`KismetMathLibrary.MakeRotator` 0.0 0.0 _returnvalue_yaw)) AxisValue))

(event `InputAxis|LookUp`
  (params (AxisValue :type "Float (single-precision)"))
  ;[0 1 0.006503] Camera
  ;;[0.01644 1 0] Mousse
  (`self.AddControllerPitchInput` AxisValue))

(event `InputAxis|LookUpRate`
  (params (AxisValue :type "Float (single-precision)"))
  ;[0 1 0.006503] Camera
  ;;[0 1 0.04173] GamePad
  (`self.AddControllerPitchInput` (* AxisValue (`self.baseLookUpRate`) (`GameplayStatics.GetWorldDeltaSeconds`))))

(fn `ActiveAltar`
  (bind _closestaltar (`self.closestAltar`))
  (bind _outactors (`GameplayStatics.GetAllActorsOfClassWithTag` "/Game/BP/World/BP_SaveAltar.BP_SaveAltar_C" "Altar"))
  (for _array_element _outactors
    (`/Engine/EditorBlueprintResources/StandardMacros.IsValid` _closestaltar
      (:`Is Valid`
        (if (< (`self.GetDistanceTo` _array_element self) (`self.GetDistanceTo` _closestaltar self))
          (set `self.closestAltar` _array_element :!label _label)))
      (:`Is Not Valid`
        (goto _label))))
  (`/Engine/EditorBlueprintResources/StandardMacros.IsValid` (`self.closestAltar`)))

(fn `SetupGameInstance`
  (bind _as_bpi_player_instance (`self.As BPI Player Instance`))
  (bind _asbpi_player_instance (cast `/Game/BP/Data/BPI_PlayerInstance` (`GameplayStatics.GetGameInstance`)))
  (set `self.As BPI Player Instance` _asbpi_player_instance)
  (set `self.RespawnPosition` (`/Game/BP/Data/BPI_PlayerInstance.savePosition` _as_bpi_player_instance))
  (set `self.LastSavePoint` (`/Game/BP/Data/BPI_PlayerInstance.ActiveAltar` _as_bpi_player_instance))
  (bind _output_get (set `self.Previous Level` (`/Game/BP/Data/BPI_PlayerInstance.PreviousLevel` _as_bpi_player_instance)))
  (bind _returnvalue (`GameplayStatics.GetCurrentLevelName` true))
  (if (== _output_get (`KismetStringLibrary.Conv_StringToName` _returnvalue))
    (`SceneComponent.K2_SetWorldLocation` (`self.CapsuleComponent`) (`self.RespawnPosition`) false true)
    (`self.ActiveAltar`)))

(fn `UserConstructionScript`)

(fn `WidgetVisibility`
  (params (Target :type "Widget Object Reference") (Show :type Boolean))
  (bind _returnvalue (`GameplayStatics.GetPlayerController` 0))
  (if Show
    (`Widget.SetVisibility` Target "Visible")
    (`WidgetBlueprintLibrary.SetInputMode_GameAndUIEx` _returnvalue null "DoNotLock" false)
    (set `PlayerController.bShowMouseCursor` true _returnvalue)
    (else
      (`Widget.SetVisibility` Target "Hidden")
      (`WidgetBlueprintLibrary.SetInputMode_GameOnly` _returnvalue)
      (set `PlayerController.bShowMouseCursor` false _returnvalue))))