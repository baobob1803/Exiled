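; BP_VFX_PlayerSpawn is the player spawn effect, driving a Niagara system and the MPC_CharacterSpawn material parameter collection.
; On BeginPlay it registers as the Niagara export callback and runs the Particle timeline into Amount2.
; When the first exported particle's Velocity and Position values lie within a small distance, it deactivates Niagara once and runs the Player timeline into Amount1.
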(event `self.ReceiveBeginPlay`
  (`NiagaraComponent.SetVariableObject` (`self.Niagara`) "CallBack" self)
  (bind (_direction _newtrack_0) (`Timeline|Particle` :!via `PlayFromStart`)
    (:`Update`
      (`KismetMaterialLibrary.SetScalarParameterValue` "/Game/Ressources/Materials/PlayerSpawn/MPC_CharacterSpawn.MPC_CharacterSpawn" "Amount2" _newtrack_0))))

(event `self.ReceiveParticleData`
  (params (Data :type "Array of BasicParticleData Structure (by ref)") (NiagaraSystem :type "NiagaraSystem Object Reference"))
  (bind (_position _size _velocity) (break `BasicParticleData` (`|GetArrayItem` Data)))
  (if (<= (`KismetMathLibrary.VSize` (- _velocity _position)) 30.0)
    (`/Engine/EditorBlueprintResources/StandardMacros.DoOnce` false
      (:`Completed`
        (`ActorComponent.Deactivate` (`self.Niagara`))
        (bind (_direction _newtrack_0) (`Timeline|Player` :!via `PlayFromStart`)
          (:`Update`
            (`KismetMaterialLibrary.SetScalarParameterValue` "/Game/Ressources/Materials/PlayerSpawn/MPC_CharacterSpawn.MPC_CharacterSpawn" "Amount1" _newtrack_0)))))))

(fn `UserConstructionScript`)