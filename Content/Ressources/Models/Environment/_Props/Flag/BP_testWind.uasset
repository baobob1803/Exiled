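; BP_testWind is a test Blueprint in the flag prop folder that varies a referenced wind source at runtime to produce gusty, changing wind.
; From BeginPlay, WindRandomizer loops by calling itself after a short random delay, picking a new random strength and speed each pass.
; WindEffect applies both values directly to the WindSourceRef component, so changes are abrupt steps with no interpolation.
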(event `self.ReceiveBeginPlay`
  (`self.WindRandomizer`))

(event `WindRandomizer`
  (`KismetSystemLibrary.Delay` (`KismetMathLibrary.RandomFloatInRange` 0.2 1.5))
  (set `self.wStrength` (`KismetMathLibrary.RandomFloatInRange` 0.2 3.0))
  (set `self.wSpeed` (`KismetMathLibrary.RandomFloatInRange` 0.2 0.8))
  (`self.WindEffect`)
  (`self.WindRandomizer`))

(event `WindEffect`
  (`WindDirectionalSourceComponent.SetStrength` (`WindDirectionalSource.Component` (`self.windSourceRef`)) (`self.wStrength`))
  (`WindDirectionalSourceComponent.SetSpeed` (`WindDirectionalSource.Component` (`self.windSourceRef`)) (`self.wSpeed`)))

(fn `UserConstructionScript`)