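; BP_IntroCinematic is an actor that runs the game's intro cinematic at BeginPlay, if the GameInstance and its EnableCinematic flag allow it.
; It adds the intro widget to the viewport, hides the player's HUD after a short delay, then creates and starts a Level Sequence player.
; TextEvent passes a text index to the widget for display and prints it for debugging.
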(event `self.ReceiveBeginPlay`
  (bind _value (message `/Game/BP/Interface/BPI_Save.GetShowCinematic` (`GameplayStatics.GetGameInstance`)))
  (if (and _value (`self.enable cinematic`))
    (bind _returnvalue (`GameplayStatics.GetActorOfClass` "/Game/BP/Character/Player/BP_MasterPlayer.BP_MasterPlayer_C"))
    (set `self.Player` _returnvalue)
    (bind _returnvalue_2 (`|CreateWidget` "/Game/BP/Widget/Cinematic/WBP_IntroCinematicTest.WBP_IntroCinematicTest_C"))
    (`UserWidget.AddToViewport` _returnvalue_2 0)
    (set `self.IntroWidgetRef` _returnvalue_2)
    (`KismetSystemLibrary.Delay` 0.1)
    (`Widget.SetVisibility` (`/Game/BP/Character/Player/BP_MasterPlayer.HUD` (`self.Player`)) "Hidden")
    (`self.StartIntroCinematic`)))

(event `StartIntroCinematic`
  (bind _outactor (`LevelSequencePlayer.CreateLevelSequencePlayer` "/Game/Ressources/Cinematique/IntroCinematic/Sequencer_IntroCinematic_First.Sequencer_IntroCinematic_First" (make `MovieSceneSequencePlaybackSettings` false (struct) -1.0)))
  (`MovieSceneSequencePlayer.PlayTo` :`self` (`LevelSequenceActor.SequencePlayer` _outactor)))

(event `TextEvent`
  (params (TextIndex :type Integer))
  (`/Game/BP/Widget/Cinematic/WBP_IntroCinematicTest.DisplayText` (`self.IntroWidgetRef`) TextIndex)
  (`KismetSystemLibrary.PrintString` (`KismetStringLibrary.Conv_IntToString` TextIndex)))

(fn `UserConstructionScript`)