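; BP_MasterIA is an AI-controlled character that acts as the body for an AIC_IAController and carries a patrol route.
; On BeginPlay it registers itself with the controller and copies its stats component's values into it.
; Damage and targeting events forward to the controller, while getters expose patrol marks with end-of-route reversal, AI state and mesh data.
; A state-to-material switch for visual feedback exists but is disconnected.
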(event `self.ReceiveBeginPlay`
  (bind _asaic_iacontroller (cast `/Game/BP/Character/IA/AIC_IAController` (`AIBlueprintHelperLibrary.GetAIController` self)))
  (bind _output_get (set `self.As AIC IAController` _asaic_iacontroller))
  (set `/Game/BP/Character/IA/AIC_IAController.As BP Master IA` self _output_get)
  (set `/Game/BP/ActorComponent/AC_IAStats.stats` (`/Game/BP/ActorComponent/AC_IAStats.stats` (`self.AC_IAStats`)) (`/Game/BP/Character/IA/AIC_IAController.AC_IAStats` (`self.As AIC IAController`))))

(event `self.ReceiveTick`
  (params (DeltaSeconds :type "Float (single-precision)")))

(event `/Game/BP/Interface/BPI_IAHelper.GetDamage`
  (params (Value :type "Float (single-precision)"))
  (`/Game/BP/Character/IA/AIC_IAController.GetDamage` (`self.As AIC IAController`) Value))

(event `/Game/BP/Interface/BPI_IAHelper.SetIsTargeted`
  (params (Targeted :type Boolean))
  (bind _output_get (set `/Game/BP/Character/IA/AIC_IAController.IsTargeted` Targeted (`self.As AIC IAController`)))
  (`KismetSystemLibrary.PrintString` (`KismetStringLibrary.Concat_StrStr` (`KismetSystemLibrary.GetDisplayName` self) " : " (`KismetStringLibrary.Conv_BoolToString` _output_get))))

(fn `Get Mesh World Rotation`
  (returns (Rotation :type "Rotator Structure"))
  (return (`SceneComponent.K2_GetComponentRotation` (`self.Mesh`))))

(fn `GetAIStates`
  (returns (`Current State` :type "/Game/BP/Enum/E_IAStates Enum"))
  (return (`/Game/BP/Character/IA/AIC_IAController.CurrentState` (`self.As AIC IAController`))))

(fn `GetMesh`
  (returns (Mesh :type "SkeletalMeshComponent Object Reference"))
  (return (`self.Mesh`)))

(fn `GetNextPatrolMark`
  (params (CurrentPatrolMark :type Integer) (reversed :type Boolean))
  (returns (Output :type "/Game/BP/World/BP_PatrolMark Object Reference") (reverse :type Boolean))
  (bind _patrolroute (`self.PatrolRoute`))
  (bind _output (`|GetArrayItem` _patrolroute CurrentPatrolMark))
  (if (>= CurrentPatrolMark (- (`KismetArrayLibrary.Array_Length` _patrolroute) 1))
    (return _output true)
    (elif (== CurrentPatrolMark 0)
      (return _output false)
      (else
        (return _output reversed)))))

(fn `UserConstructionScript`)