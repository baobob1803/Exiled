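; Player puzzle-mode actor for dragging runes into slots on a RunicReceptacle, using mouse or gamepad.
; Press traces under the mouse or stick-driven CursorTest, spawning a draggable BP_Rune from a hit rune or clearing a hit slot.
; Tick moves the held rune to the trace impact; release writes its info to TargetChildActor if set, destroys it and updates the receptacle key.
; Exit keys call ReturnToChara on the receptacle.
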(event `self.ReceiveTick`
  (params (DeltaSeconds :type "Float (single-precision)"))
  (bind _returnvalue (`SceneComponent.K2_GetComponentLocation` (`self.Cursor Test`)))
  (bind (_worldlocation _worlddirection) (`PlayerController.DeprojectMousePositionToWorld` (`GameplayStatics.GetPlayerController` 0)))
  (bind _returnvalue_2 (`SceneComponent.K2_GetComponentLocation` (`self.Camera`)))
  (bind _rune (`self.Rune`)
    (:`then`
      (bind _outhit (`KismetSystemLibrary.LineTraceSingle` (select `bool` (`self.inputGamepad`) :`false` _worldlocation :`true` _returnvalue_2) (select `bool` (`self.inputGamepad`) :`false` (+ _worldlocation (* _worlddirection 150.0)) :`true` (+ (* (- _returnvalue _returnvalue_2) 150.0) _returnvalue)) "TraceTypeQuery1" false (`|MakeArray` _rune :!type "Actor Object Reference")))
      (bind (_bblockinghit _binitialoverlap _time _distance _location _impactpoint) (`GameplayStatics.BreakHitResult` _outhit))
      (`self.K2_SetActorLocation` (`self.Rune`) (`KismetMathLibrary.MakeVector` (.x _impactpoint) (.y _impactpoint) (+ (.z _impactpoint) 0.0)) false false))
    (:`else`)))

(event `Key|LeftMouseButton`
  (params (Key :type "Key Structure"))
  (bind (_worldlocation _worlddirection) (`PlayerController.DeprojectMousePositionToWorld` (`GameplayStatics.GetPlayerController` 0)))
  (bind _returnvalue (`SceneComponent.K2_GetComponentLocation` (`self.Cursor Test`)))
  (:`Pressed`
    (set `PlayerController.bShowMouseCursor` true (`GameplayStatics.GetPlayerController` 0) :!label _label)
    (bind _returnvalue_2 (`KismetInputLibrary.Key_IsGamepadKey` (stale `Key|Gamepad_FaceButton_Bottom` Key)))
    (set `self.inputGamepad` _returnvalue_2)
    (bind _outhit (`KismetSystemLibrary.LineTraceSingle` :`Start` (select `bool` _returnvalue_2 :`false` _worldlocation :`true` (`SceneComponent.K2_GetComponentLocation` (`self.Camera`))) :`End` (select `bool` _returnvalue_2 :`false` (+ _worldlocation (* _worlddirection 150.0)) :`true` (+ (* (- _returnvalue (`SceneComponent.K2_GetComponentLocation` (`self.Camera`))) 150.0) _returnvalue)) :`TraceChannel` "TraceTypeQuery1" :`DrawDebugType` "ForDuration"))
    (bind (_bblockinghit _binitialoverlap _time _distance _location _impactpoint _normal _impactnormal _physmat _hitactor _hitcomponent) (`GameplayStatics.BreakHitResult` _outhit))
    (if _bblockinghit
      (`|ExecutionSequence`
        (:`then_0`
          (if (`self.ActorHasTag` _hitactor "RuneInteract")
            (bind _key (message `/Game/BP/Interface/BPI_PuzzleRune.GetKey` _hitactor))
            (`/Game/BP/World/PuzzleOracle/BP_RunicReceptacle.SetRuneVisibility` (`self.RunicReceptacle`) _key true false)
            (bind _runeinfo (message `/Game/BP/Interface/BPI_PuzzleRune.GetRuneInfo` _hitactor))
            (bind (_returnvalue_x _returnvalue_y _returnvalue_z) (`KismetMathLibrary.BreakVector` (`SceneComponent.K2_GetComponentLocation` _hitcomponent)))
            (bind _returnvalue_3 (`|SpawnActorFromClass` "/Game/BP/World/PuzzleOracle/BP_Rune.BP_Rune_C" (`KismetMathLibrary.MakeTransform` (`KismetMathLibrary.MakeVector` _returnvalue_x _returnvalue_y (- _returnvalue_z 50.0))) "Undefined" "OverrideRootScale" null _runeinfo null))
            (set `self.Rune` _returnvalue_3)))
        (:`then_1`
          (if (`self.ActorHasTag` _hitactor "Slot")
            (bind _key_2 (message `/Game/BP/Interface/BPI_PuzzleRune.GetKey` _hitactor))
            (`/Game/BP/World/PuzzleOracle/BP_RunicReceptacle.SetRuneVisibility` (`self.RunicReceptacle`) _key_2 false true)
            (message `/Game/BP/Interface/BPI_PuzzleRune.ResetRuneInfo` _hitactor)
            (message `/Game/BP/Interface/BPI_PuzzleRune.UpdateMaterial` _hitactor))))))
  (:`Released`
    (`|ExecutionSequence` :!label _label_2
      (:`then_0`
        (bind _targetchildactor (`self.targetChildActor`)
          (:`then`
            (bind _childactor (`ChildActorComponent.ChildActor` _targetchildactor))
            (bind _key_3 (message `/Game/BP/Interface/BPI_PuzzleRune.GetKey` _childactor))
            (`/Game/BP/World/PuzzleOracle/BP_RunicReceptacle.SetRuneVisibility` (`self.RunicReceptacle`) _key_3 false true)
            (message `/Game/BP/Interface/BPI_PuzzleRune.SetRuneInfo` _childactor (`/Game/BP/World/PuzzleOracle/BP_Rune.RuneInfo` (`self.Rune`)))
            (message `/Game/BP/Interface/BPI_PuzzleRune.UpdateMaterial` _childactor)
            (set `self.targetChildActor` null))
          (:`else`
            (bind _key_4 (message `/Game/BP/Interface/BPI_PuzzleRune.GetKey` (`self.Rune`)))
            (`/Game/BP/World/PuzzleOracle/BP_RunicReceptacle.SetRuneVisibility` (`self.RunicReceptacle`) _key_4 false true))))
      (:`then_1`
        (`self.K2_DestroyActor` (`self.Rune`))
        (set `self.Rune` null)
        (`/Game/BP/World/PuzzleOracle/BP_RunicReceptacle.UpdateKey` (`self.RunicReceptacle`))))))

(event `Key|Gamepad_FaceButton_Bottom`
  (params (Key :type "Key Structure"))
  (:`Pressed`
    (goto _label))
  (:`Released`
    (goto _label_2)))

(event `Key|Z`
  (params (Key :type "Key Structure"))
  (:`Pressed`
    (`/Game/BP/World/PuzzleOracle/BP_RunicReceptacle.ReturnToChara` (`self.RunicReceptacle`) :!label _label_3)))

(event `Key|Q`
  (params (Key :type "Key Structure"))
  (:`Pressed`
    (goto _label_3)))

(event `Key|S`
  (params (Key :type "Key Structure"))
  (:`Pressed`
    (goto _label_3)))

(event `Key|D`
  (params (Key :type "Key Structure"))
  (:`Pressed`
    (goto _label_3)))

(event `Key|Gamepad_FaceButton_Right`
  (params (Key :type "Key Structure"))
  (:`Pressed`
    (goto _label_3)))

(event `InputAxisKey|Gamepad_LeftX`
  (params (AxisValue :type "Float (single-precision)"))
  (`SceneComponent.K2_SetWorldLocation` (`self.Cursor Test`) (+ (* (`self.GetActorRightVector`) (* 1 AxisValue)) (`SceneComponent.K2_GetComponentLocation` (`self.Cursor Test`))) false false))

(event `InputAxis|Horizontal`
  (params (AxisValue :type "Float (single-precision)")))

(event `InputAxisKey|Gamepad_LeftY`
  (params (AxisValue :type "Float (single-precision)"))
  (`SceneComponent.K2_SetWorldLocation` (`self.Cursor Test`) (+ (* (`self.GetActorUpVector`) (* 1 AxisValue)) (`SceneComponent.K2_GetComponentLocation` (`self.Cursor Test`))) false false))

(event `InputAxis|Vertical`
  (params (AxisValue :type "Float (single-precision)")))

(fn `UserConstructionScript`)