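; Master player character Blueprint with a third-person lock-on camera, sprint, dodge, and save-altar respawn.
; Lock-on picks tagged actors in LockZone by camera angle, switches by stick direction, and a looping timer keeps spring arm and mesh facing the target.
; The Sprint input dodges while locked, otherwise timelines blend speed and arm length.
; Health comes from ACStats, and the game instance stores altar save position and level for respawn.
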(event `ResetCamera`
  (bind _charactermovement (`self.CharacterMovement`))
  ;[0 1 0] Lock
  ;;[0 1 0] ResetCam
  (`KismetSystemLibrary.K2_PauseTimerHandle` (`self.camRotateEvent`))
  (set `self.actualTarget` null)
  (`Controller.SetControlRotation` (`GameplayStatics.GetPlayerController` 0) (`SceneComponent.K2_GetComponentRotation` (`self.SpringArm`)))
  (`SceneComponent.K2_SetWorldRotation` (`self.CapsuleComponent`) (`SceneComponent.K2_GetComponentRotation` (`self.Mesh`)) false false)
  (`SceneComponent.K2_SetWorldRotation` (`self.Mesh`) (`SceneComponent.K2_GetComponentRotation` (`self.CapsuleComponent`)) false false)
  (set `SpringArmComponent.bUsePawnControlRotation` true (`self.SpringArm`))
  (`self.TakeAwayCam`)
  (set `self.bUseControllerRotationYaw` false)
  (set `CharacterMovementComponent.bOrientRotationToMovement` true _charactermovement)
  (set `CharacterMovementComponent.bUseControllerDesiredRotation` true _charactermovement))

(event `HangOutCam`
  ;[0 1 0] Lock
  ;;[0 1 0] TimeLineTraveling
  (bind (_direction _lerp_0_1) (`Timeline|Traveling` :!label _label)
    (:`Update`
      (set `SpringArmComponent.TargetArmLength` (`KismetMathLibrary.Lerp` 275.0 200.0 _lerp_0_1) (`self.SpringArm`))
      (`CameraComponent.SetFieldOfView` (`self.Camera`) (`KismetMathLibrary.Lerp` 90.0 80.0 _lerp_0_1)))))

(event `InputAction|Lock`
  (params (Key :type "Key Structure"))
  ;[0 1 0] Lock
  ;;[0 1 0] LockInput
  (:`Pressed`
    (`self.actualTarget`
      (:`then`
        (`self.ResetCamera`))
      (:`else`
        (if (>= (`KismetArrayLibrary.Array_Length` (`self.targetInRange`)) 1)
          (`self.SelectTarget` 0.0)
          (`self.actualTarget`
            (:`then`
              (`self.SwitchTarget`)
              (set `SpringArmComponent.bUsePawnControlRotation` false (`self.SpringArm`))
              (`self.TBlockRotMesh`)
              (`self.HangOutCam`))
            (:`else`)))))))

(event `TakeAwayCam`
  ;[0 1 0] Lock
  ;;[0 1 0] TimeLineTraveling
  (goto _label :!via `Reverse`))

(event `SwitchTarget`
  (bind _camrotateevent (`self.camRotateEvent`))
  ;[0 1 0] Lock
  ;;[0 1 0] SwitchTarget
  (`|ExecutionSequence`
    (:`then_0`
      (if (not (`KismetSystemLibrary.K2_IsTimerPausedHandle` _camrotateevent))
        (`KismetSystemLibrary.K2_PauseTimerHandle` _camrotateevent)))
    (:`then_1`
      (set `self.initCamRotation` (`SceneComponent.K2_GetComponentRotation` (`self.Camera`)))
      (set `self.initMeshRotation` (`SceneComponent.K2_GetComponentRotation` (`self.Mesh`)))
      (bind (_direction _lerp) (`Timeline|switch` :!via `PlayFromStart`)
        (:`Update`
          (`self.actualTarget`
            (:`then`
              (`SceneComponent.K2_SetWorldRotation` (`self.SpringArm`) (`|EaseFunction` "CircularOut" _lerp (`self.initCamRotation`) (`KismetMathLibrary.FindLookAtRotation` (`SceneComponent.K2_GetComponentLocation` (`self.SpringArm`)) (`self.K2_GetActorLocation` (`self.actualTarget`)))) false false)
              (`SceneComponent.K2_SetWorldRotation` (`self.Mesh`) (`KismetMathLibrary.MakeRotator` 0.0 0.0 (.yaw (`|EaseFunction` "CircularOut" _lerp (`self.initMeshRotation`) (`KismetMathLibrary.FindLookAtRotation` (`SceneComponent.K2_GetComponentLocation` (`self.Mesh`)) (`self.K2_GetActorLocation` (`self.actualTarget`)))))) false false))
            (:`else`)))
        (:`Finished`
          (`KismetSystemLibrary.K2_UnPauseTimerHandle` (`self.camRotateEvent`)))))))

(event `TBlockRotMesh`
  (bind _charactermovement (`self.CharacterMovement`))
  ;[0 1 0] Lock
  (set `self.bUseControllerRotationYaw` true)
  (set `CharacterMovementComponent.bOrientRotationToMovement` false _charactermovement)
  (set `CharacterMovementComponent.bUseControllerDesiredRotation` true _charactermovement))

(event `self.LockZone.OnComponentBeginOverlap`
  (params (OverlappedComponent :type "PrimitiveComponent Object Reference") (OtherActor :type "Actor Object Reference") (OtherComp :type "PrimitiveComponent Object Reference") (OtherBodyIndex :type Integer) (bFromSweep :type Boolean) (SweepResult :type "HitResult Structure (by ref)"))
  ;[0 1 0] Lock
  ;;[0 1 0] Add A new target to the array
  (if (!= OtherActor self)
    (for _array_element (`Actor.Tags` OtherActor)
      (if (== _array_element "Target")
        (`KismetArrayLibrary.Array_Add` (`self.targetInRange`) OtherActor)
        (break)))))

(event `self.LockZone.OnComponentEndOverlap`
  (params (OverlappedComponent :type "PrimitiveComponent Object Reference") (OtherActor :type "Actor Object Reference") (OtherComp :type "PrimitiveComponent Object Reference") (OtherBodyIndex :type Integer))
  ;[0 1 0] Lock
  ;;[0 1 0] Remove a target from the array
  (if (!= OtherActor self)
    (for _array_element (`Actor.Tags` OtherActor)
      (if (and (== _array_element "Target") (!= (`KismetArrayLibrary.Array_Find` (`self.targetInRange`) OtherActor) -1))
        (`KismetArrayLibrary.Array_RemoveItem` (`self.targetInRange`) OtherActor)
        (if (== (`self.actualTarget`) OtherActor)
          (`self.ResetCamera`)
          (break))))))

(event `/Game/BP/BPI_Stats.UpdateHealth`
  (params (Value :type "Float (single-precision)"))
  (bind ((`health_28_F233DD9E4E1A7496AF43D784D6E1E722` _health)) (break `/Game/BP/ST_Stats` (`/Game/BP/AC_Stats.stats` (`self.AC_Stats`))))
  (`/Game/BP/AC_Stats.StatsBehaviour` (`self.AC_Stats`) "NewEnumerator0" Value)
  (`KismetSystemLibrary.PrintString` (`KismetStringLibrary.Conv_DoubleToString` _health))
  (if (<= _health 0.0)
    (`self.Respawn`)))

(event `InputAction|DebugInput`
  (params (Key :type "Key Structure"))
  (:`Pressed`
    (bind _isa (`/Engine/EditorBlueprintResources/StandardMacros.FlipFlop`)
      (:`A`
        _)
      (:`B`
        _))
    (`self.WidgetVisibility` (`/Game/BP/Widget/WBP_DebugPanel.B_Debug` (`self.DebugWidget`)) _isa)))

(event `self.ReceiveBeginPlay`
  (bind _returnvalue (`|CreateWidget` "/Game/BP/Widget/WBP_DebugPanel.WBP_DebugPanel_C" null self))
  (bind _output_get (set `self.DebugWidget` _returnvalue))
  (`UserWidget.AddToViewport` _output_get 0)
  (`self.SetupGameInstance`)
  (bind _returnvalue_2 (`KismetSystemLibrary.K2_SetTimer` null "RotateCamera" 0.008333 true))
  (bind _output_get_2 (set `self.camRotateEvent` _returnvalue_2))
  (`KismetSystemLibrary.K2_PauseTimerHandle` _output_get_2)
  (set `CharacterMovementComponent.MaxWalkSpeed` (`.walkSpeed_31_326818EC43BFC962EA0ADCA66ED62FFC` (break `/Game/BP/ST_Stats` (`/Game/BP/AC_Stats.stats` (`self.AC_Stats`)))) (`self.CharacterMovement`))
  (`/Game/BP/AC_Stats.StatsBehaviour` (`self.AC_Stats`) "NewEnumerator5" 0.0))

(event `Respawn`
  (bind _previous_level (`self.Previous Level`))
  (bind _ac_stats (`self.AC_Stats`))
  (if (== _previous_level "None")
    (`/Engine/EditorBlueprintResources/StandardMacros.IsValid` (`self.LastSavePoint`) :!label _label_2
      (:`Is Valid`
        (`SceneComponent.K2_SetWorldLocation` (`self.CapsuleComponent`) (`self.RespawnPosition`) false true)
        (`/Game/BP/AC_Stats.StatsBehaviour` _ac_stats "NewEnumerator0" (`.maxHealth_29_A0B28AD744A6E2962FC9578F2703DB58` (break `/Game/BP/ST_Stats` (`/Game/BP/AC_Stats.stats` _ac_stats)))))
      (:`Is Not Valid`
        (`KismetSystemLibrary.PrintString` "No respawn Point Valid")))
    (else
      (bind _returnvalue (`GameplayStatics.GetCurrentLevelName` true))
      (if (`KismetStringLibrary.EqualEqual_StrStr` _returnvalue (`KismetStringLibrary.Conv_NameToString` _previous_level))
        (goto _label_2)
        (else
          (`GameplayStatics.OpenLevel` (`self.Previous Level`)))))))

(event `SaveAltar`
  (bind _returnvalue (`GameplayStatics.GetCurrentLevelName` true))
  (`/Game/BP/Data/BPI_PlayerInstance.SaveAltar` (`self.As BPI Player Instance`) (`KismetStringLibrary.Conv_StringToName` _returnvalue) (`self.RespawnPosition`) (`self.LastSavePoint`)))

(event `InputAxis|Vertical`
  (params (AxisValue :type "Float (single-precision)"))
  (bind (_returnvalue_roll _returnvalue_pitch _returnvalue_yaw) (`KismetMathLibrary.BreakRotator` (select `bool` (`KismetSystemLibrary.IsValid` (`self.actualTarget`)) :`false` (`self.GetControlRotation`) :`true` (`SceneComponent.K2_GetComponentRotation` (`self.Camera`)))))
  ;[0 1 0] Movement
  (`self.AddMovementInput` (`KismetMathLibrary.GetForwardVector` (`KismetMathLibrary.MakeRotator` 0.0 0.0 _returnvalue_yaw)) AxisValue))

(event `InputAxis|LookUpRate`
  (params (AxisValue :type "Float (single-precision)"))
  ;[0 1 0] Camera
  ;;[0 1 0] GamePad
  (`self.AddControllerPitchInput` (* AxisValue (`self.baseLookUpRate`) (`GameplayStatics.GetWorldDeltaSeconds`))))

(event `InputAxis|Turn`
  (params (AxisValue :type "Float (single-precision)"))
  ;[0 1 0] Camera
  ;;[0 1 0] Mousse
  (`self.actualTarget`
    (:`then`)
    (:`else`
      (`self.AddControllerYawInput` AxisValue))))

(event `InputAxis|TurnRate`
  (params (AxisValue :type "Float (single-precision)"))
  ;[0 1 0] Camera
  ;;[0 1 0] GamePad
  (`self.actualTarget`
    (:`then`
      ;[0 1 0] ChangeTarget
      (if (`KismetMathLibrary.InRange_FloatFloat` AxisValue -0.6 0.6)
        (`/Engine/EditorBlueprintResources/StandardMacros.DoOnce` false :!label _label
          (:`Completed`
            (goto _label_2 :!via `Reset`)))
        (else
          (`/Engine/EditorBlueprintResources/StandardMacros.DoOnce` false :!label _label_2
            (:`Completed`
              (`self.SelectTarget` AxisValue)
              (`self.SwitchTarget`)
              (goto _label :!via `Reset`))))))
    (:`else`
      (`self.AddControllerYawInput` (* AxisValue (`self.baseTurnRate`) (`GameplayStatics.GetWorldDeltaSeconds`))))))

(event `InputAxis|Horizontal`
  (params (AxisValue :type "Float (single-precision)"))
  (bind (_returnvalue_roll _returnvalue_pitch _returnvalue_yaw) (`KismetMathLibrary.BreakRotator` (select `bool` (`KismetSystemLibrary.IsValid` (`self.actualTarget`)) :`false` (`self.GetControlRotation`) :`true` (`SceneComponent.K2_GetComponentRotation` (`self.Camera`)))))
  ;[0 1 0] Movement
  (`self.AddMovementInput` (`KismetMathLibrary.GetRightVector` (`KismetMathLibrary.MakeRotator` 0.0 0.0 _returnvalue_yaw)) AxisValue))

(event `InputAxis|LookUp`
  (params (AxisValue :type "Float (single-precision)"))
  ;[0 1 0] Camera
  ;;[0 1 0] Mousse
  (`self.AddControllerPitchInput` AxisValue))

(event `InputAxis|ChangeTarget`
  (params (AxisValue :type "Float (single-precision)"))
  ;[0 1 0] ChangeTarget
  (`self.actualTarget`
    (:`then`
      (if (`KismetMathLibrary.InRange_FloatFloat` AxisValue -0.6 0.6)
        (`/Engine/EditorBlueprintResources/StandardMacros.DoOnce` false :!label _label_3
          (:`Completed`
            (goto _label_4 :!via `Reset`)))
        (else
          (`/Engine/EditorBlueprintResources/StandardMacros.DoOnce` false :!label _label_4
            (:`Completed`
              (`self.SelectTarget` AxisValue)
              (`self.SwitchTarget`)
              (goto _label_3 :!via `Reset`))))))
    (:`else`)))

(event `Dodge`
  ;[0 1 0] Sprint / Dodge
  ;;[0 1 0] Dodge
  (set `self.isDodging` true)
  (set `CharacterMovementComponent.MaxWalkSpeed` (* 0.0 (`.walkSpeed_31_326818EC43BFC962EA0ADCA66ED62FFC` (break `/Game/BP/ST_Stats` (`/Game/BP/AC_Stats.stats` (`self.AC_Stats`))))) (`self.CharacterMovement`))
  (`KismetSystemLibrary.Delay` 0.3)
  (`self.PlayAnimMontage` null)
  (`self.DodgeCD`)
  (set `CharacterMovementComponent.MaxWalkSpeed` (`.walkSpeed_31_326818EC43BFC962EA0ADCA66ED62FFC` (break `/Game/BP/ST_Stats` (`/Game/BP/AC_Stats.stats` (`self.AC_Stats`)))) (`self.CharacterMovement`)))

(event `InputAction|Sprint`
  (params (Key :type "Key Structure"))
  ;[0 1 0] Sprint / Dodge
  ;;[0 1 0] Input
  (:`Pressed`
    (`self.actualTarget`
      (:`then`
        (if (not (`self.isDodging`))
          (`self.Dodge`)))
      (:`else`
        (`self.Sprint`))))
  (:`Released`
    (`self.actualTarget`
      (:`then`)
      (:`else`
        (`self.StopSprint`)))))

(event `DodgeCD`
  ;[0 1 0] Sprint / Dodge
  ;;[0 1 0] DodgeCD
  (`KismetSystemLibrary.Delay` 1.0)
  (set `self.isDodging` false))

(event `Sprint`
  (bind _deceleration (`self.deceleration`))
  (bind ((`walkSpeed_31_326818EC43BFC962EA0ADCA66ED62FFC` _walkspeed) (`speedSprint_27_7BA06322413550B5D6CC468C262A3F9B` _speedsprint)) (break `/Game/BP/ST_Stats` (`/Game/BP/AC_Stats.stats` (`self.AC_Stats`))))
  ;[0 1 0] Sprint / Dodge
  ;;[0 1 0] Sprint
  ;;;[0 1 0] Start Sprint
  (set `self.isSprinting` true)
  (`TimelineComponent.Stop` _deceleration)
  (`TimelineComponent.SetPlaybackPosition` (`self.acceleration`) (* (`TimelineComponent.GetPlaybackPosition` _deceleration) 3.0) false true)
  (bind (_direction _lerp) (`Timeline|acceleration`)
    (:`Update`
      (bind _output_get (set `CharacterMovementComponent.MaxWalkSpeed` (`KismetMathLibrary.Lerp` _walkspeed _speedsprint _lerp) (`self.CharacterMovement`)))
      (set `SpringArmComponent.TargetArmLength` (`KismetMathLibrary.Lerp` 275.0 350.0 _lerp) (`self.SpringArm`))
      (`KismetSystemLibrary.PrintString` (`KismetStringLibrary.Conv_DoubleToString` _output_get) true true (struct :`G` 1.0 :`B` 0.033423 :`A` 1.0) 10.0))))

(event `StopSprint`
  (bind _acceleration (`self.acceleration`))
  (bind ((`walkSpeed_31_326818EC43BFC962EA0ADCA66ED62FFC` _walkspeed) (`speedSprint_27_7BA06322413550B5D6CC468C262A3F9B` _speedsprint)) (break `/Game/BP/ST_Stats` (`/Game/BP/AC_Stats.stats` (`self.AC_Stats`))))
  ;[0 1 0] Sprint / Dodge
  ;;[0 1 0] Sprint
  ;;;[0 1 0] Stop Sprint
  (set `self.isSprinting` false)
  (`TimelineComponent.Stop` _acceleration)
  (`TimelineComponent.SetPlaybackPosition` (`self.deceleration`) (/ (`TimelineComponent.GetPlaybackPosition` _acceleration) 3.0) false true)
  (bind (_direction _lerp) (`Timeline|deceleration` :!via `Reverse`)
    (:`Update`
      (bind _output_get (set `CharacterMovementComponent.MaxWalkSpeed` (`KismetMathLibrary.Lerp` _walkspeed _speedsprint _lerp) (`self.CharacterMovement`)))
      (set `SpringArmComponent.TargetArmLength` (`KismetMathLibrary.Lerp` 275.0 350.0 _lerp) (`self.SpringArm`))
      (`KismetSystemLibrary.PrintString` (`KismetStringLibrary.Conv_DoubleToString` _output_get) true true (struct :`R` 1.0 :`G` 0.09287 :`A` 1.0) 10.0))))

(fn `ActiveAltar`
  (bind _closestaltar (`self.closestAltar`))
  (bind _closestaltar_2 (`self.closestAltar`))
  (bind _outactors (`GameplayStatics.GetAllActorsOfClassWithTag` "/Game/BP/World/BP_SaveAltar.BP_SaveAltar_C" "Altar"))
  (for _array_element _outactors
    (`/Engine/EditorBlueprintResources/StandardMacros.IsValid` _closestaltar
      (:`Is Valid`
        (if (< (`self.GetDistanceTo` _array_element self) (`self.GetDistanceTo` _closestaltar self))
          (set `self.closestAltar` _array_element :!label _label)))
      (:`Is Not Valid`
        (goto _label))))
  (`/Engine/EditorBlueprintResources/StandardMacros.IsValid` _closestaltar_2
    (:`Is Valid`
      (`/Game/BP/World/BP_SaveAltar.SetActivation` _closestaltar_2 self))))

(fn `RotateCamera`
  (bind (_returnvalue_roll _returnvalue_pitch _returnvalue_yaw) (`KismetMathLibrary.BreakRotator` (`KismetMathLibrary.FindLookAtRotation` (`SceneComponent.K2_GetComponentLocation` (`self.Mesh`)) (`self.K2_GetActorLocation` (`self.actualTarget`)))))
  (bind (_returnvalue_roll_2 _returnvalue_pitch_2 _returnvalue_yaw_2) (`KismetMathLibrary.BreakRotator` (`KismetMathLibrary.FindLookAtRotation` (`SceneComponent.K2_GetComponentLocation` (`self.SpringArm`)) (`self.K2_GetActorLocation` (`self.actualTarget`)))))
  (`self.actualTarget`
    (:`then`
      (`SceneComponent.K2_SetWorldRotation` (`self.SpringArm`) (`KismetMathLibrary.MakeRotator` _returnvalue_roll_2 _returnvalue_pitch_2 _returnvalue_yaw_2) false false)
      (`SceneComponent.K2_SetWorldRotation` (`self.Mesh`) (`KismetMathLibrary.MakeRotator` 0.0 0.0 _returnvalue_yaw) false false))
    (:`else`)))

(fn `SelectTarget`
  (params (InputDirection :type "Float (double-precision)"))
  (locals (L_closeTargetAngle :type "Map of Float (double-precision) to Actor Object Reference") (L_lastEnemy :type "Actor Object Reference") (L_farTargetAngle :type "Map of Float (double-precision) to Actor Object Reference") (L_actualElement :type "Actor Object Reference") (L_actualDistance :type "Float (double-precision)" :default 0.0) (L_actualAngle :type "Float (double-precision)" :default 0.0) (L_inputDirection :type "Float (double-precision)"))
  (bind _returnvalue (`self.GetDistanceTo` (`local.L_lastEnemy`) (`local.L_actualElement`)))
  (bind _returnvalue_2 (`KismetMathLibrary.Vector_Distance` (+ (`self.K2_GetActorLocation` (`local.L_lastEnemy`)) (`SceneComponent.GetRightVector` (`self.Camera`))) (`self.K2_GetActorLocation` (`local.L_actualElement`))))
  (set `local.L_inputDirection` InputDirection)
  (`self.actualTarget`
    (:`then`
      ;[0 1 0] Lock is already active. So, you switch the target
      (set `local.L_lastEnemy` (`self.actualTarget`))
      (for _array_element (`self.targetInRange`)
        (bind _output_get (set `local.L_actualElement` _array_element))
        (if (!= _output_get (`local.L_lastEnemy`))
          (bind _returnvalue_3 (`self.CheckAngle` (`local.L_actualElement`) 64.0)
            (:`inCone`
              (set `local.L_actualAngle` _returnvalue_3)
              (if (and (< _returnvalue _returnvalue_2) (<= (`local.L_inputDirection`) -0.6))
                (`BlueprintMapLibrary.Map_Add` (`local.L_closeTargetAngle`) (`local.L_actualAngle`) (`local.L_actualElement`))
                (elif (and (> _returnvalue _returnvalue_2) (>= (`local.L_inputDirection`) 0.6))
                  (`BlueprintMapLibrary.Map_Add` (`local.L_closeTargetAngle`) (`local.L_actualAngle`) (`local.L_actualElement`))))))))
      (bind _values (`BlueprintMapLibrary.Map_Values` (`local.L_closeTargetAngle`)))
      (if (> (`KismetArrayLibrary.Array_Length` _values) 0)
        (bind _keys (`BlueprintMapLibrary.Map_Keys` (`local.L_closeTargetAngle`)))
        (set `self.actualTarget` (`BlueprintMapLibrary.Map_Find` (`local.L_closeTargetAngle`) (`.MinValue` (`KismetMathLibrary.MinOfFloatArray` _keys))))))
    (:`else`
      ;[0 1 0] Lock Is Inactive
      (for _array_element_2 (`self.targetInRange`)
        (set `local.L_actualElement` _array_element_2)
        (bind _outhit (`KismetSystemLibrary.LineTraceSingle` :`Start` (`self.K2_GetActorLocation`) :`End` (`self.K2_GetActorLocation` (`local.L_actualElement`)) :`TraceChannel` "TraceTypeQuery1" :`DrawDebugType` "ForDuration"))
        (if (== (`.HitActor` (`GameplayStatics.BreakHitResult` _outhit)) (`local.L_actualElement`))
          (bind _returnvalue_4 (`self.CheckAngle` (`local.L_actualElement`) 65.0)
            (:`inCone`
              (set `local.L_actualAngle` _returnvalue_4)
              (if (< (`self.GetDistanceTo` (`local.L_actualElement`)) 250.0)
                (`BlueprintMapLibrary.Map_Add` (`local.L_closeTargetAngle`) (`local.L_actualAngle`) (`local.L_actualElement`))
                (else
                  (`BlueprintMapLibrary.Map_Add` (`local.L_farTargetAngle`) (`local.L_actualAngle`) (`local.L_actualElement`))))))))
      (bind _values_2 (`BlueprintMapLibrary.Map_Values` (`local.L_closeTargetAngle`)))
      (if (> (`KismetArrayLibrary.Array_Length` _values_2) 0)
        (bind _keys_2 (`BlueprintMapLibrary.Map_Keys` (`local.L_closeTargetAngle`)))
        (set `self.actualTarget` (`BlueprintMapLibrary.Map_Find` (`local.L_closeTargetAngle`) (`.MinValue` (`KismetMathLibrary.MinOfFloatArray` _keys_2))))
        (else
          (bind _values_3 (`BlueprintMapLibrary.Map_Values` (`local.L_farTargetAngle`)))
          (if (> (`KismetArrayLibrary.Array_Length` _values_3) 0)
            (bind _keys_3 (`BlueprintMapLibrary.Map_Keys` (`local.L_farTargetAngle`)))
            (set `self.actualTarget` (`BlueprintMapLibrary.Map_Find` (`local.L_farTargetAngle`) (`.MinValue` (`KismetMathLibrary.MinOfFloatArray` _keys_3))))))))))

(fn `SetupGameInstance`
  (bind _as_bpi_player_instance (`self.As BPI Player Instance`))
  (bind _asbpi_player_instance (cast `/Game/BP/Data/BPI_PlayerInstance` (`GameplayStatics.GetGameInstance`)))
  (set `self.As BPI Player Instance` _asbpi_player_instance)
  (set `self.RespawnPosition` (`/Game/BP/Data/BPI_PlayerInstance.savePosition` _as_bpi_player_instance))
  (set `self.LastSavePoint` (`/Game/BP/Data/BPI_PlayerInstance.ActiveAltar` _as_bpi_player_instance))
  (bind _output_get (set `self.Previous Level` (`/Game/BP/Data/BPI_PlayerInstance.PreviousLevel` _as_bpi_player_instance)))
  (bind _returnvalue (`GameplayStatics.GetCurrentLevelName` true))
  (if (== _output_get (`KismetStringLibrary.Conv_StringToName` _returnvalue))
    (`SceneComponent.K2_SetWorldLocation` (`self.CapsuleComponent`) (`self.RespawnPosition`) false true)
    (`self.ActiveAltar`)))

(fn `UserConstructionScript`)

(fn `WidgetVisibility`
  (params (Target :type "Widget Object Reference") (Show :type Boolean))
  (bind _returnvalue (`GameplayStatics.GetPlayerController` 0))
  (if Show
    (`Widget.SetVisibility` Target "Visible")
    (`WidgetBlueprintLibrary.SetInputMode_GameAndUIEx` _returnvalue null "DoNotLock" false)
    (set `PlayerController.bShowMouseCursor` true _returnvalue)
    (else
      (`Widget.SetVisibility` Target "Hidden")
      (`WidgetBlueprintLibrary.SetInputMode_GameOnly` _returnvalue)
      (set `PlayerController.bShowMouseCursor` false _returnvalue))))