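; Boss character that tracks the player and picks attacks by distance band.
; A looping timer sets the range enum, writes it to the Blackboard and toggles a yaw-only look-at timer.
; A second timer randomly picks force-pulse projectile or backstep at Close, teleport or lunge at Long; other ranges have no attack.
; Backstep and lunge pause timers during Timeline moves; their traces only print hits, and the mirrored-movement helper's result is unused.
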(event `self.ReceiveBeginPlay`
  (bind _returnvalue (`GameplayStatics.GetActorOfClass` "/Game/BP/Character/Player/BP_MasterPlayer.BP_MasterPlayer_C"))
  (set `self.Player` _returnvalue)
  (bind _returnvalue_2 (`KismetSystemLibrary.K2_SetTimerDelegate` (delegate `get distance from player`) 0.1 true))
  (set `self.TH_CheckDistance` _returnvalue_2)
  (bind _returnvalue_3 (`KismetSystemLibrary.K2_SetTimer` null "AttackManager" 2.0 true))
  (set `self.TH_AttackManager` _returnvalue_3)
  (`BlackboardComponent.SetValueAsEnum` (`AIBlueprintHelperLibrary.GetBlackboard` null) "Current Range" (`self.CurrentRange`)))

(event `get distance from player`
  (bind _currentrange (`self.CurrentRange`))
  (bind _keys (`BlueprintMapLibrary.Map_Keys` (`self.Range`)))
  (for (_array_element _array_index) _keys
    (if (< (`self.GetDistanceTo` (`self.Player`) self) _array_element)
      (bind _values (`BlueprintMapLibrary.Map_Values` (`self.Range`)))
      (set `self.CurrentRange` (`|GetArrayItem` _values _array_index))
      (break)
      (else
        (set `self.CurrentRange` "NewEnumerator4"))))
  (`BlackboardComponent.SetValueAsEnum` (`AIBlueprintHelperLibrary.GetBlackboard` null) "Current Range" _currentrange)
  (`KismetSystemLibrary.PrintString` (`|GetEnumeratorNameAsString` _currentrange))
  (switch `/Game/BP/Enum/E_BossRange` (`self.CurrentRange`)
    (:`NewEnumerator0`
      (`self.look at player in range` :!label _label))
    (:`NewEnumerator1`
      (goto _label))
    (:`NewEnumerator2`
      (goto _label))
    (:`NewEnumerator3`
      (goto _label))
    (:`NewEnumerator4`
      (`KismetSystemLibrary.K2_PauseTimerHandle` (`self.TH_Look at Player`))
      (set `self.midPoint Set` false))))

(event `look at player in range`
  (bind _th_look_at_player (`self.TH_Look at Player`))
  (if (`KismetSystemLibrary.K2_IsValidTimerHandle` _th_look_at_player)
    (if (not (`KismetSystemLibrary.K2_IsTimerActiveHandle` _th_look_at_player))
      (bind _returnvalue (`KismetSystemLibrary.K2_SetTimer` null "Look at Player" 0.01 true :!label _label_2))
      (set `self.TH_Look at Player` _returnvalue))
    (else
      (goto _label_2))))

(event `Offensive BackStep`
  (bind _returnvalue (`self.K2_GetActorLocation`))
  (bind _returnvalue_2 (`self.K2_GetActorLocation`))
  ;[1 1 1] Close Range Attack 2
  (`KismetSystemLibrary.K2_PauseTimerHandle` (`self.TH_CheckDistance`))
  (`KismetSystemLibrary.K2_PauseTimerHandle` (`self.TH_Look at Player`))
  (set `self.midPoint Set` false)
  (bind (_outhit _returnvalue_3) (`KismetSystemLibrary.SphereTraceSingle` :`Start` _returnvalue :`End` (+ (* (`self.GetActorForwardVector`) 100.0) _returnvalue) :`Radius` 10.0 :`TraceChannel` "TraceTypeQuery2" :`DrawDebugType` "ForDuration"))
  (if _returnvalue_3
    (`KismetSystemLibrary.PrintString` (`KismetSystemLibrary.GetDisplayName` (`.HitActor` (`GameplayStatics.BreakHitResult` _outhit))))
    (bind (_direction _newtrack_1) (`Timeline|BackStep` :!via `PlayFromStart` :!label _label_3)
      (:`Update`
        (`self.K2_SetActorLocation` (`KismetMathLibrary.VLerp` _returnvalue_2 (+ (* (`self.GetActorForwardVector`) -50.0) _returnvalue_2) _newtrack_1)))
      (:`Finished`
        (`KismetSystemLibrary.K2_UnPauseTimerHandle` (`self.TH_CheckDistance`))))
    (else
      (goto _label_3 :!via `PlayFromStart`))))

(event `Lunge Forward`
  (bind _returnvalue (`self.K2_GetActorLocation`))
  (`KismetSystemLibrary.K2_PauseTimerHandle` (`self.TH_CheckDistance`))
  (`KismetSystemLibrary.K2_PauseTimerHandle` (`self.TH_AttackManager`))
  (`KismetSystemLibrary.K2_PauseTimerHandle` (`self.TH_Look at Player`))
  (set `self.midPoint Set` false)
  (set `self.StartDashPosition` (`self.K2_GetActorLocation`))
  (set `self.distance to player` (`self.GetDistanceTo` (`self.Player`)))
  (`BlueprintMapLibrary.Map_Keys` (`self.Range`))
  (bind (_direction _alpha) (`Timeline|TL_Dash` :!via `PlayFromStart`)
    (:`Update`
      (`self.K2_SetActorLocation` (`KismetMathLibrary.VLerp` (`self.StartDashPosition`) (+ (* (`self.GetActorForwardVector`) (`self.distance to player`)) (`self.StartDashPosition`)) _alpha))
      (bind (_outhit _returnvalue_2) (`KismetSystemLibrary.LineTraceSingle` :`Start` _returnvalue :`End` (+ (* (`self.GetActorForwardVector`) 100.0) _returnvalue) :`TraceChannel` "TraceTypeQuery2" :`DrawDebugType` "ForDuration"))
      (if _returnvalue_2
        (`KismetSystemLibrary.PrintString` (`KismetSystemLibrary.GetDisplayName` (`.HitActor` (`GameplayStatics.BreakHitResult` _outhit))))))
    (:`Finished`
      (`KismetSystemLibrary.Delay` 2.0)
      (`KismetSystemLibrary.K2_UnPauseTimerHandle` (`self.TH_Look at Player`))
      (`KismetSystemLibrary.K2_UnPauseTimerHandle` (`self.TH_CheckDistance`))
      (bind _returnvalue_3 (`KismetSystemLibrary.K2_SetTimer` null "AttackManager" 2.0 true))
      (set `self.TH_AttackManager` _returnvalue_3))))

(fn `AttackManager`
  (switch `/Game/BP/Enum/E_BossRange` (`self.CurrentRange`)
    (:`NewEnumerator0`
      (if (`KismetMathLibrary.RandomBool`)
        (`KismetSystemLibrary.PrintString` "Force Pulse")
        (`self.ForcePulse`)
        (else
          (`KismetSystemLibrary.PrintString` "Offiensive Backstep")
          (`self.Offensive BackStep`))))
    (:`NewEnumerator2`
      (if (`KismetMathLibrary.RandomBool`)
        (`KismetSystemLibrary.PrintString` "TP")
        (`self.Teleport`)
        (else
          (`KismetSystemLibrary.PrintString` "Lunge Forward")
          (`self.Lunge Forward`))))))

(fn `ForcePulse`
  (bind _returnvalue (`|SpawnActorFromClass` "/Game/BP/Character/Boss/BP_BossProjectile.BP_BossProjectile_C" (`KismetMathLibrary.MakeTransform` (+ (* (`self.GetActorForwardVector`) 50.0) (`self.K2_GetActorLocation`)) (struct) (0.5 0.5 0.5)) "Undefined" "OverrideRootScale" null (`self.Player`) self null))
  (`/Game/BP/Character/Boss/BP_BossProjectile.Throw` _returnvalue (* (`self.GetActorForwardVector`) 10000.0)))

(fn `Look at Player`
  (bind (_returnvalue_roll _returnvalue_pitch) (`KismetMathLibrary.BreakRotator` (`SceneComponent.K2_GetComponentRotation` (`self.CapsuleComponent`))))
  (bind (_returnvalue_roll_2 _returnvalue_pitch_2 _returnvalue_yaw) (`KismetMathLibrary.BreakRotator` (`KismetMathLibrary.FindLookAtRotation` (`SceneComponent.K2_GetComponentLocation` (`self.CapsuleComponent`)) (`self.K2_GetActorLocation` (`self.Player`)))))
  (`SceneComponent.K2_SetWorldRotation` (`self.CapsuleComponent`) (`KismetMathLibrary.MakeRotator` _returnvalue_roll _returnvalue_pitch _returnvalue_yaw) false false)
  (`self.Oppsite Movement`))

(fn `Oppsite Movement`
  (returns (Destination :type "Vector Structure"))
  (bind (_returnvalue_x _returnvalue_y _returnvalue_z) (`KismetMathLibrary.BreakVector` (`self.K2_GetActorLocation`)))
  (bind (_midlepoint_x _midlepoint_y) (`KismetMathLibrary.BreakVector` (`self.MidlePoint`)))
  (bind (_returnvalue_x_2 _returnvalue_y_2) (`KismetMathLibrary.BreakVector` (`self.K2_GetActorLocation` (`self.Player`))))
  (bind _returnvalue (`self.K2_GetActorLocation` (`self.Player`)))
  (bind (_returnvalue_x_3 _returnvalue_y_3 _returnvalue_z_2) (`KismetMathLibrary.BreakVector` (+ (/ (- (`self.K2_GetActorLocation`) _returnvalue) 2.0) _returnvalue)))
  (if (`self.midPoint Set`)
    (return (`KismetMathLibrary.MakeVector` (- _midlepoint_x (- 0.0 (- _midlepoint_x _returnvalue_x_2))) (- _midlepoint_y (- 0.0 (- _midlepoint_y _returnvalue_y_2))) _returnvalue_z))
    (else
      (bind _output_get (set `self.MidlePoint` (`KismetMathLibrary.MakeVector` _returnvalue_x_3 _returnvalue_y_3 _returnvalue_z_2)))
      (set `self.midPoint Set` true)
      (return _output_get))))

(fn `Teleport`
  (bind _keys (`BlueprintMapLibrary.Map_Keys` (`self.Range`)))
  (`self.K2_SetActorLocation` (+ (* (`self.GetActorForwardVector`) (- (`self.GetDistanceTo` (`self.Player`)) (+ (`|GetArrayItem` _keys 1) -50.0))) (`self.K2_GetActorLocation`)))
  (set `self.midPoint Set` false))

(fn `UserConstructionScript`)