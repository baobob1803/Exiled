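; Boss projectile that is launched by a physics impulse and shoves the player on impact.
; Throw applies the given force to the Sphere, whose hit event reacts only to actors tagged Player.
; A timeline then repeatedly lerps the Player from its current location along the Launcher's forward vector without sweeping, so the push accumulates per update.
; The projectile destroys itself when the timeline finishes.
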(event `self.ReceiveBeginPlay`)

(event `Throw`
  (params (Force :type "Vector Structure"))
  (`PrimitiveComponent.AddImpulse` (`self.Sphere`) Force "None" false))

(event `self.Sphere.OnComponentHit`
  (params (HitComponent :type "PrimitiveComponent Object Reference") (OtherActor :type "Actor Object Reference") (OtherComp :type "PrimitiveComponent Object Reference") (NormalImpulse :type "Vector Structure") (Hit :type "HitResult Structure (by ref)"))
  (bind _returnvalue (`self.K2_GetActorLocation` (`self.Player`)))
  (if (`self.ActorHasTag` OtherActor "Player")
    ;[1 1 1] Add In Player
    (bind (_direction _newtrack_0) (`Timeline|Player Throw` :!via `PlayFromStart`)
      (:`Update`
        (`self.K2_SetActorLocation` (`self.Player`) (`KismetMathLibrary.VLerp` _returnvalue (+ _returnvalue (* (`self.GetActorForwardVector` (`self.Launcher`)) 50.0)) _newtrack_0) false false))
      (:`Finished`
        (`self.K2_DestroyActor`)))))

(fn `UserConstructionScript`)