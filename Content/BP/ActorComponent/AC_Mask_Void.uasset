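; Actor component for the Void mask, which isolates the player and their target in an abyss and boosts player power.
; Passive adds data-table damage at 30% health or below and starts a looping debug trace from the nearest save altar.
; Active teleports both to BP_Abyss, signals other AIs and adds damage.
; CancelVoid restores both transforms on timeout or death, delaying the power reset after a death.
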(event `self.OnEquipMask`
  (params (Player :type "/Game/BP/Character/Player/BP_MasterPlayer Object Reference"))
  (bind (_datatable _rowname) (break `DataTableRowHandle` (`self.maskInfo`)))
  (set `self.Player` Player)
  (`self.Passive` null)
  (bind _returnvalue (`|GetDataTableRow` _datatable _rowname)
    (:`then`
      (set `self.ST_Mask` _returnvalue))))

(event `Timer pass Close Altar`
  (bind _closest_altar (`self.GetClosestAltar`))
  (`KismetSystemLibrary.LineTraceSingle` :`Start` (`Actor.K2_GetActorLocation` _closest_altar) :`End` (`Actor.K2_GetActorLocation` (`self.Player`)) :`TraceChannel` "TraceTypeQuery1" :`DrawDebugType` "ForDuration" :`TraceColor` (struct :`R` 0.024998 :`G` 0.134644 :`B` 1.0 :`A` 1.0) :`TraceHitColor` (struct :`G` 0.044537 :`B` 1.0 :`A` 1.0) :`DrawTime` 1.0))

(event `self.Passive`
  (params (hitActor :type "Actor Object Reference"))
  (bind _health (message `/Game/BP/Interface/BPI_Stats.GetHealth` (`self.Player`)))
  (set `self.PlayerHealth` _health)
  (bind _maxhealth (message `/Game/BP/Interface/BPI_Stats.GetMaxHealth` (`self.Player`)))
  (set `self.Player Max Health` _maxhealth)
  (if (<= (/ (`self.PlayerHealth`) (`self.Player Max Health`)) 0.3)
    (message `/Game/BP/Interface/BPI_Stats.UpdatePower` (`self.Player`) (`.AdditionnalDamage_3_C14042B24355F4C4CB32BA9A7539E283` (break `/Game/BP/Structure/ST_Void` (`.Void_36_0F21BF43443E628937F894AF0C694F8C` (break `/Game/BP/Structure/ST_Mask` (`self.ST_Mask`))))))
    (bind _returnvalue (`KismetSystemLibrary.K2_SetTimerDelegate` (delegate `Timer pass Close Altar`) 0.1 true))
    (set `self.TH_Closest altar pass` _returnvalue)
    (else
      (`KismetSystemLibrary.K2_PauseTimerHandle` (`self.TH_Closest altar pass`)))))

(event `self.OnUnequipMask`
  (`KismetSystemLibrary.K2_PauseTimerHandle` (`self.TH_Closest altar pass`))
  (message `/Game/BP/Interface/BPI_Stats.UpdatePower` (`self.Player`) (- 0.0 (`.AdditionnalDamage_3_C14042B24355F4C4CB32BA9A7539E283` (break `/Game/BP/Structure/ST_Void` (`.Void_36_0F21BF43443E628937F894AF0C694F8C` (break `/Game/BP/Structure/ST_Mask` (`self.ST_Mask`))))))))

(event `self.Active`
  (params (useCooldown :type Boolean) (`Hud Ref` :type "/Game/BP/Widget/WBP_HUD Object Reference"))
  (if useCooldown
    (if (<= (`self.time`) 0.0)
      (bind _actualtarget (message `/Game/BP/Interface/BPI_PlayerAnim.GetActualTarget` (`self.Player`)))
      (`/Engine/EditorBlueprintResources/StandardMacros.IsValid` _actualtarget
        (:`Is Valid`
          (`parent.Cooldown` `Hud Ref`)
          (bind _outactors (`GameplayStatics.GetAllActorsOfClass` "/Game/BP/Character/IA/BP_MasterIA.BP_MasterIA_C"))
          (for _array_element _outactors
            (bind _actualtarget_2 (message `/Game/BP/Interface/BPI_PlayerAnim.GetActualTarget` (`self.Player`)))
            (if (== _array_element _actualtarget_2)
              (set `self.IA in Void` _actualtarget_2)
              (elif (not (== _array_element (`self.IA in Void`)))
                (message `/Game/BP/Interface/BPI_IAHelper.Trigger void Mask active` _array_element false)
                (bind _returnvalue (`KismetSystemLibrary.K2_SetTimerDelegate` (delegate `disable void`) (`.voidtime_6_0BA9E2D74FC9242242480982F1B5B1FB` (break `/Game/BP/Structure/ST_Void` (`.Void_36_0F21BF43443E628937F894AF0C694F8C` (break `/Game/BP/Structure/ST_Mask` (`self.ST_Mask`)))))))
                (set `self.TH_void` _returnvalue))))
          (`self.TP to Abyss`)
          (message `/Game/BP/Interface/BPI_Stats.UpdatePower` (`self.Player`) (`.AdditionnalDamage_3_C14042B24355F4C4CB32BA9A7539E283` (break `/Game/BP/Structure/ST_Void` (`.Void_36_0F21BF43443E628937F894AF0C694F8C` (break `/Game/BP/Structure/ST_Mask` (`self.ST_Mask`)))))))))))

(event `disable void`
  (`self.Cancel Void` false))

(fn `Cancel Void`
  (params (`With death` :type Boolean))
  (locals (`death?` :type Boolean))
  (bind _output_get (set `local.death?` `With death`))
  (if _output_get
    (`KismetSystemLibrary.K2_PauseTimerHandle` (`self.TH_void`)))
  (bind _outactors (`GameplayStatics.GetAllActorsOfClass` "/Game/BP/Character/IA/BP_MasterIA.BP_MasterIA_C"))
  (for _array_element _outactors
    (if (not (== (`self.IA in Void`) _array_element))
      (message `/Game/BP/Interface/BPI_IAHelper.Trigger void Mask active` _array_element false)))
  (`Actor.K2_SetActorTransform` (`self.Player`) (`self.Player Previous Transform`) false true)
  (bind _ia_in_void (`self.IA in Void`)
    (:`then`
      (`Actor.K2_SetActorTransform` _ia_in_void (`self.IA Previous transform`) false true)
      (bind _iacontroller (message `/Game/BP/Interface/BPI_IAHelper.get Controller` (`self.IA in Void`)))
      (`Controller.StopMovement` _iacontroller)
      (`/Game/BP/Character/IA/AIC_IAController.Change state` _iacontroller "NewEnumerator4")
      (set `/Game/BP/Character/IA/AIC_IAController.in void ?` false _iacontroller))
    (:`else`
      _))
  (set `self.IA in Void` null)
  (if (`local.death?`)
    (`KismetSystemLibrary.K2_SetTimer` null "Reset Player Power " (`.Poweraftervoidcooldown_9_A0940EB441DD2C964E691F8CDC347D43` (break `/Game/BP/Structure/ST_Void` (`.Void_36_0F21BF43443E628937F894AF0C694F8C` (break `/Game/BP/Structure/ST_Mask` (`self.ST_Mask`))))))
    (else
      (`/Game/BP/Interface/BPI_Stats.UpdatePower` (`self.Player`) (- 0.0 (`.AdditionnalDamage_3_C14042B24355F4C4CB32BA9A7539E283` (break `/Game/BP/Structure/ST_Void` (`.Void_36_0F21BF43443E628937F894AF0C694F8C` (break `/Game/BP/Structure/ST_Mask` (`self.ST_Mask`)))))))))
  (`KismetSystemLibrary.K2_PauseTimerHandle` (`self.TH_void`)))

(fn `GetClosestAltar`
  (returns (`closest Altar` :type "/Game/BP/World/BP_SaveAltar Object Reference"))
  (bind _outactors (`GameplayStatics.GetAllActorsOfClass` "/Game/BP/World/BP_SaveAltar.BP_SaveAltar_C"))
  (for _array_element _outactors
    (bind _closestaltar (`self.ClosestAltar`)
      (:`then`
        (if (< (`Actor.GetDistanceTo` _array_element (`self.Player`)) (`Actor.GetDistanceTo` _closestaltar (`self.Player`)))
          (set `self.ClosestAltar` _array_element)))
      (:`else`
        (set `self.ClosestAltar` _array_element))))
  (return (`self.ClosestAltar`)))

(fn `Reset Player Power `
  (`KismetSystemLibrary.PrintString` "End of Power Up")
  (`/Game/BP/Interface/BPI_Stats.UpdatePower` (`self.Player`) (- 0.0 (`.AdditionnalDamage_3_C14042B24355F4C4CB32BA9A7539E283` (break `/Game/BP/Structure/ST_Void` (`.Void_36_0F21BF43443E628937F894AF0C694F8C` (break `/Game/BP/Structure/ST_Mask` (`self.ST_Mask`))))))))

(fn `TP to Abyss`
  (bind _player (`self.Player`))
  (bind _ia_pos (`/Game/BP/World/BP_Abyss.IA pos` (`self.Abyss`)))
  (`self.Abyss`
    (:`then`
      _)
    (:`else`
      (bind _returnvalue (`GameplayStatics.GetActorOfClass` "/Game/BP/World/BP_Abyss.BP_Abyss_C"))
      (bind _output_get (set `self.Abyss` _returnvalue))))
  (set `self.Player Previous Transform` (`Actor.GetTransform` (`self.Player`)))
  (bind _player_pos (`/Game/BP/World/BP_Abyss.Player Pos` _output_get))
  (`Actor.K2_SetActorLocationAndRotation` _player (`SceneComponent.K2_GetComponentLocation` _player_pos) (`SceneComponent.K2_GetComponentRotation` _player_pos) false false)
  (`/Game/BP/Character/Player/BP_MasterPlayer.Lock in void` _player)
  (`SceneComponent.K2_SetRelativeRotation` :`self` (`/Game/BP/Character/Player/BP_MasterPlayer.Camera` _player))
  (set `self.IA Previous transform` (`Actor.GetTransform` (`self.IA in Void`)))
  (`Actor.K2_SetActorLocationAndRotation` (`self.IA in Void`) (`SceneComponent.K2_GetComponentLocation` _ia_pos) (`SceneComponent.K2_GetComponentRotation` _ia_pos) false false)
  (bind _iacontroller (message `/Game/BP/Interface/BPI_IAHelper.get Controller` (`self.IA in Void`)))
  (`/Game/BP/Character/IA/AIC_IAController.UpdateBattleHandler` _iacontroller true)
  (`Controller.StopMovement` _iacontroller)
  (`/Game/BP/Character/IA/AIC_IAController.Change state` _iacontroller "NewEnumerator4")
  (set `/Game/BP/Character/IA/AIC_IAController.in void ?` true _iacontroller))