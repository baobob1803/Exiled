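; Mask ability component for Matter that switches its owner between a life-steal stance and a life-sacrifice boost stance.
; Active, gated by the cooldown Timer when requested, flips the passive trigger between OnHitEnemy and OnAttack and sends that stance's power multiplier.
; Passive applies the matching health change, or resets power to 1 if an attack sacrifice would deplete health.
; Equipping runs Active without cooldown; unequipping restores neutral state.
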(event `self.Active`
  (params (useCooldown :type Boolean))
  ;[1 1 1] Active
  (if useCooldown
    (if (<= (`self.timer`) 0.0)
      (`parent.Active` false)
      (set `self.typePassive` (select `/Game/BP/Enum/ETypePassive` (`self.typePassive`) :`NewEnumerator0` "NewEnumerator1" :`NewEnumerator1` "NewEnumerator4" :`NewEnumerator2` "NewEnumerator4" :`NewEnumerator4` "NewEnumerator1" :!type "/Game/BP/Enum/ETypePassive Enum") :!label _label)
      (message `/Game/BP/Interface/BPI_Stats.UpdatePower` (`self.GetOwner`) (select `/Game/BP/Enum/ETypePassive` (`self.typePassive`) :`NewEnumerator0` 1.0 :`NewEnumerator1` (`self.multiplierOnLifeSteal`) :`NewEnumerator2` 1.0 :`NewEnumerator4` (`self.multiplierOnBoost`))))
    (else
      (goto _label))))

(event `self.Passive`
  ;[1 1 1] Passive
  (bind _health (message `/Game/BP/Interface/BPI_Stats.GetHealth` (`self.GetOwner`)))
  (if (or (> (+ _health (`self.lifeSacrifice`)) 0.0) (`|EnumEquality` (`self.typePassive`) "NewEnumerator1"))
    (message `/Game/BP/Interface/BPI_Stats.UpdateHealth` (`self.GetOwner`) (select `/Game/BP/Enum/ETypePassive` (`self.typePassive`) :`NewEnumerator1` (`self.lifeSteal`) :`NewEnumerator4` (`self.lifeSacrifice`)) false)
    (else
      (message `/Game/BP/Interface/BPI_Stats.UpdatePower` (`self.GetOwner`) 1.0))))

(event `self.OnEquipMask`
  ;[1 1 1] Ekip
  (`self.Active` false))

(event `self.OnUnequipMask`
  ;[1 1 1] UnEkip
  (set `self.typePassive` "NewEnumerator0")
  (message `/Game/BP/Interface/BPI_Stats.UpdatePower` (`self.GetOwner`) 1.0))