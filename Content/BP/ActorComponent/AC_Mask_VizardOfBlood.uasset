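; Vizard of Blood mask component that toggles the owner between life steal on hit and health sacrifice for boosted attacks.
; Active switches TypePassive, gated by cooldown except on equip, and sets that mode's power multiplier from the mask's DataTable row.
; Passive applies the mode's health change, or resets power to 1 when sacrifice would deplete health.
; Unequipping restores default mode and power.
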(event `self.Passive`
  (params (hitActor :type "Actor Object Reference"))
  (bind (_datatable _rowname) (break `DataTableRowHandle` (`self.maskInfo`)))
  ;[1 1 1] Passive
  (bind _health (message `/Game/BP/Interface/BPI_Stats.GetHealth` (`self.GetOwner`)))
  (bind _returnvalue (`|GetDataTableRow` _datatable _rowname)
    (:`then`
      (bind ((`lifeSteal_2_0E77C6634A16D475C9B9A7B893E8D0AF` _lifesteal) (`lifeSacrifice_6_F6E1E3944A088342004271BC4E1E53DF` _lifesacrifice)) (break `/Game/BP/Structure/ST_Vizard` (`.Vizard_19_27B1B7B8403C54F3765C0BBB98617216` (break `/Game/BP/Structure/ST_Mask` _returnvalue))))
      (if (or (> (+ _health _lifesacrifice) 0.0) (`|EnumEquality` (`self.typePassive`) "NewEnumerator1"))
        (message `/Game/BP/Interface/BPI_Stats.UpdateHealth` (`self.GetOwner`) (select `/Game/BP/Enum/ETypePassive` (`self.typePassive`) :`NewEnumerator1` _lifesteal :`NewEnumerator4` _lifesacrifice) false)
        (else
          (message `/Game/BP/Interface/BPI_Stats.UpdatePower` (`self.GetOwner`) 1.0))))))

(event `self.OnEquipMask`
  (params (Player :type "/Game/BP/Character/Player/BP_MasterPlayer Object Reference"))
  ;[1 1 1] Ekip
  (`self.Active` false))

(event `self.OnUnequipMask`
  ;[1 1 1] UnEkip
  (set `self.typePassive` "NewEnumerator0")
  (message `/Game/BP/Interface/BPI_Stats.UpdatePower` (`self.GetOwner`) 1.0))

(event `self.Active`
  (params (useCooldown :type Boolean) (`Hud Ref` :type "/Game/BP/Widget/WBP_HUD Object Reference"))
  (bind (_datatable _rowname) (break `DataTableRowHandle` (`self.maskInfo`)))
  ;[1 1 1] Active
  (if useCooldown
    (if (<= (`self.time`) 0.0)
      (`parent.Cooldown` `Hud Ref`)
      (set `self.typePassive` (select `/Game/BP/Enum/ETypePassive` (`self.typePassive`) :`NewEnumerator0` "NewEnumerator1" :`NewEnumerator1` "NewEnumerator4" :`NewEnumerator2` "NewEnumerator4" :`NewEnumerator4` "NewEnumerator1" :`NewEnumerator5` "NewEnumerator0" :!type "/Game/BP/Enum/ETypePassive Enum") :!label _label)
      (bind _returnvalue (`|GetDataTableRow` _datatable _rowname)
        (:`then`
          (bind ((`multiplierOnLifeSteal_7_7AE5A3DF43FFC8DBDD1C5294156DD222` _multiplieronlifesteal) (`multiplierOnBoost_8_6D02EADB4E3EF74192C02AA5A12FDD6B` _multiplieronboost)) (break `/Game/BP/Structure/ST_Vizard` (`.Vizard_19_27B1B7B8403C54F3765C0BBB98617216` (break `/Game/BP/Structure/ST_Mask` _returnvalue))))
          (message `/Game/BP/Interface/BPI_Stats.UpdatePower` (`self.GetOwner`) (select `/Game/BP/Enum/ETypePassive` (`self.typePassive`) :`NewEnumerator0` 1.0 :`NewEnumerator1` _multiplieronlifesteal :`NewEnumerator2` 1.0 :`NewEnumerator4` _multiplieronboost)))))
    (else
      (goto _label))))