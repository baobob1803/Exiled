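; Base actor component for masks, with empty Passive, Active, equip and unequip events plus a shared active-ability cooldown.
; Cooldown stores the HUD reference, reads the duration from the mask's data table row and starts or unpauses a looping timer.
; Each ActiveCooldown tick decrements the remaining time and updates the HUD, then at zero pauses the timer and calls ResetActiveMessage on the owner.
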(event `Passive`
  (params (hitActor :type "Actor Object Reference")))

(event `Active`
  (params (useCooldown :type Boolean) (`Hud Ref` :type "/Game/BP/Widget/WBP_HUD Object Reference")))

(event `Cooldown`
  (params (hudRef :type "/Game/BP/Widget/WBP_HUD Object Reference"))
  (bind (_datatable _rowname) (break `DataTableRowHandle` (`self.maskInfo`)))
  (set `self.Hud Ref` hudRef)
  (bind _returnvalue (`|GetDataTableRow` _datatable _rowname)
    (:`then`
      (set `self.time` (`.cooldown_7_931E1E894A548774E6BBFC81BB6BAE5B` (break `/Game/BP/Structure/ST_Mask` _returnvalue)))
      (if (`KismetSystemLibrary.K2_IsValidTimerHandle` (`self.cooldownTimerHandler`))
        (`KismetSystemLibrary.K2_UnPauseTimerHandle` (`self.cooldownTimerHandler`))
        (else
          (bind _returnvalue_2 (`KismetSystemLibrary.K2_SetTimer` null "ActiveCooldown" (`self.refreshTimerValue`) true))
          (set `self.cooldownTimerHandler` _returnvalue_2))))))

(event `OnUnequipMask`)

(event `OnEquipMask`
  (params (Player :type "/Game/BP/Character/Player/BP_MasterPlayer Object Reference")))

(fn `ActiveCooldown`
  (bind (_datatable _rowname) (break `DataTableRowHandle` (`self.maskInfo`)))
  (bind _output_get (set `self.time` (- (`self.time`) (`self.refreshTimerValue`))))
  (bind _returnvalue (`|GetDataTableRow` _datatable _rowname)
    (:`then`
      (bind ((`Model_45_3234E68B486017BF8E1AD79EA7DC5996` _model) (`cooldown_7_931E1E894A548774E6BBFC81BB6BAE5B` _cooldown) (`mask_33_BC673CA1426A6C8F23DFCEA3D029F2E2` _mask)) (break `/Game/BP/Structure/ST_Mask` _returnvalue))
      (`/Game/BP/Widget/WBP_HUD.UpdateActiveCD` (`self.Hud Ref`) _output_get _cooldown _mask)
      (if (<= _output_get 0.0)
        (`KismetSystemLibrary.K2_PauseTimerHandle` (`self.cooldownTimerHandler`))
        (message `/Game/BP/Interface/BPI_Mask.resetActive` (`self.GetOwner`))))))