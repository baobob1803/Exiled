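; Mask component for the Veil of Visions, which places mind marks on AI enemies and triggers them through an event dispatcher.
; Depending on the passive type, a hit either adds timed marks and binds the AI controller, or broadcasts a fear range scaled by its mark count.
; The active ability starts the parent cooldown and broadcasts mark damage, with tuning read from a DataTable.
; Equipping selects the marking passive; unequipping notifies listeners.
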(event `self.Active`
  (params (useCooldown :type Boolean) (`Hud Ref` :type "/Game/BP/Widget/WBP_HUD Object Reference"))
  (bind (_datatable _rowname) (break `DataTableRowHandle` (`self.maskInfo`)))
  (if (<= (`self.time`) 0.0)
    (`parent.Cooldown` `Hud Ref`)
    (bind _returnvalue (`|GetDataTableRow` _datatable _rowname)
      (:`then`
        (`self.ED_UseMarks` true (`.markDamage_11_80D14EEE4E418351031CB9BE3DB46EE8` (break `/Game/BP/Structure/ST_Veil` (`.Veil_22_0838F7C84E80820E3C97E29BF725196A` (break `/Game/BP/Structure/ST_Mask` _returnvalue)))))
        (`KismetSystemLibrary.PrintString` "ALED")))))

(event `self.Passive`
  (params (hitActor :type "Actor Object Reference"))
  (bind _returnvalue (`AIBlueprintHelperLibrary.GetAIController` hitActor))
  (bind (_datatable _rowname) (break `DataTableRowHandle` (`self.maskInfo`)))
  (bind _returnvalue_2 (`|GetDataTableRow` _datatable _rowname)
    (:`then`
      (if (`|EnumEquality` (`self.typePassive`) "NewEnumerator1")
        (bind _asaic_iacontroller (cast `/Game/BP/Character/IA/AIC_IAController` _returnvalue))
        (bind ((`rangeMultiplicator_5_F65294B04EC368ADBD1B529CBCA90985` _rangemultiplicator) (`marksLifetime_7_6D89112E4D6817FBF622F5ABFE2F9DD3` _markslifetime) (`fearTime_10_0AF661DB444F57A18A85859070E0D153` _feartime)) (break `/Game/BP/Structure/ST_Veil` (`.Veil_22_0838F7C84E80820E3C97E29BF725196A` (break `/Game/BP/Structure/ST_Mask` _returnvalue_2))))
        (`/Game/BP/Character/IA/AIC_IAController.AddMarks` _asaic_iacontroller _markslifetime)
        (`/Game/BP/Character/IA/AIC_IAController.bindEvent` _asaic_iacontroller self)
        (else
          (bind _asaic_iacontroller_2 (cast `/Game/BP/Character/IA/AIC_IAController` _returnvalue))
          (`self.ED_UseMarks` false 0.0 _asaic_iacontroller_2 false (* (`/Game/BP/Character/IA/AIC_IAController.nbMindMarks` _asaic_iacontroller_2) (* 1000 _rangemultiplicator)) _feartime)
          (`KismetSystemLibrary.PrintString` "use Marks" true true (struct :`R` 1.0 :`G` 0.07511 :`A` 1.0) 20.0))))))

(event `self.OnEquipMask`
  (set `self.typePassive` "NewEnumerator1"))

(event `self.OnUnequipMask`
  (`self.ED_UseMarks` false 0.0 null true))