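; AC_IAStats is an actor component that holds a Stats struct with Health, Dodge Ratio, Block Ratio and Battle Score.
; SetStat switches on a stat enum and writes the given value to the matching struct field.
; UpdateStat uses the same switch but writes the given value plus one, without reading the field's current value.
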(fn `SetStat`
  (params (statsEnum :type "/Game/BP/Enum/E_IAStats Enum" :default "NewEnumerator4") (Value :type "Float (double-precision)"))
  (switch `/Game/BP/Enum/E_IAStats` statsEnum
    (:`NewEnumerator4`
      (bind _structout (setmembers `/Game/BP/Structure/ST_IAStats` :`StructRef` (`self.stats`) :`health` Value))
      (set `self.stats` _structout))
    (:`NewEnumerator11`
      (bind _structout_2 (setmembers `/Game/BP/Structure/ST_IAStats` :`StructRef` (`self.stats`) :`DodgeRatio` Value))
      (set `self.stats` _structout_2))
    (:`NewEnumerator12`
      (bind _structout_3 (setmembers `/Game/BP/Structure/ST_IAStats` :`StructRef` (`self.stats`) :`BlockRatio` Value))
      (set `self.stats` _structout_3))
    (:`NewEnumerator13`
      (bind _structout_4 (setmembers `/Game/BP/Structure/ST_IAStats` :`StructRef` (`self.stats`) :`Battlescore` Value))
      (set `self.stats` _structout_4))))

(fn `Update Stat`
  (params (statsEnum :type "/Game/BP/Enum/E_IAStats Enum" :default "NewEnumerator4") (Value :type "Float (double-precision)"))
  (switch `/Game/BP/Enum/E_IAStats` statsEnum
    (:`NewEnumerator4`
      (bind _structout (setmembers `/Game/BP/Structure/ST_IAStats` :`StructRef` (`self.stats`) :`health` (+ Value 1.0)))
      (set `self.stats` _structout))
    (:`NewEnumerator11`
      (bind _structout_2 (setmembers `/Game/BP/Structure/ST_IAStats` :`StructRef` (`self.stats`) :`DodgeRatio` (+ Value 1.0)))
      (set `self.stats` _structout_2))
    (:`NewEnumerator12`
      (bind _structout_3 (setmembers `/Game/BP/Structure/ST_IAStats` :`StructRef` (`self.stats`) :`BlockRatio` (+ Value 1.0)))
      (set `self.stats` _structout_3))
    (:`NewEnumerator13`
      (bind _structout_4 (setmembers `/Game/BP/Structure/ST_IAStats` :`StructRef` (`self.stats`) :`Battlescore` (+ Value 1.0)))
      (set `self.stats` _structout_4))))