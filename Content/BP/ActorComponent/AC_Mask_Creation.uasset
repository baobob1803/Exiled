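; Actor component for the Creation mask, providing its active ability, passive hit effect and equip bonus from a data table row.
; Active with cooldown runs the parent cooldown and raises the player's CreationMaskActive flag until a timer clears it; without cooldown, it restarts that timer using the bonus duration.
; Passive damages hit AI through their controller.
; Equipping changes the player's poise regen and restarts its regen setup, while unequipping restores the saved value.
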(event `self.Active`
  (params (useCooldown :type Boolean) (`Hud Ref` :type "/Game/BP/Widget/WBP_HUD Object Reference"))
  (bind (_datatable _rowname) (break `DataTableRowHandle` (`self.maskInfo`)))
  (bind (_datatable_2 _rowname_2) (break `DataTableRowHandle` (`self.maskInfo`)))
  (if useCooldown
    (`parent.Cooldown` `Hud Ref`)
    (if (not (`/Game/BP/Character/Player/BP_MasterPlayer.CreationMaskActive` (`self.Player`)))
      (set `/Game/BP/Character/Player/BP_MasterPlayer.CreationMaskActive` true (`self.Player`))
      (bind _returnvalue (`|GetDataTableRow` _datatable _rowname)
        (:`then`
          (`KismetSystemLibrary.K2_SetTimer` null "TimerActive" (`.activeTime_6_09457FDD4E81918A0D2F918F8CC47635` (break `/Game/BP/Structure/ST_Creation` (`.Creation_39_CA059B174FD18078D6BC6186B00FB4EC` (break `/Game/BP/Structure/ST_Mask` _returnvalue))))))))
    (elif (`/Game/BP/Character/Player/BP_MasterPlayer.CreationMaskActive` (`self.Player`))
      (bind _returnvalue_2 (`|GetDataTableRow` _datatable_2 _rowname_2)
        (:`then`
          (`KismetSystemLibrary.PrintString` "reset active" true true (struct :`R` 1.0 :`G` 0.466667 :`A` 1.0))
          (`KismetSystemLibrary.K2_SetTimer` null "TimerActive" (`.activeTimeBonus_12_D770E36B429846CE821D91B814605987` (break `/Game/BP/Structure/ST_Creation` (`.Creation_39_CA059B174FD18078D6BC6186B00FB4EC` (break `/Game/BP/Structure/ST_Mask` _returnvalue_2))))))))))

(event `self.Passive`
  (params (hitActor :type "Actor Object Reference"))
  (bind (_datatable _rowname) (break `DataTableRowHandle` (`self.maskInfo`)))
  (bind _asbp_master_ia (cast `/Game/BP/Character/IA/BP_MasterIA` hitActor))
  (bind _returnvalue (`|GetDataTableRow` _datatable _rowname)
    (:`then`
      (`/Game/BP/Character/IA/AIC_IAController.TakeDamage` (`/Game/BP/Character/IA/BP_MasterIA.As AIC IAController` _asbp_master_ia) (`.Damage_2_2667A275453BC925D9C4A7A630126516` (break `/Game/BP/Structure/ST_Creation` (`.Creation_39_CA059B174FD18078D6BC6186B00FB4EC` (break `/Game/BP/Structure/ST_Mask` _returnvalue)))))
      (`KismetSystemLibrary.PrintString` "WTF Bro " true true (struct :`R` 0.152 :`B` 0.984375 :`A` 1.0)))))

(event `self.OnEquipMask`
  (params (Player :type "/Game/BP/Character/Player/BP_MasterPlayer Object Reference"))
  (bind (_datatable _rowname) (break `DataTableRowHandle` (`self.maskInfo`)))
  (bind _output_get (set `self.Player` Player))
  (`KismetSystemLibrary.K2_PauseTimerHandle` (`/Game/BP/Character/Player/BP_MasterPlayer.timerRegenPoise` _output_get))
  (bind _ac_stats (`/Game/BP/Character/Player/BP_MasterPlayer.AC_Stats` _output_get))
  (set `self.basePoiseRengen` (`.poiseRegen_41_752E3CE74E34AC0C60BC79ABB0561E9A` (break `/Game/BP/Structure/ST_Stats` (`/Game/BP/ActorComponent/AC_Stats.stats` _ac_stats))))
  (bind _returnvalue (`|GetDataTableRow` _datatable _rowname)
    (:`then`
      (`/Game/BP/ActorComponent/AC_Stats.StatsBehaviour` _ac_stats "NewEnumerator7" (`.poiseRegen_8_172DEB7245E853F74F852B91E39E50A6` (break `/Game/BP/Structure/ST_Creation` (`.Creation_39_CA059B174FD18078D6BC6186B00FB4EC` (break `/Game/BP/Structure/ST_Mask` _returnvalue)))))
      (`/Game/BP/Character/Player/BP_MasterPlayer.SetupRegenPoiseEvent` _output_get))))

(event `self.OnUnequipMask`
  (bind _asbp_master_player (cast `/Game/BP/Character/Player/BP_MasterPlayer` (`self.GetOwner`)))
  (`KismetSystemLibrary.K2_PauseTimerHandle` (`/Game/BP/Character/Player/BP_MasterPlayer.timerRegenPoise` _asbp_master_player))
  (`/Game/BP/ActorComponent/AC_Stats.StatsBehaviour` (`/Game/BP/Character/Player/BP_MasterPlayer.AC_Stats` _asbp_master_player) "NewEnumerator7" (`self.basePoiseRengen`))
  (`/Game/BP/Character/Player/BP_MasterPlayer.SetupRegenPoiseEvent` _asbp_master_player))

(fn `TimerActive`
  (set `/Game/BP/Character/Player/BP_MasterPlayer.CreationMaskActive` false (`self.Player`))
  (`KismetSystemLibrary.PrintString` "disable Active" true true (struct :`R` 1.0 :`G` 0.555584 :`B` 0.074615 :`A` 1.0)))