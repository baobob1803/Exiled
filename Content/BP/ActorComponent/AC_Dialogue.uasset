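; Actor component that holds an NPC's main and repeated dialogue and feeds it to the dialogue screen widget.
; ParseDialogue splits an entry on "¤" into lines, which NextDialogueLine displays one by one, returning a length-based cooldown with a minimum floor.
; ContinueDialogue advances or ends the sequence, GetQuestion reads question data, and AfficherQuestion builds branching answer widgets.
; Cooldown ratio and answers always come from the main dialogue array.
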(event `self.ReceiveBeginPlay`
  (`self.ParseDialogue` 0 true))

(event `ParseDialogue`
  (params (DialogueIndex :type Integer) (`MainDialogue?` :type Boolean))
  (if `MainDialogue?`
    (bind _output_get (set `self.Dialogue Index` DialogueIndex))
    (set `self.ParsedDialogue` (`KismetStringLibrary.ParseIntoArray` (`KismetTextLibrary.Conv_TextToString` (`.Dialogue_2_114EBEB9402713DA8E2AFA86631E269E` (break `/Game/BP/Structure/ST_Dialogue` (`|GetArrayItem` (`self.ST_MainDialogue`) _output_get)))) "¤"))
    (else
      (bind _output_get_2 (set `self.Dialogue Index` DialogueIndex))
      (set `self.ParsedDialogue` (`KismetStringLibrary.ParseIntoArray` (`KismetTextLibrary.Conv_TextToString` (`.Dialogue_2_114EBEB9402713DA8E2AFA86631E269E` (break `/Game/BP/Structure/ST_Dialogue` (`|GetArrayItem` (`self.ST_RepeatedDialogue`) _output_get_2)))) "¤")))))

(fn `AfficherQuestion`
  (params (Widget :type "/Game/BP/Widget/WBP_MasterDialogue Object Reference") (Pnj :type "/Game/BP/World/BP_PNJ Object Reference"))
  (`PanelWidget.ClearChildren` (`/Game/BP/Widget/WBP_MasterDialogue.VB_Answer` Widget))
  (for _array_element (`.Answers_19_1879D3F9479D932C54D79FB61FFED417` (break `/Game/BP/Structure/ST_Dialogue` (`|GetArrayItem` (`self.ST_MainDialogue`) (`self.Dialogue Index`))))
    (bind (_answer _toindexdialogue) (break `/Game/BP/Structure/ST_DialogueAnswer` _array_element))
    (bind _returnvalue (`|CreateWidget` "/Game/BP/Widget/WBP_Answer.WBP_Answer_C" null _answer self _toindexdialogue Pnj))
    (`PanelWidget.AddChild` (`/Game/BP/Widget/WBP_MasterDialogue.VB_Answer` Widget) _returnvalue)))

(fn `Continue Dialogue`
  (params (MainDialogue :type Boolean))
  (returns (Value :type Boolean) (`Dialogue Index` :type Integer))
  (bind _returnvalue (+ (`self.Dialogue Index`) 1))
  (bind _returnvalue_2 (+ (`self.Dialogue Index`) 1))
  (if MainDialogue
    (if (== _returnvalue (`KismetArrayLibrary.Array_Length` (`self.ST_MainDialogue`)))
      (return true 0)
      (else
        (return false _returnvalue)))
    (elif (== _returnvalue_2 (`KismetArrayLibrary.Array_Length` (`self.ST_RepeatedDialogue`)))
      (return true 0)
      (else
        (return false _returnvalue_2)))))

(fn `GetQuestion?`
  (params (DialogueIndex :type Integer) (MainDialogue :type Boolean))
  (returns (NewParam :type Boolean))
  (if MainDialogue
    (return (`.Question?_8_117873A3438FC4CD2D6B78A4E314D006` (break `/Game/BP/Structure/ST_Dialogue` (`|GetArrayItem` (`self.ST_MainDialogue`) DialogueIndex))))
    (else
      (return (`.Question?_8_117873A3438FC4CD2D6B78A4E314D006` (break `/Game/BP/Structure/ST_Dialogue` (`|GetArrayItem` (`self.ST_RepeatedDialogue`) DialogueIndex)))))))

(fn `NextDialogueLine`
  (params (CurrentIndex :type Integer) (WBP_DialogueScreen :type "/Game/BP/Widget/WBP_MasterDialogue Object Reference"))
  (returns (ReturnValue :type Boolean) (CurrentIndexLine :type Integer) (ChangeCooldown :type "Float (double-precision)"))
  (locals (currentIndexDialogue :type Integer) (`current index` :type Integer))
  (bind _parseddialogue (`self.ParsedDialogue`))
  (bind _output_get (set `local.current index` CurrentIndex))
  (if (== (`KismetArrayLibrary.Array_Length` _parseddialogue) CurrentIndex)
    (return true 0 2.0)
    (else
      (bind _output (`|GetArrayItem` _parseddialogue _output_get))
      (`/Game/BP/Widget/WBP_MasterDialogue.ChangeDialogue` WBP_DialogueScreen _output)
      (bind _returnvalue (/ (`KismetMathLibrary.Conv_IntToDouble` (`KismetStringLibrary.Len` _output)) (`.CoolDownRatio_26_4627CF574CFA0B47010DFF8447B8120A` (break `/Game/BP/Structure/ST_Dialogue` (`|GetArrayItem` (`self.ST_MainDialogue`) (`self.Dialogue Index`))))))
      (if (< _returnvalue 2.0)
        (set `self.dialogueChangeCooldown` 2.0)
        (else
          (set `self.dialogueChangeCooldown` _returnvalue)))
      (bind _output_get_2 (set `local.currentIndexDialogue` (+ (`local.current index`) 1)))
      (return false _output_get_2 (`self.dialogueChangeCooldown`)))))