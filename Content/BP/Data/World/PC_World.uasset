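; World player controller that owns the pause menus and handles camera view switching.
; On BeginPlay it creates the pause, options and masks widgets, cross-links them and adds them to the viewport hidden and disabled.
; Pause input notifies the pawn, then toggles game pause, input mode and cursor, inferring paused state from whether any listed widget is enabled.
; SwitchCamera blends briefly between a supplied altar view target and the BP_MasterPlayer actor.
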(event `self.ReceiveBeginPlay`
  (bind _listofallexistingpausewidgets (`self.ListOfAllExistingPauseWidgets`))
  ;[1 1 1] Initialize Widgets
  (set `self.bShowMouseCursor` false)
  (`WidgetBlueprintLibrary.SetInputMode_GameOnly` self)
  (bind _returnvalue (`|CreateWidget` "/Game/BP/Widget/WBP_Pause.WBP_Pause_C" null null self))
  (`KismetArrayLibrary.Array_Add` _listofallexistingpausewidgets _returnvalue)
  (set `self.PauseMenu` _returnvalue)
  (bind _returnvalue_2 (`|CreateWidget` "/Game/BP/Widget/MainMenuWidgets/OptionsWigets/WBP_MainOptions.WBP_MainOptions_C" null false null _returnvalue))
  (`KismetArrayLibrary.Array_Add` _listofallexistingpausewidgets _returnvalue_2)
  (set `/Game/BP/Widget/WBP_Pause.mainOption` _returnvalue_2 _returnvalue)
  (bind _returnvalue_3 (`|CreateWidget` "/Game/BP/Widget/WBP_Masks.WBP_Masks_C" null null self _returnvalue))
  (`KismetArrayLibrary.Array_Add` _listofallexistingpausewidgets _returnvalue_3)
  (set `/Game/BP/Widget/WBP_Pause.MasksMenu` _returnvalue_3 _returnvalue)
  (set `self.MaskMenuRef` _returnvalue_3)
  (`self.InitializeWidgetsState`))

(event `InitializeWidgetsState`
  ;[1 1 1] Initialize Widget States
  (for _array_element (`self.ListOfAllExistingPauseWidgets`)
    (`self.AddAndHideWidget` _array_element 1))
  (`KismetSystemLibrary.PrintString` "All Widgets initialized" true true (struct :`R` 0.013678 :`G` 0.364583 :`A` 1.0) 3.0))

(event `PauseBehaviour`
  (bind _pausemenu (`self.PauseMenu`))
  ;[1 1 1] Pause Behavior
  (for _array_element (`self.ListOfAllExistingPauseWidgets`)
    (if (`Widget.GetIsEnabled` _array_element)
      (set `self.GamePaused` true)
      (break)
      (else
        (set `self.GamePaused` false))))
  (if (`self.GamePaused`)
    ;;[0 0.1591 1] Unpause Game
    (for _array_element_2 (`self.ListOfAllExistingPauseWidgets`)
      (`Widget.SetVisibility` _array_element_2 "Hidden")
      (`Widget.SetIsEnabled` _array_element_2 false))
    (set `self.bShowMouseCursor` false)
    (`WidgetBlueprintLibrary.SetInputMode_GameOnly` self)
    (`GameplayStatics.SetGamePaused` false)
    (else
      ;;[1 0 0] Pause Game
      (`Widget.SetVisibility` _pausemenu "Visible")
      (`Widget.SetIsEnabled` _pausemenu true)
      (`WidgetBlueprintLibrary.SetInputMode_GameAndUIEx` self (`/Game/BP/Widget/WBP_Pause.ResumeButton` (`self.PauseMenu`)))
      (set `self.bShowMouseCursor` true)
      (`GameplayStatics.SetGamePaused` true))))

(event `Switch Camera`
  (params (`Altar view` :type Boolean) (NewViewTarget :type "Actor Object Reference"))
  (if `Altar view`
    (`self.SetViewTargetWithBlend` NewViewTarget 0.2)
    (else
      (bind _returnvalue (`GameplayStatics.GetActorOfClass` "/Game/BP/Character/Player/BP_MasterPlayer.BP_MasterPlayer_C"))
      (`self.SetViewTargetWithBlend` _returnvalue 0.2))))

(event `InputAction|Pause` :paused true
  (params (Key :type "Key Structure"))
  ;[1 1 1] Pause Input
  (:`Pressed`
    (`self.Pause Input Pressed`)))

(event `Pause Input Pressed`
  ;[1 1 1] Pause Input
  (message `/Game/BP/Interface/BPI_Mask.Pause` (`GameplayStatics.GetPlayerPawn` 0))
  (`KismetSystemLibrary.Delay` 0.01)
  (`self.PauseBehaviour`))

(fn `AddAndHideWidget`
  (params (widgetTarget :type "UserWidget Object Reference") (ZOrder :type Integer))
  (`Widget.SetVisibility` widgetTarget "Hidden")
  (`Widget.SetIsEnabled` widgetTarget false)
  (`UserWidget.AddToViewport` widgetTarget ZOrder))

(fn `UserConstructionScript`)