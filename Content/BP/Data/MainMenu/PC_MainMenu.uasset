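; Main menu player controller that builds the main menu UI on BeginPlay, showing the cursor and using Game and UI input.
; It creates the main menu widget plus options and credits widgets, each given a reference to the menu and stored back on it.
; A helper adds the two submenus to the viewport hidden and disabled, so they exist up front without being shown.
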(event `self.ReceiveBeginPlay`
  (set `self.bShowMouseCursor` true)
  (`WidgetBlueprintLibrary.SetInputMode_GameAndUIEx` self null)
  (bind _returnvalue (`|CreateWidget` "/Game/BP/Widget/MainMenuWidgets/WBP_MainMenu.WBP_MainMenu_C"))
  (bind _output_get (set `self.mainMenu` _returnvalue))
  (`UserWidget.AddToViewport` _output_get 1)
  (bind _returnvalue_2 (`|CreateWidget` "/Game/BP/Widget/MainMenuWidgets/OptionsWigets/WBP_MainOptions.WBP_MainOptions_C" null true _returnvalue null))
  (`self.AddAndHideWidget` _returnvalue_2 1)
  (set `/Game/BP/Widget/MainMenuWidgets/WBP_MainMenu.optionMenu` _returnvalue_2 (`self.mainMenu`))
  (bind _returnvalue_3 (`|CreateWidget` "/Game/BP/Widget/MainMenuWidgets/WBP_Credits.WBP_Credits_C" null (`self.mainMenu`)))
  (`self.AddAndHideWidget` _returnvalue_3 1)
  (set `/Game/BP/Widget/MainMenuWidgets/WBP_MainMenu.CreditMenu` _returnvalue_3 (`self.mainMenu`)))

(fn `AddAndHideWidget`
  (params (widgetTarget :type "UserWidget Object Reference") (ZOrder :type Integer))
  (`Widget.SetVisibility` widgetTarget "Hidden")
  (`Widget.SetIsEnabled` widgetTarget false)
  (`UserWidget.AddToViewport` widgetTarget ZOrder))

(fn `UserConstructionScript`)