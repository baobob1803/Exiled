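; Breakable chain world actor that reports whether it is broken and can push a dialogue change to an NPC.
; BeginPlay makes it visible and collidable and caches the player; IsChainbroken treats the hidden state as broken.
; DialogueIndexModEvent prints a debug string, sets FoundNPC's dialogue index and sends it an interaction message with the player.
; The BP_PNJ lookup that assigns FoundNPC is disconnected and never runs.
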(event `self.ReceiveBeginPlay`
  (`self.SetActorHiddenInGame` false)
  (`self.SetActorEnableCollision` true)
  (bind _returnvalue (`GameplayStatics.GetActorOfClass` "/Game/BP/Character/Player/BP_MasterPlayer.BP_MasterPlayer_C"))
  (set `self.Player` _returnvalue))

(event `DialogueIndexModEvent`
  (params (DesiredIndex :type Integer))
  (`KismetSystemLibrary.PrintString` "Event Was Sent !" true true (struct :`R` 0.037358 :`G` 1.0 :`A` 1.0))
  (`/Game/BP/ActorComponent/AC_Dialogue.SetCurrentDialogueIndex` (`/Game/BP/World/BP_PNJ.AC_Dialogue` (`self.FoundNPC`)) DesiredIndex)
  (message `/Game/BP/Interface/BPI_Interaction.Interaction` (`self.FoundNPC`) (`self.Player`)))

(fn `IsChainbroken`
  (returns (ChainIsBroken :type Boolean))
  (if (`self.bHidden`)
    (return true)
    (else
      (return false))))

(fn `UserConstructionScript`)