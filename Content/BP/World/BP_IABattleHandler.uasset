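; Battle coordinator that chooses which registered enemy AIs attack the player.
; Registering an AI starts a timer, if none exists, with a random delay scaled by group size; on firing, selected attackers receive SelectAttack.
; Selection skips AIs in certain states, then scores candidates by targeted status or angle from the player's right vector.
; Score-weighted random rolls thin the candidates, falling back to the highest scorer when none win.
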(event `self.ReceiveBeginPlay`
  (bind _returnvalue (`GameplayStatics.GetActorOfClass` "/Game/BP/Character/Player/BP_MasterPlayer.BP_MasterPlayer_C"))
  (set `self.Player` _returnvalue))

(event `self.ReceiveTick`
  (params (DeltaSeconds :type "Float (single-precision)")))

(fn `AddToList`
  (params (NewItem :type "/Game/BP/Character/IA/AIC_IAController Object Reference (by ref)"))
  (`KismetArrayLibrary.Array_Add` (`self.IA`) NewItem)
  (if (not (`KismetSystemLibrary.K2_TimerExistsHandle` (`self.TimerHandlerIAMove`)))
    (`self.Update Timer Function` false)))

(fn `Angle`
  (params (Target :type "/Game/BP/Character/IA/BP_MasterIA Object Reference"))
  (returns (degree :type "Float (double-precision)"))
  (locals (PointAA :type "Vector Structure") (PointAB :type "Vector Structure") (PointBC :type "Vector Structure") (PointBD :type "Vector Structure"))
  (bind _player (`self.Player`))
  (bind _returnvalue (`self.K2_GetActorLocation` _player))
  (set `local.PointAA` _returnvalue)
  (set `local.PointAB` (`self.K2_GetActorLocation` Target))
  (set `local.PointBC` _returnvalue)
  (set `local.PointBD` (+ (* (`SceneComponent.GetRightVector` (`Character.Mesh` _player)) (`self.GetDistanceTo` Target (`self.Player`))) _returnvalue))
  (return (`KismetMathLibrary.DegAcos` (/ (+ (* (- (.x (`local.PointAB`)) (.x (`local.PointAA`))) (- (.x (`local.PointBD`)) (.x (`local.PointBC`)))) (* (- (.y (`local.PointAB`)) (.y (`local.PointAA`))) (- (.y (`local.PointBD`)) (.y (`local.PointBC`))))) (* (`KismetMathLibrary.Sqrt` (+ (`KismetMathLibrary.Square` (- (.x (`local.PointAB`)) (.x (`local.PointAA`)))) (`KismetMathLibrary.Square` (- (.y (`local.PointAB`)) (.y (`local.PointAA`)))))) (`KismetMathLibrary.Sqrt` (+ (`KismetMathLibrary.Square` (- (.x (`local.PointBD`)) (.x (`local.PointBC`)))) (`KismetMathLibrary.Square` (- (.y (`local.PointBD`)) (.y (`local.PointBC`)))))))))))

(fn `Attribute Battle Score with angle`
  (params (AI_Controller :type "/Game/BP/Character/IA/AIC_IAController Object Reference") (Angle :type "Float (double-precision)"))
  (returns (Score :type "Float (double-precision)"))
  (locals (`Score index` :type Integer) (L_Angle :type "Float (double-precision)") (L_AIController :type "/Game/BP/Character/IA/AIC_IAController Object Reference"))
  (bind (_health _dodgeratio _blockratio _dodgedistance _battlescore _positionscoreanglescore) (break `/Game/BP/Structure/ST_IAStats` (`/Game/BP/ActorComponent/AC_IAStats.stats` (`/Game/BP/Character/IA/AIC_IAController.AC_IAStats` (`local.L_AIController`)))))
  (set `local.L_AIController` AI_Controller)
  (set `local.L_Angle` Angle)
  (bind _keys (`BlueprintMapLibrary.Map_Keys` _positionscoreanglescore))
  (for (_array_element _array_index) _keys
    (if (< (`local.L_Angle`) _array_element)
      (set `local.Score index` _array_index)
      (break)))
  (bind _values (`BlueprintMapLibrary.Map_Values` _positionscoreanglescore))
  (return (`|GetArrayItem` _values (`local.Score index`))))

(fn `IAMove Handler`
  (if (>= (`KismetArrayLibrary.Array_Length` (`self.IA`)) 1)
    (bind (_attacker _listattacker) (`self.Select Attacker`))
    (for _array_element _listattacker
      (`/Engine/EditorBlueprintResources/StandardMacros.IsValid` _array_element
        (:`Is Valid`
          (`/Game/BP/Character/IA/AIC_IAController.SelectAttack` _array_element))))))

(fn `RemoveFromList`
  (params (Item :type "/Game/BP/Character/IA/AIC_IAController Object Reference (by ref)"))
  (bind _ia (`self.IA`))
  (`KismetArrayLibrary.Array_RemoveItem` _ia Item)
  (`KismetArrayLibrary.Array_Resize` _ia (`KismetArrayLibrary.Array_Length` _ia)))

(fn `Select Attacker`
  (returns (Attacker :type "/Game/BP/Character/IA/AIC_IAController Object Reference") (ListAttacker :type "Array of /Game/BP/Character/IA/AIC_IAController Object Reference"))
  (locals (tempIA :type "/Game/BP/Character/IA/AIC_IAController Object Reference") (TotalBattleScore :type "Float (double-precision)") (BattleIAList :type "Array of /Game/BP/Character/IA/AIC_IAController Object Reference") (GreatestScoreIA :type "/Game/BP/Character/IA/AIC_IAController Object Reference") (WinnerIA :type "Array of /Game/BP/Character/IA/AIC_IAController Object Reference"))
  (bind _greatestscoreia (`local.GreatestScoreIA`))
  (bind _returnvalue (`KismetArrayLibrary.Array_Length` (`local.WinnerIA`)))
  (bind _ac_iastats (`/Game/BP/Character/IA/AIC_IAController.AC_IAStats` (`local.tempIA`)))
  (set `local.TotalBattleScore` 0.0)
  (set `local.GreatestScoreIA` null)
  (for _array_element (`self.IA`)
    (bind _output_get (set `local.tempIA` _array_element))
    (bind _newparam (`self.TestState` _output_get))
    (if (not _newparam)
      (`KismetArrayLibrary.Array_Add` (`local.BattleIAList`) (`local.tempIA`))
      (if (`/Game/BP/Character/IA/AIC_IAController.IsTargeted` (`local.tempIA`))
        (`/Game/BP/ActorComponent/AC_IAStats.Update Stat` _ac_iastats "NewEnumerator13" (`.targetedScore_51_074524124726DBDD44A8BA8965083D6E` (break `/Game/BP/Structure/ST_IAStats` (`/Game/BP/ActorComponent/AC_IAStats.stats` _ac_iastats))))
        (else
          (bind _degree (`self.Angle` (`/Game/BP/Character/IA/AIC_IAController.As BP Master IA` (`local.tempIA`))))
          (bind _score (`self.Attribute Battle Score with angle` (`local.tempIA`) _degree))
          (`/Game/BP/ActorComponent/AC_IAStats.Update Stat` (`/Game/BP/Character/IA/AIC_IAController.AC_IAStats` (`local.tempIA`)) "NewEnumerator13" _score)))))
  (for _array_element_2 (`local.BattleIAList`) :!label _label
    (set `local.TotalBattleScore` (+ (`.Battlescore_42_27AEFA984D3DD14FF87A7CA4EFD2232E` (break `/Game/BP/Structure/ST_IAStats` (`/Game/BP/ActorComponent/AC_IAStats.stats` (`/Game/BP/Character/IA/AIC_IAController.AC_IAStats` _array_element_2)))) (`local.TotalBattleScore`))))
  (for (_array_element_3 _array_index) (`local.BattleIAList`)
    (if (<= (`KismetMathLibrary.RandomFloatInRange` 0.0 1.0) (/ (`.Battlescore_42_27AEFA984D3DD14FF87A7CA4EFD2232E` (break `/Game/BP/Structure/ST_IAStats` (`/Game/BP/ActorComponent/AC_IAStats.stats` (`/Game/BP/Character/IA/AIC_IAController.AC_IAStats` _array_element_3)))) (`local.TotalBattleScore`)))
      (bind _ac_iastats_2 (`/Game/BP/Character/IA/AIC_IAController.AC_IAStats` _array_element_3))
      (`KismetSystemLibrary.PrintString` (`KismetStringLibrary.Concat_StrStr` "win wtith Score : " (`KismetStringLibrary.Conv_DoubleToString` (`.Battlescore_42_27AEFA984D3DD14FF87A7CA4EFD2232E` (break `/Game/BP/Structure/ST_IAStats` (`/Game/BP/ActorComponent/AC_IAStats.stats` _ac_iastats_2))))) true true (struct :`G` 0.66 :`B` 1.0 :`A` 1.0) 5.0)
      (`KismetArrayLibrary.Array_Add` (`local.WinnerIA`) _array_element_3)
      (else
        (`/Game/BP/ActorComponent/AC_IAStats.Update Stat` _ac_iastats_2 "NewEnumerator13" 1.0)
        (`KismetArrayLibrary.Array_Remove` (`local.BattleIAList`) _array_index))))
  (`KismetArrayLibrary.Array_Resize` (`local.BattleIAList`) _returnvalue)
  (`KismetSystemLibrary.PrintString` (`KismetStringLibrary.Concat_StrStr` "battleList = " (`KismetStringLibrary.Conv_IntToString` _returnvalue)) true true (struct :`G` 0.66 :`B` 1.0 :`A` 1.0) 5.0)
  (if (> _returnvalue 1)
    (if (> (`KismetArrayLibrary.Array_Length` (`local.BattleIAList`)) 3)
      (goto _label)
      (else
        (`KismetSystemLibrary.PrintString` (`KismetStringLibrary.Concat_StrStr` "There are " (`KismetStringLibrary.Conv_IntToString` (`KismetArrayLibrary.Array_Length` (`self.IA`))) " able enemies, so " (`KismetStringLibrary.Conv_IntToString` (`KismetArrayLibrary.Array_Length` (`local.BattleIAList`))) "of them will attacl"))
        (return null (`local.BattleIAList`))))
    (elif (== _returnvalue 0)
      (`KismetArrayLibrary.Array_Shuffle` (`self.IA`))
      (for _array_element_4 (`self.IA`)
        (bind _greatestscoreia_2 (`local.GreatestScoreIA`)
          (:`then`
            (if (> (`.Battlescore_42_27AEFA984D3DD14FF87A7CA4EFD2232E` (break `/Game/BP/Structure/ST_IAStats` (`/Game/BP/ActorComponent/AC_IAStats.stats` (`/Game/BP/Character/IA/AIC_IAController.AC_IAStats` _array_element_4)))) (`.Battlescore_42_27AEFA984D3DD14FF87A7CA4EFD2232E` (break `/Game/BP/Structure/ST_IAStats` (`/Game/BP/ActorComponent/AC_IAStats.stats` (`/Game/BP/Character/IA/AIC_IAController.AC_IAStats` _greatestscoreia_2)))))
              (set `local.GreatestScoreIA` _array_element_4)))
          (:`else`
            (set `local.GreatestScoreIA` _array_element_4))))
      (`KismetSystemLibrary.PrintString` (`KismetStringLibrary.Concat_StrStr` "There are " (`KismetStringLibrary.Conv_IntToString` (`KismetArrayLibrary.Array_Length` (`self.IA`))) " able enemies, so " "1" " of them will attacl"))
      (`KismetSystemLibrary.PrintString` (`KismetStringLibrary.Concat_StrStr` "win wtith Score : " (`KismetStringLibrary.Conv_DoubleToString` (`.Battlescore_42_27AEFA984D3DD14FF87A7CA4EFD2232E` (break `/Game/BP/Structure/ST_IAStats` (`/Game/BP/ActorComponent/AC_IAStats.stats` (`/Game/BP/Character/IA/AIC_IAController.AC_IAStats` (`local.GreatestScoreIA`))))))))
      (return _greatestscoreia (`|MakeArray` _greatestscoreia))
      (else
        (`KismetSystemLibrary.PrintString` (`KismetStringLibrary.Concat_StrStr` "There are " (`KismetStringLibrary.Conv_IntToString` (`KismetArrayLibrary.Array_Length` (`self.IA`))) " able enemies, so " (`KismetStringLibrary.Conv_IntToString` (`KismetArrayLibrary.Array_Length` (`local.BattleIAList`))) " of them will attacl"))
        (return null (`local.BattleIAList`))))))

(fn `TestState`
  (params (Target :type "/Game/BP/Character/IA/AIC_IAController Object Reference"))
  (returns (NewParam :type Boolean))
  (bind _currentstate (`/Game/BP/Character/IA/AIC_IAController.CurrentState` Target))
  (return (or (`|EnumEquality` _currentstate "NewEnumerator10") (`|EnumEquality` _currentstate "NewEnumerator9") (`|EnumEquality` _currentstate "NewEnumerator13") (`|EnumEquality` _currentstate "NewEnumerator14") (`|EnumEquality` _currentstate "NewEnumerator2") (`|EnumEquality` _currentstate "NewEnumerator11") (`|EnumEquality` _currentstate "NewEnumerator11") (`|EnumEquality` _currentstate "NewEnumerator15"))))

(fn `Update Timer Function`
  (params (`in void` :type Boolean))
  (bind _returnvalue (`KismetArrayLibrary.Array_Length` (`self.IA`)))
  (if (== _returnvalue 0)
    (`KismetSystemLibrary.K2_ClearAndInvalidateTimerHandle` (`self.TimerHandlerIAMove`))
    (else
      (if `in void`
        (set `self.Time` 1.0)
        (else
          (bind _output_get (set `self.Time` (`KismetMathLibrary.RandomFloatInRange` (* 1 (`KismetMathLibrary.Conv_IntToDouble` _returnvalue)) (* 2 (`KismetMathLibrary.Conv_IntToDouble` _returnvalue)))))))
      (bind _returnvalue_2 (`KismetSystemLibrary.K2_SetTimer` null "IAMove Handler" _output_get))
      (set `self.TimerHandlerIAMove` _returnvalue_2))))

(fn `UserConstructionScript`)