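; BP_IASpawner is a world actor that spawns a configurable number of BP_MasterIA actors when play begins.
; A DoN-gated event calls itself recursively, placing each AI at a random navigable point around the spawner.
; Each AI receives the spawner's patrol mark array as its route, with a random starting index.
; The construction script labels each patrol mark's text render with its array index.
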(event `SpawnIANTime`
  (bind _bp_patrolmark (`self.BP_PatrolMark`))
  (`/Engine/EditorBlueprintResources/StandardMacros.Do N` (`self.NbIAToSpawn`) :!label _label
    (:`Exit`
      (bind _randomlocation (`NavigationSystemV1.K2_GetRandomLocationInNavigableRadius` (`self.K2_GetActorLocation`) 500.0 null null))
      (`|SpawnActorFromClass` "/Game/BP/Character/IA/BP_MasterIA.BP_MasterIA_C" (`KismetMathLibrary.MakeTransform` _randomlocation) "AdjustIfPossibleButAlwaysSpawn" "OverrideRootScale" null _bp_patrolmark (`.OutIndex` (`KismetArrayLibrary.Array_Random` _bp_patrolmark)) null)
      (`self.SpawnIANTime`))))

(event `self.ReceiveBeginPlay`
  (goto _label))

(fn `UserConstructionScript`
  (for (_array_element _array_index) (`self.BP_PatrolMark`)
    (`TextRenderComponent.K2_SetText` (`/Game/BP/World/BP_PatrolMark.TextRender` _array_element) (`KismetTextLibrary.Conv_IntToText` _array_index))))