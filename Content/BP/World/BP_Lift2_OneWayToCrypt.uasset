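; One-way lift, apparently to the crypt, that carries the player down and opens another level.
; BeginPlay snaps the lift to its up position and caches the master player and game instance.
; Overlapping the box while idle flags a lift transition, calls the player's LiftInteract and starts a timeline that lerps the lift between markers.
; When the timeline finishes, it passes the spawn location name to the game instance and loads the target level.
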(event `self.ReceiveBeginPlay`
  ;[1 0.3856 0.2958] Init References and Lift Position
  (bind _returnvalue (`GameplayStatics.GetActorOfClass` "/Game/BP/Character/Player/BP_MasterPlayer.BP_MasterPlayer_C"))
  (set `self.MasterPlayerRef` _returnvalue)
  (bind _asbpi_player_instance (cast `/Game/BP/Data/BPI_PlayerInstance` (`GameplayStatics.GetGameInstance`)))
  (set `self.BPIPlayerInstanceRef` _asbpi_player_instance)
  (`SceneComponent.K2_SetWorldLocation` (`self.Lift`) (`SceneComponent.K2_GetComponentLocation` (`self.UpPosition`)) false true))

(event `MovingLIft`
  ;[0.2901 0.8291 1] Lift Movement
  (set `self.Moving` true)
  (if (== (`SceneComponent.K2_GetComponentLocation` (`self.Lift`)) (`SceneComponent.K2_GetComponentLocation` (`self.UpPosition`)) :`ErrorTolerance` 2.0)
    (bind (_direction _timetomove) (`Timeline|LiftTimer` :!via `ReverseFromEnd` :!label _label)
      (:`Update`
        (`SceneComponent.K2_SetWorldLocation` (`self.Lift`) (`KismetMathLibrary.VLerp` (`SceneComponent.K2_GetComponentLocation` (`self.DownPosition`)) (`SceneComponent.K2_GetComponentLocation` (`self.UpPosition`)) _timetomove) false false))
      (:`Finished`
        (set `self.Moving` false)
        (set `/Game/BP/Data/BPI_PlayerInstance.transitionLocationName` (`self.SpawnLocationName`) (`self.BPIPlayerInstanceRef`))
        (`GameplayStatics.OpenLevel` (`self.LevelToOpenName`))))
    (else
      (goto _label))))

(event `self.Box.OnComponentBeginOverlap`
  (params (OverlappedComponent :type "PrimitiveComponent Object Reference") (OtherActor :type "Actor Object Reference") (OtherComp :type "PrimitiveComponent Object Reference") (OtherBodyIndex :type Integer) (bFromSweep :type Boolean) (SweepResult :type "HitResult Structure (by ref)"))
  (if (not (`self.Moving`))
    (set `/Game/BP/Data/BPI_PlayerInstance.IsLiftTransition` true (`self.BPIPlayerInstanceRef`))
    (`/Game/BP/Character/Player/BP_MasterPlayer.LiftInteract` (`self.MasterPlayerRef`))
    (`self.MovingLIft`)))

(fn `UserConstructionScript`)