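; NPC (PNJ) that shows dialogue lines to the player who interacts with it inside its detection sphere.
; Overlap registers it as the player's dialogue trigger and toggles the input prompt; leaving hides the dialogue and resets the index.
; Interaction shows the widget or skips ahead, while a retriggerable delay scaled to line length auto-advances.
; Construction splits TestText on "¤" into the main dialogue; once finished, repeated dialogue plays instead.
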(event `self.Sphere.OnComponentBeginOverlap`
  (params (OverlappedComponent :type "PrimitiveComponent Object Reference") (OtherActor :type "Actor Object Reference") (OtherComp :type "PrimitiveComponent Object Reference") (OtherBodyIndex :type Integer) (bFromSweep :type Boolean) (SweepResult :type "HitResult Structure (by ref)"))
  (bind _as_bp_master_player (`self.As BP Master Player`))
  (`/Engine/EditorBlueprintResources/StandardMacros.IsValid` (`self.As BP Master Player`)
    (:`Is Valid`
      (set `/Game/BP/Character/Player/BP_MasterPlayer.TriggerDialogue` self _as_bp_master_player)
      (`/Game/BP/Character/Player/BP_MasterPlayer.ToggleInteractionInputVisibility` _as_bp_master_player))
    (:`Is Not Valid`
      (bind _asbp_master_player (cast `/Game/BP/Character/Player/BP_MasterPlayer` OtherActor))
      (bind _output_get (set `self.As BP Master Player` _asbp_master_player))
      (set `/Game/BP/Character/Player/BP_MasterPlayer.TriggerDialogue` self _output_get)
      (`/Game/BP/Character/Player/BP_MasterPlayer.ToggleInteractionInputVisibility` _output_get))))

(event `self.Sphere.OnComponentEndOverlap`
  (params (OverlappedComponent :type "PrimitiveComponent Object Reference") (OtherActor :type "Actor Object Reference") (OtherComp :type "PrimitiveComponent Object Reference") (OtherBodyIndex :type Integer))
  (bind _as_bp_master_player (`self.As BP Master Player`))
  (`/Game/BP/Character/Player/BP_MasterPlayer.WidgetVisibility` (`self.As BP Master Player`) (`/Game/BP/Widget/WBP_MasterDialogue.B_Dialogue` (`self.WBP Dialogue`)) false false)
  (`/Game/BP/Character/Player/BP_MasterPlayer.ToggleInteractionInputVisibility` _as_bp_master_player)
  (set `/Game/BP/Character/Player/BP_MasterPlayer.TriggerDialogue` null _as_bp_master_player)
  (set `self.currentIndexDialogue` 0))

(event `AutoChangeDialogue`
  (bind _dialoguechangecooldown (`self.dialogueChangeCooldown`))
  (if (`self.MainDialogueEnded`) :!label _label
    (bind _returnvalue (`self.NextDialogueLine` (`self.RepeatedDialogue`) (`self.currentIndexDialogue`)))
    (if _returnvalue
      (set `self.currentIndexDialogue` 0)
      (`/Game/BP/Character/Player/BP_MasterPlayer.WidgetVisibility` (`self.As BP Master Player`) (`/Game/BP/Widget/WBP_MasterDialogue.B_Dialogue` (`self.WBP Dialogue`)) false false)
      (else
        (`KismetSystemLibrary.RetriggerableDelay` (`self.dialogueChangeCooldown`))
        (`self.AutoChangeDialogue`)))
    (else
      (bind _returnvalue_2 (`self.NextDialogueLine` (`self.MainDialogue`) (`self.currentIndexDialogue`)))
      (if _returnvalue_2
        (set `self.MainDialogueEnded` true)
        (set `self.currentIndexDialogue` 0)
        (`/Game/BP/Character/Player/BP_MasterPlayer.WidgetVisibility` (`self.As BP Master Player`) (`/Game/BP/Widget/WBP_MasterDialogue.B_Dialogue` (`self.WBP Dialogue`)) false false)
        (else
          (`KismetSystemLibrary.RetriggerableDelay` _dialoguechangecooldown)
          (`KismetSystemLibrary.PrintString` (`KismetStringLibrary.Conv_DoubleToString` _dialoguechangecooldown))
          (`self.AutoChangeDialogue`))))))

(event `/Game/BP/Interface/BPI_Interaction.Interaction`
  (params (Player :type "/Game/BP/Character/Player/BP_MasterPlayer Object Reference"))
  (bind _as_bp_master_player (`self.As BP Master Player`))
  (bind _b_dialogue (`/Game/BP/Widget/WBP_MasterDialogue.B_Dialogue` (`self.WBP Dialogue`)))
  (`/Engine/EditorBlueprintResources/StandardMacros.IsValid` (`/Game/BP/Character/Player/BP_MasterPlayer.WBP_Dialogue` Player)
    (:`Is Valid`
      _)
    (:`Is Not Valid`
      (`/Game/BP/Character/Player/BP_MasterPlayer.AddDialogueScreen` _as_bp_master_player)
      (set `self.WBP Dialogue` (`/Game/BP/Character/Player/BP_MasterPlayer.WBP_Dialogue` _as_bp_master_player))))
  (if (`Widget.IsVisible` _b_dialogue)
    (goto _label)
    (else
      (`/Game/BP/Character/Player/BP_MasterPlayer.WidgetVisibility` (`self.As BP Master Player`) _b_dialogue true false)
      (goto _label))))

(fn `NextDialogueLine`
  (params (CurrentDialogue :type "Array of String") (CurrentIndex :type Integer))
  (returns (ReturnValue :type Boolean))
  (bind _output (`|GetArrayItem` CurrentDialogue CurrentIndex))
  (bind _returnvalue (/ (`KismetMathLibrary.Conv_IntToDouble` (`KismetStringLibrary.Len` _output)) (`self.CooldownRatio`)))
  (if (== (`KismetArrayLibrary.Array_Length` CurrentDialogue) (`self.currentIndexDialogue`))
    (return true)
    (else
      (`/Game/BP/Widget/WBP_MasterDialogue.ChangeDialogue` (`self.WBP Dialogue`) _output)
      (if (< _returnvalue 2.0)
        (set `self.dialogueChangeCooldown` 2.0)
        (else
          (set `self.dialogueChangeCooldown` _returnvalue)))
      (set `self.currentIndexDialogue` (+ (`self.currentIndexDialogue`) 1))
      (return false))))

(fn `TextToArray`
  (set `self.MainDialogue` (`KismetStringLibrary.ParseIntoArray` (`KismetTextLibrary.Conv_TextToString` (`self.TestText`)) "¤" false)))

(fn `UserConstructionScript`
  (`SphereComponent.SetSphereRadius` (`self.Sphere`) (`self.detectionRange`) true)
  (`self.TextToArray`))