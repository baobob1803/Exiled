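; Bell actor that shows an interaction prompt and plays a sequence of sounds when the player approaches; its Interaction event only prints a debug message.
; Box overlaps with "interact"-tagged components call SetInteractionVisibility on the cached BP_MasterPlayer's HUD, on both enter and exit.
; Entering also plays the Sound array in order at the Sphere through a duration-based Delay loop up to index 3, which exiting does not stop.
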(event `self.ReceiveBeginPlay`
  (bind _asbp_master_player (cast `/Game/BP/Character/Player/BP_MasterPlayer` (`GameplayStatics.GetPlayerPawn` 0)))
  (set `self.As BP Master Player` _asbp_master_player))

(event `/Game/BP/Interface/BPI_Interaction.Interaction`
  (params (Player :type "/Game/BP/Character/Player/BP_MasterPlayer Object Reference") (displayUI :type Boolean))
  (`KismetSystemLibrary.PrintString` "Hello"))

(event `self.Box.OnComponentBeginOverlap`
  (params (OverlappedComponent :type "PrimitiveComponent Object Reference") (OtherActor :type "Actor Object Reference") (OtherComp :type "PrimitiveComponent Object Reference") (OtherBodyIndex :type Integer) (bFromSweep :type Boolean) (SweepResult :type "HitResult Structure (by ref)"))
  (if (`ActorComponent.ComponentHasTag` OtherComp "interact")
    (`/Game/BP/Widget/WBP_HUD.SetInteractionVisibility` (`/Game/BP/Character/Player/BP_MasterPlayer.HUD` (`self.As BP Master Player`)))
    (set `self.SoundIndex` 0)
    (bind _returnvalue (`GameplayStatics.SpawnSoundAtLocation` (`|GetArrayItem` (`self.Sound`) (`self.SoundIndex`)) (`SceneComponent.K2_GetComponentLocation` (`self.Sphere`)) (struct) 1.0 1.0 0.0 null null :!label _label))
    (`KismetSystemLibrary.Delay` (`SoundBase.Duration` (`AudioComponent.Sound` _returnvalue)))
    (bind _result (`/Engine/EditorBlueprintResources/StandardMacros.IncrementInt` (`self.SoundIndex`))
      (:`  `
        (`/Engine/EditorBlueprintResources/StandardMacros.CompareInt` _result 3
          (:`==`
            (goto _label))
          (:`<`
            (goto _label)))))))

(event `self.Box.OnComponentEndOverlap`
  (params (OverlappedComponent :type "PrimitiveComponent Object Reference") (OtherActor :type "Actor Object Reference") (OtherComp :type "PrimitiveComponent Object Reference") (OtherBodyIndex :type Integer))
  (if (`ActorComponent.ComponentHasTag` OtherComp "interact")
    (bind _as_bp_master_player (`self.As BP Master Player`)
      (:`then`
        (`/Game/BP/Widget/WBP_HUD.SetInteractionVisibility` (`/Game/BP/Character/Player/BP_MasterPlayer.HUD` _as_bp_master_player)))
      (:`else`))))

(fn `UserConstructionScript`)