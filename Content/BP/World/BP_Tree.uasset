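; BP_Tree is a world tree actor whose three falling-leaf Niagara effects respond to the level's wind.
; On BeginPlay it takes the first WindDirectionalSource found and starts a looping 0.1-second timer.
; Each tick of that timer copies the wind's strength and speed into float parameters on all three leaf systems.
; The wind's yaw is stored once at startup but is not passed to the effects.
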(event `self.ReceiveBeginPlay`
  (bind _outactors (`GameplayStatics.GetAllActorsOfClass` "/Script/Engine.WindDirectionalSource"))
  (bind _output_get (set `self.Wind Directionnal` (`|GetArrayItem` _outactors)))
  (bind (_returnvalue_roll _returnvalue_pitch _returnvalue_yaw) (`KismetMathLibrary.BreakRotator` (`self.K2_GetActorRotation` _output_get)))
  (set `self.WindDirection` _returnvalue_yaw)
  (`KismetSystemLibrary.K2_SetTimer` null "Get_Wind" 0.1 true))

(event `Get_Wind`
  (bind _ns_fallleaf (`self.NS_fallLeaf`))
  (bind _component (`WindDirectionalSource.Component` (`self.Wind Directionnal`)))
  (`NiagaraComponent.SetVariableFloat` _ns_fallleaf "WindStrengh" (`WindDirectionalSourceComponent.Strength` _component))
  (`NiagaraComponent.SetVariableFloat` (`self.NS_fallLeaf1`) "WindStrengh" (`WindDirectionalSourceComponent.Strength` _component))
  (`NiagaraComponent.SetVariableFloat` (`self.NS_fallLeaf2`) "WindStrengh" (`WindDirectionalSourceComponent.Strength` _component))
  (`NiagaraComponent.SetVariableFloat` _ns_fallleaf "WindSpeed" (`WindDirectionalSourceComponent.Speed` _component))
  (`NiagaraComponent.SetVariableFloat` (`self.NS_fallLeaf2`) "WindSpeed" (`WindDirectionalSourceComponent.Speed` _component))
  (`NiagaraComponent.SetVariableFloat` (`self.NS_fallLeaf1`) "WindSpeed" (`WindDirectionalSourceComponent.Speed` _component)))

(fn `UserConstructionScript`)