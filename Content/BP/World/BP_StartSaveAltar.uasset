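; BP_StartSaveAltar is a child save altar that interacts with and activates itself for the player when play begins.
; After the parent BeginPlay and a very short delay, it calls Interaction with the UI hidden, then SetActivation, both using the BPMasterPlayer reference.
; Interaction simply forwards to the parent, and the construction script adds nothing of its own.
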(event `self.ReceiveBeginPlay`
  (bind _as_bp_master_player (`self.As BP Master Player`))
  (`parent.ReceiveBeginPlay`)
  (`KismetSystemLibrary.Delay` 0.01)
  (`self.Interaction` _as_bp_master_player false)
  (`self.SetActivation` _as_bp_master_player))

(event `self.Interaction`
  (params (Player :type "/Game/BP/Character/Player/BP_MasterPlayer Object Reference") (displayUI :type Boolean))
  (`parent.Interaction` Player displayUI))

(fn `UserConstructionScript`
  (`parent.UserConstructionScript`))