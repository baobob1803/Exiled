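; A one-use trigger volume that clears the player's LiftSpawn flag when entered.
; On BeginPlay it creates a WBP_OneWay widget, adds it to the viewport and plays its fade.
; When BP_MasterPlayer overlaps its box, it sets LiftSpawn to false and destroys itself.
; A delayed camera shake branch is present but never runs.
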(event `self.ReceiveBeginPlay`
  (bind _returnvalue (`|CreateWidget` "/Game/BP/Widget/WBP_OneWay.WBP_OneWay_C"))
  (`UserWidget.AddToViewport` _returnvalue 5)
  (`/Game/BP/Widget/WBP_OneWay.Fade` _returnvalue))

(event `self.Box.OnComponentBeginOverlap`
  (params (OverlappedComponent :type "PrimitiveComponent Object Reference") (OtherActor :type "Actor Object Reference") (OtherComp :type "PrimitiveComponent Object Reference") (OtherBodyIndex :type Integer) (bFromSweep :type Boolean) (SweepResult :type "HitResult Structure (by ref)"))
  (if (== (`GameplayStatics.GetObjectClass` OtherActor) "/Game/BP/Character/Player/BP_MasterPlayer.BP_MasterPlayer_C")
    (bind _asbp_master_player (cast `/Game/BP/Character/Player/BP_MasterPlayer` OtherActor))
    (set `/Game/BP/Character/Player/BP_MasterPlayer.LiftSpawn` false _asbp_master_player)
    (`self.K2_DestroyActor`)))

(fn `UserConstructionScript`)