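; BP_FloatingRocks is a world actor that moves a rock back and forth along a spline, starting at BeginPlay.
; MoveRocks randomly loads one of two curves into RockTimeline, then a FlipFlop alternates playing it forward and in reverse.
; The timeline scales spline length to position Rock1 and calls MoveRocks again when finished, looping the motion.
; Several disconnected leftovers, including older timeline and rotation logic, never run.
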(event `self.ReceiveBeginPlay`
  (`self.MoveRocks`))

(event `MoveRocks`
  (bind _spline (`self.Spline`))
  (bind (_curve1 _curve2) (break `/Game/BP/Structure/ST_RocksCurves` (`self.CurveStruct`)))
  (switch `int` (`KismetMathLibrary.RandomIntegerInRange` 0 1)
    (:`0`
      (`TimelineComponent.SetFloatCurve` (`self.RockTimeline`) _curve1 "MovementCurve"))
    (:`1`
      (`TimelineComponent.SetFloatCurve` (`self.RockTimeline`) _curve2 "MovementCurve")))
  (`/Engine/EditorBlueprintResources/StandardMacros.FlipFlop`
    (:`A`
      (bind (_direction _movementcurve) (`Timeline|RockTimeline` :!via `PlayFromStart` :!label _label)
        (:`Update`
          (`SceneComponent.K2_SetWorldLocation` (`self.Rock1`) (`SplineComponent.GetLocationAtDistanceAlongSpline` _spline (* _movementcurve (`SplineComponent.GetSplineLength` _spline)) "World") false false))
        (:`Finished`
          (`self.MoveRocks`))))
    (:`B`
      (goto _label :!via `Reverse`))))

(fn `UserConstructionScript`)