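; BP_Trigger_HelpRune is a world trigger that lets the player view a rune help image on the HUD.
; Overlapping its box with an "interact"-tagged component registers it on BP_MasterPlayer and refreshes the interaction prompt.
; Interaction flip-flops between freezing movement while showing the image and restoring walking while hiding it.
; The image comes from BDD_RuneInfo via an enum row name, swapping "Keyboard" for "Gamepad" when gamepad input was last used.
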(event `/Game/BP/Interface/BPI_Interaction.Interaction`
  (params (Player :type "/Game/BP/Character/Player/BP_MasterPlayer Object Reference") (displayUI :type Boolean))
  (bind _returnvalue (`|GetEnumeratorNameAsString` (`self.EnumRowName`)))
  (bind _image_helprune (`/Game/BP/Widget/WBP_HUD.Image_HelpRune` (`/Game/BP/Character/Player/BP_MasterPlayer.HUD` (`self.BP_master_Player`))))
  (`/Engine/EditorBlueprintResources/StandardMacros.FlipFlop`
    (:`A`
      (`CharacterMovementComponent.DisableMovement` (`Character.CharacterMovement` (`self.BP_master_Player`)))
      (if (`/Game/BP/Character/Player/BP_MasterPlayer.lastInputFromGamepad` (`self.BP_master_Player`))
        (bind _returnvalue_2 (`|GetDataTableRow` "/Game/BP/BDD/BDD_RuneInfo.BDD_RuneInfo" (`KismetStringLibrary.Conv_StringToName` (`KismetStringLibrary.Replace` _returnvalue "Keyboard" "Gamepad")))
          (:`then`
            (`Image.SetBrushFromTexture` _image_helprune (`.Image_9_300BFA564DDD23C75E84BF88F914B1F2` (break `/Game/BP/Structure/ST_HelpInfo` _returnvalue_2)) true)
            (`Widget.SetVisibility` _image_helprune "Visible")))
        (else
          (bind _returnvalue_3 (`|GetDataTableRow` "/Game/BP/BDD/BDD_RuneInfo.BDD_RuneInfo" (`KismetStringLibrary.Conv_StringToName` _returnvalue))
            (:`then`
              (`Image.SetBrushFromTexture` _image_helprune (`.Image_9_300BFA564DDD23C75E84BF88F914B1F2` (break `/Game/BP/Structure/ST_HelpInfo` _returnvalue_3)) true)
              (`Widget.SetVisibility` _image_helprune "Visible"))))))
    (:`B`
      (`CharacterMovementComponent.SetMovementMode` (`Character.CharacterMovement` (`self.BP_master_Player`)) "MOVE_Walking" 0)
      (`Widget.SetVisibility` _image_helprune "Hidden"))))

(event `self.ReceiveBeginPlay`
  ;[1 1 1] Event Begin Play
  (bind _asbp_master_player (cast `/Game/BP/Character/Player/BP_MasterPlayer` (`GameplayStatics.GetPlayerCharacter` 0)))
  (set `self.BP_master_Player` _asbp_master_player)
  (`ActorComponent.Activate` (`self.NiagaraParticle`) false))

(event `self.TriggerBox.OnComponentBeginOverlap`
  (params (OverlappedComponent :type "PrimitiveComponent Object Reference") (OtherActor :type "Actor Object Reference") (OtherComp :type "PrimitiveComponent Object Reference") (OtherBodyIndex :type Integer) (bFromSweep :type Boolean) (SweepResult :type "HitResult Structure (by ref)"))
  (bind _bp_master_player (`self.BP_master_Player`))
  ;[1 1 1] Begin Overlap
  (if (`ActorComponent.ComponentHasTag` OtherComp "interact")
    (set `/Game/BP/Character/Player/BP_MasterPlayer.Trigger HelpRune` self _bp_master_player)
    (`/Game/BP/Widget/WBP_HUD.SetInteractionVisibility` (`/Game/BP/Character/Player/BP_MasterPlayer.HUD` _bp_master_player))))

(event `self.TriggerBox.OnComponentEndOverlap`
  (params (OverlappedComponent :type "PrimitiveComponent Object Reference") (OtherActor :type "Actor Object Reference") (OtherComp :type "PrimitiveComponent Object Reference") (OtherBodyIndex :type Integer))
  ;[1 1 1] End Overlap
  (if (`ActorComponent.ComponentHasTag` OtherComp "interact")
    (bind _bp_master_player (`self.BP_master_Player`)
      (:`then`
        (set `/Game/BP/Character/Player/BP_MasterPlayer.Trigger HelpRune` null _bp_master_player)
        (`/Game/BP/Widget/WBP_HUD.SetInteractionVisibility` (`/Game/BP/Character/Player/BP_MasterPlayer.HUD` _bp_master_player)))
      (:`else`))))

(fn `UserConstructionScript`)