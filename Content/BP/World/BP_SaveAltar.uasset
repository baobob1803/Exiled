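; Save altar actor that serves as the player's checkpoint and respawn point.
; A range-sized trigger sphere toggles the player's interaction prompt and registers the altar as TriggerAltar.
; Interaction deactivates the previous altar's visuals, stores itself and its respawn location on BP_MasterPlayer, turns green, then calls the player's save and the GameInstance save message.
; SetActivation re-marks the altar as active for a given target without saving.
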(event `self.ReceiveBeginPlay`
  (bind _returnvalue (`GameplayStatics.GetActorOfClass` "/Game/BP/Character/Player/BP_MasterPlayer.BP_MasterPlayer_C"))
  (set `self.As BP Master Player` _returnvalue))

(event `/Game/BP/Interface/BPI_Interaction.Interaction`
  (params (Player :type "/Game/BP/Character/Player/BP_MasterPlayer Object Reference"))
  (`self.DisablePreviousAltar`)
  (set `/Game/BP/Character/Player/BP_MasterPlayer.LastSavePoint` self (`self.As BP Master Player`))
  (set `/Game/BP/Character/Player/BP_MasterPlayer.RespawnPosition` (`SceneComponent.K2_GetComponentLocation` (`self.RespawnLocation`)) (`self.As BP Master Player`))
  (`PrimitiveComponent.SetMaterial` (`self.Cube`) 0 "/Game/BP/World/TestMaterials/M_AltarActivate.M_AltarActivate")
  (`ArrowComponent.SetArrowColor` (`self.Arrow`) (struct :`G` 1.0 :`A` 1.0))
  (`/Game/BP/Character/Player/BP_MasterPlayer.SaveAltar` (`self.As BP Master Player`))
  (message `/Game/BP/Interface/BPI_Save.Save` (`GameplayStatics.GetGameInstance`)))

(event `DisablePreviousAltar`
  (bind _lastsavepoint (`/Game/BP/Character/Player/BP_MasterPlayer.LastSavePoint` (`self.As BP Master Player`)))
  (`/Engine/EditorBlueprintResources/StandardMacros.IsValid` _lastsavepoint
    (:`Is Valid`
      (`PrimitiveComponent.SetMaterial` (`/Game/BP/World/BP_SaveAltar.Cube` _lastsavepoint) 0 "/Game/BP/World/TestMaterials/M_AltarDesactivate.M_AltarDesactivate")
      (`ArrowComponent.SetArrowColor` (`/Game/BP/World/BP_SaveAltar.Arrow` (`/Game/BP/Character/Player/BP_MasterPlayer.LastSavePoint` (`self.As BP Master Player`))) (struct :`R` 1.0 :`A` 1.0)))))

(event `SetActivation`
  (params (Target :type "/Game/BP/Character/Player/BP_MasterPlayer Object Reference"))
  (set `/Game/BP/Character/Player/BP_MasterPlayer.LastSavePoint` self Target)
  (`PrimitiveComponent.SetMaterial` (`self.Cube`) 0 "/Game/BP/World/TestMaterials/M_AltarActivate.M_AltarActivate")
  (`ArrowComponent.SetArrowColor` (`self.Arrow`) (struct :`G` 1.0 :`A` 1.0)))

(event `self.Sphere.OnComponentBeginOverlap`
  (params (OverlappedComponent :type "PrimitiveComponent Object Reference") (OtherActor :type "Actor Object Reference") (OtherComp :type "PrimitiveComponent Object Reference") (OtherBodyIndex :type Integer) (bFromSweep :type Boolean) (SweepResult :type "HitResult Structure (by ref)"))
  (bind _as_bp_master_player (`self.As BP Master Player`))
  (if (`self.ActorHasTag` OtherActor "Player")
    (`/Game/BP/Character/Player/BP_MasterPlayer.ToggleInteractionInputVisibility` _as_bp_master_player)
    (set `/Game/BP/Character/Player/BP_MasterPlayer.triggerAltar` self _as_bp_master_player)))

(event `self.Sphere.OnComponentEndOverlap`
  (params (OverlappedComponent :type "PrimitiveComponent Object Reference") (OtherActor :type "Actor Object Reference") (OtherComp :type "PrimitiveComponent Object Reference") (OtherBodyIndex :type Integer))
  (bind _as_bp_master_player (`self.As BP Master Player`))
  (if (`self.ActorHasTag` OtherActor "Player")
    (`/Game/BP/Character/Player/BP_MasterPlayer.ToggleInteractionInputVisibility` _as_bp_master_player)
    (set `/Game/BP/Character/Player/BP_MasterPlayer.triggerAltar` null _as_bp_master_player)))

(fn `UserConstructionScript`
  (`SphereComponent.SetSphereRadius` (`self.Sphere`) (`self.TriggerRange`) true))