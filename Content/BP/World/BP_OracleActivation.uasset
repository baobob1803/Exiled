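; BP_OracleActivation is a world trigger that plays a one-time cinematic lighting the oracle's blue fires.
; On overlap it sets the game instance's OracleGraveUsed flag, switches to UI-only input and blends the view to itself.
; Timed delays then activate the BlueFireList Niagara effects, stop player movement, blend back and restore game input.
; On BeginPlay, a saved used state relights the fires and disables the trigger.
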(event `self.ReceiveBeginPlay`
  (`self.InitReferences`)
  (bind _value (message `/Game/BP/Interface/BPI_Save.GetOracleGraveUsed` (`self.BPIPlayerInstanceRef`)))
  (if _value
    (`self.BlueFireActivation`)
    (`PrimitiveComponent.SetCollisionEnabled` (`self.Trigger`) "NoCollision")))

(event `self.Trigger.OnComponentBeginOverlap`
  (params (OverlappedComponent :type "PrimitiveComponent Object Reference") (OtherActor :type "Actor Object Reference") (OtherComp :type "PrimitiveComponent Object Reference") (OtherBodyIndex :type Integer) (bFromSweep :type Boolean) (SweepResult :type "HitResult Structure (by ref)"))
  (`self.OracleActivated`))

(event `OracleActivated`
  (`/Engine/EditorBlueprintResources/StandardMacros.DoOnce` false
    (:`Completed`
      (set `/Game/BP/Data/BPI_PlayerInstance.oracleGraveUsed` true (`self.BPIPlayerInstanceRef`))
      (`WidgetBlueprintLibrary.SetInputMode_UIOnlyEx` (`GameplayStatics.GetPlayerController` 0) null)
      (`PlayerController.SetViewTargetWithBlend` (`self.PCWorldRef`) self 10.0 "VTBlend_Linear" 0.0 false)
      (`KismetSystemLibrary.Delay` 10.0)
      (`self.BlueFireActivation`)
      (`KismetSystemLibrary.Delay` 1.5)
      (`MovementComponent.StopMovementImmediately` (`Character.CharacterMovement` (`self.MasterPlayerRef`)))
      (`PlayerController.SetViewTargetWithBlend` (`self.PCWorldRef`) (`self.MasterPlayerRef`) 6.0 "VTBlend_Linear" 0.0 false)
      (`KismetSystemLibrary.Delay` 6.0)
      (`WidgetBlueprintLibrary.SetInputMode_GameOnly` (`GameplayStatics.GetPlayerController` 0)))))

(fn `BlueFireActivation`
  (for _array_element (`self.BlueFireList`)
    (`ActorComponent.Activate` (`NiagaraActor.NiagaraComponent` _array_element) false))
  (return))

(fn `InitReferences`
  (bind _returnvalue (`GameplayStatics.GetActorOfClass` "/Game/BP/Character/Player/BP_MasterPlayer.BP_MasterPlayer_C"))
  (set `self.MasterPlayerRef` _returnvalue)
  (bind _aspc_world (cast `/Game/BP/Data/World/PC_World` (`GameplayStatics.GetPlayerController` 0)))
  (set `self.PCWorldRef` _aspc_world)
  (bind _asbpi_player_instance (cast `/Game/BP/Data/BPI_PlayerInstance` (`GameplayStatics.GetGameInstance`)))
  (set `self.BPIPlayerInstanceRef` _asbpi_player_instance))

(fn `UserConstructionScript`)