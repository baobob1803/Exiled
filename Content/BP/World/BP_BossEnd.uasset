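; BP_BossEnd is a world trigger that plays a game-finish sequence when its Box is overlapped, with no filter on the overlapping actor.
; On overlap it switches input to UI only and blends PC_World's view target to itself over ten seconds.
; Timed delays then zero the BP_MasterPlayer walk speed and show WBP_GameFinish as the blend completes.
; A StopMovementImmediately call is present but never runs.
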(event `self.ReceiveBeginPlay`
  (bind _returnvalue (`GameplayStatics.GetActorOfClass` "/Game/BP/Character/Player/BP_MasterPlayer.BP_MasterPlayer_C"))
  (set `self.MasterPlayerRef` _returnvalue)
  (bind _aspc_world (cast `/Game/BP/Data/World/PC_World` (`GameplayStatics.GetPlayerController` 0)))
  (set `self.PcWorldRef` _aspc_world))

(event `self.Box.OnComponentBeginOverlap`
  (params (OverlappedComponent :type "PrimitiveComponent Object Reference") (OtherActor :type "Actor Object Reference") (OtherComp :type "PrimitiveComponent Object Reference") (OtherBodyIndex :type Integer) (bFromSweep :type Boolean) (SweepResult :type "HitResult Structure (by ref)"))
  (`WidgetBlueprintLibrary.SetInputMode_UIOnlyEx` (`GameplayStatics.GetPlayerController` 0) null)
  (`PlayerController.SetViewTargetWithBlend` (`self.PcWorldRef`) self 10.0 "VTBlend_Linear" 0.0 false)
  (`KismetSystemLibrary.Delay` 3.0)
  (set `CharacterMovementComponent.MaxWalkSpeed` 0.0 (`Character.CharacterMovement` (`self.MasterPlayerRef`)))
  (`KismetSystemLibrary.Delay` 7.0)
  (bind _returnvalue (`|CreateWidget` "/Game/BP/Widget/Cinematic/WBP_GameFinish.WBP_GameFinish_C"))
  (`UserWidget.AddToViewport` _returnvalue 0))

(fn `UserConstructionScript`)