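; BP_LevelManager is a level actor that registers key locations and save altars and handles ambient sound fades.
; Its construction script maps TargetPoints by object name, indexes each BP_SaveAltar by its array position, and caches the level name.
; On BeginPlay it fades the first AmbientSound found up from near silence, timed by the GameInstance's transition message or a default.
; VolumeTransition fades that sound to silence over a scaled caller-supplied duration.
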(event `self.ReceiveBeginPlay`
  (message `/Game/BP/Interface/BPI_Save.GetAltarIndex` (`GameplayStatics.GetGameInstance`))
  (bind _returnvalue (`GameplayStatics.GetActorOfClass` "/Script/Engine.AmbientSound"))
  (set `self.ambientSound` _returnvalue)
  (`AudioComponent.AdjustVolume` (`AmbientSound.AudioComponent` (`self.ambientSound`)) 0.0 0.01 "Linear")
  (bind (_value _time) (message `/Game/BP/Interface/BPI_Save.GetNeedTransition` (`GameplayStatics.GetGameInstance`)))
  (`AudioComponent.AdjustVolume` (`AmbientSound.AudioComponent` (`self.ambientSound`)) (* (select `bool` _value :`false` 3.0 :`true` _time) 1.75) 1.0 "SCurve"))

(event `VolumeTransition`
  (params (AdjustVolumeDuration :type "Float (double-precision)"))
  (`AudioComponent.AdjustVolume` (`AmbientSound.AudioComponent` (`self.ambientSound`)) (/ AdjustVolumeDuration 1.2) 0.0 "SCurve"))

(fn `UserConstructionScript`
  (bind _outactors (`GameplayStatics.GetAllActorsOfClass` "/Script/Engine.TargetPoint"))
  (for _array_element _outactors
    (`BlueprintMapLibrary.Map_Add` (`self.levelLocations`) (`KismetStringLibrary.Conv_StringToName` (`KismetSystemLibrary.GetObjectName` _array_element)) _array_element))
  (bind _outactors_2 (`GameplayStatics.GetAllActorsOfClass` "/Game/BP/World/BP_SaveAltar.BP_SaveAltar_C"))
  (for _array_element_2 _outactors_2
    (bind _returnvalue (`KismetArrayLibrary.Array_AddUnique` (`self.altarsStates`) _array_element_2))
    (set `/Game/BP/World/BP_SaveAltar.index` _returnvalue _array_element_2))
  (bind _returnvalue_2 (`GameplayStatics.GetCurrentLevelName` true))
  (set `self.LevelName` _returnvalue_2))