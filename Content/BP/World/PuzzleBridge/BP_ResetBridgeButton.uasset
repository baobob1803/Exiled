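; Interactable button that resets the parts of a bridge puzzle.
; On BeginPlay it runs the parent logic and appends its BridgesParts to the Bridge array.
; On Interaction, if the puzzle is not complete and CheckIfUsePlatformMoving returns false, it calls ResetActor on each bridge part.
; Puzzle completion is left to the parent class.
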(event `self.ReceiveBeginPlay`
  (`parent.ReceiveBeginPlay`)
  (`KismetArrayLibrary.Array_Append` (`self.Bridge`) (`self.BridgesParts`)))

(event `/Game/BP/Interface/BPI_Interaction.Interaction`
  (params (Player :type "/Game/BP/Character/Player/BP_MasterPlayer Object Reference") (displayUI :type Boolean))
  (if (not (`self.puzzleComplete`))
    (bind _value (`self.checkIfUsePlatformMoving`))
    (if (not _value)
      (for _array_element (`self.BridgesParts`)
        (`/Game/BP/World/PuzzleBridge/BP_BridgePart.ResetActor` _array_element)))))

(event `self.PuzzleFinish`
  (`parent.PuzzleFinish`))

(fn `UserConstructionScript`
  (`parent.UserConstructionScript`))