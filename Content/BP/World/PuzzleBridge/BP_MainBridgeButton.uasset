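; BP_MainBridgeButton is the interactable button for the bridge puzzle, linked to an array of Bridge pieces.
; Its Box overlap with components tagged "interact" registers or clears it as the player's TriggerButtonBridge and updates the HUD interaction prompt.
; CheckIfUsePlatformMoving reports whether any linked piece is moving.
; The press itself is not handled in this Blueprint.
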(event `self.ReceiveBeginPlay`
  (bind _returnvalue (`GameplayStatics.GetActorOfClass` "/Game/BP/Character/Player/BP_MasterPlayer.BP_MasterPlayer_C"))
  (set `self.player` _returnvalue))

(event `self.Box.OnComponentBeginOverlap`
  (params (OverlappedComponent :type "PrimitiveComponent Object Reference") (OtherActor :type "Actor Object Reference") (OtherComp :type "PrimitiveComponent Object Reference") (OtherBodyIndex :type Integer) (bFromSweep :type Boolean) (SweepResult :type "HitResult Structure (by ref)"))
  (bind _player (`self.player`))
  (if (`ActorComponent.ComponentHasTag` OtherComp "interact")
    (set `/Game/BP/Character/Player/BP_MasterPlayer.TriggerButtonBridge` self _player)
    (`/Game/BP/Widget/WBP_HUD.SetInteractionVisibility` (`/Game/BP/Character/Player/BP_MasterPlayer.HUD` _player))))

(event `self.Box.OnComponentEndOverlap`
  (params (OverlappedComponent :type "PrimitiveComponent Object Reference") (OtherActor :type "Actor Object Reference") (OtherComp :type "PrimitiveComponent Object Reference") (OtherBodyIndex :type Integer))
  (bind _player (`self.player`))
  (if (`ActorComponent.ComponentHasTag` OtherComp "interact")
    (set `/Game/BP/Character/Player/BP_MasterPlayer.triggerButtonBridge` null _player)
    (`/Game/BP/Widget/WBP_HUD.SetInteractionVisibility` (`/Game/BP/Character/Player/BP_MasterPlayer.HUD` _player))))

(fn `checkIfUsePlatformMoving`
  (returns (value :type Boolean))
  (locals (move :type Boolean))
  (for _array_element (`self.Bridge`)
    (if (`/Game/BP/World/PuzzleBridge/BP_BridgePart.isMoving` _array_element)
      (set `local.move` true)
      (break)))
  (if (`local.move`)
    (return true)
    (else
      (return false))))

(fn `UserConstructionScript`)