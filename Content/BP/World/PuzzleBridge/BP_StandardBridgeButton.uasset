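; Puzzle bridge button that, on interaction, raises and lowers its assigned bridge parts until the puzzle is complete.
; At BeginPlay it appends both part arrays to the inherited-style Bridge list.
; Interaction is blocked by CheckIfUsePlatformMoving, otherwise it calls MoveActor down on PartsGoDown, then up on PartsGoUp.
; Only the final part moved gets the LastPartMoving flag, falling back to the down list when nothing goes up.
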(event `self.ReceiveBeginPlay`
  (`parent.ReceiveBeginPlay`)
  (`KismetArrayLibrary.Array_Append` (`self.Bridge`) (`self.PartsGoUp`))
  (`KismetArrayLibrary.Array_Append` (`self.Bridge`) (`self.PartsGoDown`)))

(event `/Game/BP/Interface/BPI_Interaction.Interaction`
  (params (Player :type "/Game/BP/Character/Player/BP_MasterPlayer Object Reference") (displayUI :type Boolean))
  (bind _partsgodown (`self.PartsGoDown`))
  (bind _partsgoup (`self.PartsGoUp`))
  (if (not (`self.puzzleComplete`))
    (bind _value (`self.checkIfUsePlatformMoving`))
    (if (not _value)
      (for (_array_element _array_index) _partsgodown
        (`/Game/BP/World/PuzzleBridge/BP_BridgePart.MoveActor` _array_element true (and (`self.CheckIsTheLastPart` _array_index _partsgodown) (== (`KismetArrayLibrary.Array_Length` (`self.PartsGoUp`)) 0))))
      (for (_array_element_2 _array_index_2) _partsgoup
        (`/Game/BP/World/PuzzleBridge/BP_BridgePart.MoveActor` _array_element_2 false (`self.CheckIsTheLastPart` _array_index_2 _partsgoup))))))

(event `self.PuzzleFinish`
  (`parent.PuzzleFinish`))

(fn `CheckIsTheLastPart`
  (params (Index :type Integer) (TargetArray :type "Array of /Game/BP/World/PuzzleBridge/BP_BridgePart Object Reference (by ref)"))
  (returns (ReturnValue :type Boolean))
  (return (select `bool` (== Index (- (`KismetArrayLibrary.Array_Length` TargetArray) 1)) :`true` true)))

(fn `UserConstructionScript`
  (`parent.UserConstructionScript`))