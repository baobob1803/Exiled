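; BP_BridgeManager tracks a bridge puzzle built from bridge parts and buttons, and marks it finished when solved.
; CheckIfBridgeComplete requires every part to match one target position, then finishes buttons and parts and records completion on the GameInstance.
; BeginPlay reads that flag and, if set, restores the finished state after a short delay.
; Construction-script logic for gathering buttons and parts and linking them to the manager is disconnected.
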(event `self.ReceiveBeginPlay`
  (bind _value (message `/Game/BP/Interface/BPI_Save.GetBridgeComplete` (`GameplayStatics.GetGameInstance`)))
  (if _value
    (set `self.puzzleComplete` true)
    (`KismetSystemLibrary.Delay` 0.1)
    (for _array_element _
      (`/Game/BP/World/PuzzleBridge/BP_MainBridgeButton.PuzzleFinish` _array_element))
    (for _array_element_2 (`self.BridgeParts`)
      (`/Game/BP/World/PuzzleBridge/BP_BridgePart.BridgeFinish` _array_element_2))))

(event `CheckIfBridgeComplete`
  (set `self.puzzleComplete` true)
  (for _array_element (`self.BridgeParts`)
    (if (`|EnumInequality` (`/Game/BP/World/PuzzleBridge/BP_BridgePart.position` _array_element) "NewEnumerator1")
      (set `self.puzzleComplete` false)
      (break)))
  (if (`self.puzzleComplete`)
    (for _array_element_2 (`self.BridgeButtons`)
      (`/Game/BP/World/PuzzleBridge/BP_MainBridgeButton.PuzzleFinish` _array_element_2))
    (for _array_element_3 (`self.BridgeParts`)
      (`/Game/BP/World/PuzzleBridge/BP_BridgePart.BridgeFinish` _array_element_3))
    (message `/Game/BP/Interface/BPI_Save.SetBridgeComplete` (`GameplayStatics.GetGameInstance`) true)))

(fn `UserConstructionScript`)