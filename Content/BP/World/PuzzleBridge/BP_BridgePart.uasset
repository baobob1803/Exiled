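; A movable segment of the bridge puzzle that shifts vertically between Up, Neutral and Down positions.
; On BeginPlay it derives the three locations from its placed location, start position and a spacing distance.
; Timelines lerp it one step per move or back to its start on reset, and the last moving part asks BridgeManager to check completion.
; Finishing the puzzle snaps it to Neutral.
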(event `self.ReceiveBeginPlay`
  (bind _returnvalue (`self.K2_GetActorLocation`))
  (bind (_neutrallocation_x _neutrallocation_y _neutrallocation_z) (`KismetMathLibrary.BreakVector` (`self.neutralLocation`)))
  (set `self.position` (`self.startPosition`))
  (set `self.startLocation` (`self.K2_GetActorLocation`))
  (switch `/Game/BP/Enum/EBridgePosition` (`self.startPosition`)
    (:`NewEnumerator0`
      (bind _output_get (set `self.upLocation` _returnvalue))
      (bind _output_get_2 (set `self.neutralLocation` (`KismetMathLibrary.MakeVector` (.x _output_get) (.y _output_get) (- (.z _output_get) (`self.distanceBetweenLocation`)))))
      (set `self.downLocation` (`KismetMathLibrary.MakeVector` (.x _output_get_2) (.y _output_get_2) (- (.z _output_get_2) (`self.distanceBetweenLocation`)))))
    (:`NewEnumerator1`
      (bind _output_get_3 (set `self.neutralLocation` _returnvalue))
      (set `self.upLocation` (`KismetMathLibrary.MakeVector` (.x _output_get_3) (.y _output_get_3) (+ (.z _output_get_3) (`self.distanceBetweenLocation`))))
      (set `self.downLocation` (`KismetMathLibrary.MakeVector` _neutrallocation_x _neutrallocation_y (- _neutrallocation_z (`self.distanceBetweenLocation`)))))
    (:`NewEnumerator2`
      (bind _output_get_4 (set `self.downLocation` _returnvalue))
      (bind _output_get_5 (set `self.neutralLocation` (`KismetMathLibrary.MakeVector` (.x _output_get_4) (.y _output_get_4) (+ (.z _output_get_4) (`self.distanceBetweenLocation`)))))
      (set `self.upLocation` (`KismetMathLibrary.MakeVector` (.x _output_get_5) (.y _output_get_5) (+ (.z _output_get_5) (`self.distanceBetweenLocation`)))))))

(event `BridgeFinish`
  (set `self.puzzleComplete` true)
  (`self.K2_SetActorLocation` (`self.neutralLocation`))
  (set `self.position` "NewEnumerator1"))

(event `MoveActor`
  (params (goDown :type Boolean) (LastPartMoving :type Boolean))
  ;[0 1 0] Movement
  (set `self.Last Part Moving` LastPartMoving)
  (if (select `bool` goDown :`false` (`|EnumInequality` (`self.position`) "NewEnumerator0") :`true` (`|EnumInequality` (`self.position`) "NewEnumerator2"))
    (set `self.isMoving` true)
    (bind (_direction _lerp) (`Timeline|move` :!via `PlayFromStart`)
      (:`Update`
        (`self.K2_SetActorLocation` (`KismetMathLibrary.VLerp` (select `/Game/BP/Enum/EBridgePosition` (`self.position`) :`NewEnumerator0` (`self.upLocation`) :`NewEnumerator1` (`self.neutralLocation`) :`NewEnumerator2` (`self.downLocation`)) (select `/Game/BP/Enum/EBridgePosition` (`self.position`) :`NewEnumerator0` (`self.neutralLocation`) :`NewEnumerator1` (select `bool` goDown :`false` (`self.upLocation`) :`true` (`self.downLocation`)) :`NewEnumerator2` (`self.neutralLocation`)) _lerp)))
      (:`Finished`
        (set `self.position` (select `/Game/BP/Enum/EBridgePosition` (`self.position`) :`NewEnumerator0` "NewEnumerator1" :`NewEnumerator1` (select `bool` goDown :`false` "NewEnumerator0" :`true` "NewEnumerator2" :!type "/Game/BP/Enum/EBridgePosition Enum") :`NewEnumerator2` "NewEnumerator1"))
        (`|ExecutionSequence`
          (:`then_0`
            (if (`self.Last Part Moving`)
              (`/Game/BP/World/PuzzleBridge/BP_BridgeManager.CheckIfBridgeComplete` (`self.bridgeManager`))))
          (:`then_1`
            (set `self.isMoving` false)
            (set `self.Last Part Moving` false)))))))

(event `ResetActor`
  (if (`|EnumInequality` (`self.position`) (`self.startPosition`))
    (set `self.isMoving` true)
    (bind (_direction _lerp) (`Timeline|reset` :!via `PlayFromStart`)
      (:`Update`
        (`self.K2_SetActorLocation` (`KismetMathLibrary.VLerp` (select `/Game/BP/Enum/EBridgePosition` (`self.position`) :`NewEnumerator0` (`self.upLocation`) :`NewEnumerator1` (`self.neutralLocation`) :`NewEnumerator2` (`self.downLocation`)) (`self.startLocation`) _lerp)))
      (:`Finished`
        (set `self.position` (`self.startPosition`))
        (set `self.isMoving` false)))))

(fn `UserConstructionScript`)