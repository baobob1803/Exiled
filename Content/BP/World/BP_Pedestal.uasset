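; World pedestal that grants the player one of four masks (Matter, Mind, Creation or Void), selected by its Mask value.
; Box overlap registers it as the player's TriggerPedestal and toggles the interaction input display.
; Interaction adds the matching mask component, unlocks the mask, sets IsEmpty and disables the Box.
; IsEmpty persists through per-mask save flags, with an event bound to the game instance's save dispatcher on BeginPlay.
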(event `OnSave`
  (params (save :type "/Game/BP/Data/SG_Save Object Reference"))
  (bind _isempty (`self.isEmpty`))
  ;[1 1 1] Save
  (switch `/Game/BP/Enum/EMasks` (`self.Mask`)
    (:`NewEnumerator1`
      (set `/Game/BP/Data/SG_Save.haveMatter` _isempty save))
    (:`NewEnumerator2`
      (set `/Game/BP/Data/SG_Save.haveMind` _isempty save))
    (:`NewEnumerator3`
      (set `/Game/BP/Data/SG_Save.haveCreation` _isempty save))
    (:`NewEnumerator4`
      (set `/Game/BP/Data/SG_Save.haveVoid` _isempty save)))
  (`KismetSystemLibrary.PrintString` "Save Pedestal"))

(event `/Game/BP/Interface/BPI_Interaction.Interaction`
  (params (Player :type "/Game/BP/Character/Player/BP_MasterPlayer Object Reference"))
  (switch `/Game/BP/Enum/EMasks` (`self.Mask`)
    (:`NewEnumerator1`
      (bind _returnvalue (`AddComponent|NODE_AddAC_Mask_Matter-0` :`self` Player))
      (set `/Game/BP/Character/Player/BP_MasterPlayer.AC_MaskMatter` _returnvalue Player))
    (:`NewEnumerator2`
      (bind _returnvalue_2 (`AddComponent|NODE_AddAC_Mask_Mind-0` :`self` Player))
      (set `/Game/BP/Character/Player/BP_MasterPlayer.AC_MaskMind` _returnvalue_2 Player))
    (:`NewEnumerator3`
      (bind _returnvalue_3 (`AddComponent|NODE_AddAC_Mask_Creation-0` :`self` Player))
      (set `/Game/BP/Character/Player/BP_MasterPlayer.AC_MaskCreation` _returnvalue_3 Player))
    (:`NewEnumerator4`
      (bind _returnvalue_4 (`AddComponent|NODE_AddAC_Mask_Void-0` :`self` Player))
      (set `/Game/BP/Character/Player/BP_MasterPlayer.AC_MaskVoid` _returnvalue_4 Player)))
  (`/Game/BP/Character/Player/BP_MasterPlayer.UnlockMask` Player (`self.Mask`))
  (set `self.isEmpty` true)
  (`ActorComponent.SetActive` (`self.Box`) false false)
  (bind _as_bp_master_player (`self.As BP Master Player`)
    (:`then`
      (set `/Game/BP/Character/Player/BP_MasterPlayer.TriggerPedestal` null _as_bp_master_player)
      (`/Game/BP/Character/Player/BP_MasterPlayer.ToggleInteractionInputVisibility` _as_bp_master_player)
      (`PrimitiveComponent.SetCollisionEnabled` (`self.Box`) "NoCollision"))
    (:`else`)))

(event `self.ReceiveBeginPlay`
  ;[1 1 1] Comment
  (bind _asbpi_player_instance (cast `/Game/BP/Data/BPI_PlayerInstance` (`GameplayStatics.GetGameInstance`)))
  (add `/Game/BP/Data/BPI_PlayerInstance.ED_SaveGame` _asbpi_player_instance (`|CreateDelegate` :!event `OnSave`)))

(event `OnLoad`
  (params (NewParam :type "/Game/BP/Data/SG_Save Object Reference"))
  ;[1 1 1] Load
  (set `self.isEmpty` (select `/Game/BP/Enum/EMasks` (`self.Mask`) :`NewEnumerator1` (`/Game/BP/Data/SG_Save.haveMatter` NewParam) :`NewEnumerator2` (`/Game/BP/Data/SG_Save.haveMind` NewParam) :`NewEnumerator3` (`/Game/BP/Data/SG_Save.haveCreation` NewParam) :`NewEnumerator4` (`/Game/BP/Data/SG_Save.haveVoid` NewParam)))
  (if (not (`self.isEmpty`))
    (`ActorComponent.SetActive` (`self.Box`) false false)))

(event `self.Box.OnComponentBeginOverlap`
  (params (OverlappedComponent :type "PrimitiveComponent Object Reference") (OtherActor :type "Actor Object Reference") (OtherComp :type "PrimitiveComponent Object Reference") (OtherBodyIndex :type Integer) (bFromSweep :type Boolean) (SweepResult :type "HitResult Structure (by ref)"))
  (bind _as_bp_master_player (`self.As BP Master Player`)
    (:`then`
      (set `/Game/BP/Character/Player/BP_MasterPlayer.TriggerPedestal` self _as_bp_master_player)
      (`/Game/BP/Character/Player/BP_MasterPlayer.ToggleInteractionInputVisibility` _as_bp_master_player))
    (:`else`
      (bind _asbp_master_player (cast `/Game/BP/Character/Player/BP_MasterPlayer` OtherActor))
      (set `self.As BP Master Player` _asbp_master_player)
      (set `/Game/BP/Character/Player/BP_MasterPlayer.TriggerPedestal` self _asbp_master_player)
      (`/Game/BP/Character/Player/BP_MasterPlayer.ToggleInteractionInputVisibility` _asbp_master_player))))

(event `self.Box.OnComponentEndOverlap`
  (params (OverlappedComponent :type "PrimitiveComponent Object Reference") (OtherActor :type "Actor Object Reference") (OtherComp :type "PrimitiveComponent Object Reference") (OtherBodyIndex :type Integer))
  (bind _as_bp_master_player (`self.As BP Master Player`)
    (:`then`
      (set `/Game/BP/Character/Player/BP_MasterPlayer.TriggerPedestal` null _as_bp_master_player)
      (`/Game/BP/Character/Player/BP_MasterPlayer.ToggleInteractionInputVisibility` _as_bp_master_player))
    (:`else`)))

(fn `UserConstructionScript`)