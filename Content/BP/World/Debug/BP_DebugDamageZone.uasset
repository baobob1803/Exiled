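; Debug damage zone that periodically hits a player standing inside its box.
; Box overlap events store any actor tagged Player as the target and clear it when a Player-tagged actor leaves.
; A looping timer started at BeginPlay sends UpdateHealthMessage with AttackValue to the stored actor while it is valid, so hits follow the timer rather than the moment of entry.
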(event `self.ReceiveBeginPlay`
  (`KismetSystemLibrary.K2_SetTimerDelegate` (delegate `Attack`) 3.0 true))

(event `Attack`
  (bind _actor (`self.actor`)
    (:`then`
      (message `/Game/BP/Interface/BPI_Stats.UpdateHealth` _actor (`self.attackValue`)))
    (:`else`)))

(event `self.Box.OnComponentBeginOverlap`
  (params (OverlappedComponent :type "PrimitiveComponent Object Reference") (OtherActor :type "Actor Object Reference") (OtherComp :type "PrimitiveComponent Object Reference") (OtherBodyIndex :type Integer) (bFromSweep :type Boolean) (SweepResult :type "HitResult Structure (by ref)"))
  (for _array_element (`Actor.Tags` OtherActor)
    (if (== _array_element "Player")
      (set `self.actor` OtherActor)
      (break))))

(event `self.Box.OnComponentEndOverlap`
  (params (OverlappedComponent :type "PrimitiveComponent Object Reference") (OtherActor :type "Actor Object Reference") (OtherComp :type "PrimitiveComponent Object Reference") (OtherBodyIndex :type Integer))
  (for _array_element (`Actor.Tags` OtherActor)
    (if (== _array_element "Player")
      (set `self.actor` null)
      (break))))

(fn `UserConstructionScript`)