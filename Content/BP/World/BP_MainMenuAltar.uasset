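; Main menu altar actor that plays a charge-up effect when play begins.
; BeginPlay activates the NSStone effect and plays the Activate timeline, which drives the Offset material parameter on AltarCharge and the intensity of MidLight.
; The construction script sizes a Sphere component from TriggerRange, though no overlap logic uses it in these graphs.
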(event `self.ReceiveBeginPlay`
  (`ActorComponent.Activate` (`self.NS_Stone`) true)
  (bind (_direction _offset _light_int) (`Timeline|Activate`)
    (:`Update`
      (`MeshComponent.SetScalarParameterValueOnMaterials` (`self.AltarCharge`) "Offset" _offset)
      (`LightComponent.SetIntensity` (`self.MidLight`) _light_int))))

(fn `UserConstructionScript`
  (`SphereComponent.SetSphereRadius` (`self.Sphere`) (`self.TriggerRange`) true))