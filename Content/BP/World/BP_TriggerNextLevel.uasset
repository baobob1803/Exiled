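; BP_TriggerNextLevel is a world trigger that moves the player to another level.
; When a component tagged "interact" enters its Box, it calls LevelInteract on the cached BP_MasterPlayer and sends FogInMessage to all LevelScriptActors.
; Its Interaction event sets the player's transition walk speed and stores post-load transition data, including spawn location name, in the GameInstance.
; It then opens the configured level by name after a delay.
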(event `self.ReceiveBeginPlay`
  (bind _asbp_master_player (cast `/Game/BP/Character/Player/BP_MasterPlayer` (`GameplayStatics.GetPlayerPawn` 0)))
  (set `self.As BP Master Player` _asbp_master_player))

(event `self.Box.OnComponentBeginOverlap`
  (params (OverlappedComponent :type "PrimitiveComponent Object Reference") (OtherActor :type "Actor Object Reference") (OtherComp :type "PrimitiveComponent Object Reference") (OtherBodyIndex :type Integer) (bFromSweep :type Boolean) (SweepResult :type "HitResult Structure (by ref)"))
  (if (`ActorComponent.ComponentHasTag` OtherComp "interact")
    (`/Game/BP/Character/Player/BP_MasterPlayer.LevelInteract` (`self.As BP Master Player`) self (`self.K2_GetActorRotation`))
    ;[1 0.0401 0] Test Timeline Up Fog
    (bind _outactors (`GameplayStatics.GetAllActorsOfClass` "/Script/Engine.LevelScriptActor"))
    (for _array_element _outactors
      (message `/Game/BP/Interface/BPI_World.FogIn` _array_element))))

(event `self.Box.OnComponentEndOverlap`
  (params (OverlappedComponent :type "PrimitiveComponent Object Reference") (OtherActor :type "Actor Object Reference") (OtherComp :type "PrimitiveComponent Object Reference") (OtherBodyIndex :type Integer))
  (if (`ActorComponent.ComponentHasTag` OtherComp "interact")
    _))

(event `Open Level`)

(event `/Game/BP/Interface/BPI_Interaction.Interaction`
  (params (Player :type "/Game/BP/Character/Player/BP_MasterPlayer Object Reference"))
  (set `/Game/BP/Character/Player/BP_MasterPlayer.transitionWalkSpeed` (`self.walkSpeed`) Player)
  (message `/Game/BP/Interface/BPI_Save.SetNeedTransition` (`GameplayStatics.GetGameInstance`) true (`self.timeAfterLoad`) (`self.walkSpeed`) (`self.spawnLocationName`))
  (`KismetSystemLibrary.Delay` (`self.timeBeforeLoad`))
  (`GameplayStatics.OpenLevel` (`self.Level Name`)))

(fn `UserConstructionScript`)