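; Level actor that lights the fires and lights of the Oracle bridge, as named, when the player enters its trigger.
; On BeginPlay it reads the Oracle grave used-message flag through the game instance interface and sets the assigned Niagara fires and lights on or off to match.
; A player overlap with the trigger switches them all on once, without checking or writing that flag.
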(event `self.ReceiveBeginPlay`
  (bind _asbpi_player_instance (cast `/Game/BP/Data/BPI_PlayerInstance` (`GameplayStatics.GetGameInstance`)))
  (bind _value (message `/Game/BP/Interface/BPI_Save.GetOracleGraveUsed` _asbpi_player_instance))
  (if _value
    (for _array_element (`self.FiresToActivate`)
      (`ActorComponent.Activate` (`NiagaraActor.NiagaraComponent` _array_element) false))
    (for _array_element_2 (`self.LightToActivate`)
      (`LightComponent.SetIntensity` (`Light.LightComponent` _array_element_2) 22.0))
    (else
      (for _array_element_3 (`self.FiresToActivate`)
        (`ActorComponent.Deactivate` (`NiagaraActor.NiagaraComponent` _array_element_3)))
      (for _array_element_4 (`self.LightToActivate`)
        (`LightComponent.SetIntensity` (`Light.LightComponent` _array_element_4) 0.0)))))

(event `self.trigger.OnComponentBeginOverlap`
  (params (OverlappedComponent :type "PrimitiveComponent Object Reference") (OtherActor :type "Actor Object Reference") (OtherComp :type "PrimitiveComponent Object Reference") (OtherBodyIndex :type Integer) (bFromSweep :type Boolean) (SweepResult :type "HitResult Structure (by ref)"))
  (if (`KismetMathLibrary.ClassIsChildOf` (`GameplayStatics.GetObjectClass` OtherActor) "/Game/BP/Character/Player/BP_MasterPlayer.BP_MasterPlayer_C")
    (`/Engine/EditorBlueprintResources/StandardMacros.DoOnce` false
      (:`Completed`
        (for _array_element (`self.FiresToActivate`)
          (`ActorComponent.Activate` (`NiagaraActor.NiagaraComponent` _array_element) false))
        (for _array_element_2 (`self.LightToActivate`)
          (`LightComponent.SetIntensity` (`Light.LightComponent` _array_element_2) 22.0))))))

(fn `UserConstructionScript`)