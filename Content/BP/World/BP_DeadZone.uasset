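; BP_DeadZone is a world hazard volume that respawns the player on contact.
; On BeginPlay it caches the first BP_MasterPlayer and BP_SaveAltar found in the level.
; When an actor of exactly the BP_MasterPlayer class begins overlapping its Box, it calls Respawn on the cached player.
; An unconnected node would set the player's LastSavePoint to the cached altar, but it never runs.
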(event `self.ReceiveBeginPlay`
  (bind _returnvalue (`GameplayStatics.GetActorOfClass` "/Game/BP/Character/Player/BP_MasterPlayer.BP_MasterPlayer_C"))
  (set `self.PlayerRef` _returnvalue)
  (bind _returnvalue_2 (`GameplayStatics.GetActorOfClass` "/Game/BP/World/BP_SaveAltar.BP_SaveAltar_C"))
  (set `self.AltarRef` _returnvalue_2))

(event `self.Box.OnComponentBeginOverlap`
  (params (OverlappedComponent :type "PrimitiveComponent Object Reference") (OtherActor :type "Actor Object Reference") (OtherComp :type "PrimitiveComponent Object Reference") (OtherBodyIndex :type Integer) (bFromSweep :type Boolean) (SweepResult :type "HitResult Structure (by ref)"))
  ;[1 0.919 0.6759] Respawn if player hits
  (if (== (`GameplayStatics.GetObjectClass` OtherActor) "/Game/BP/Character/Player/BP_MasterPlayer.BP_MasterPlayer_C")
    (`/Game/BP/Character/Player/BP_MasterPlayer.Respawn` (`self.PlayerRef`))))

(fn `UserConstructionScript`)