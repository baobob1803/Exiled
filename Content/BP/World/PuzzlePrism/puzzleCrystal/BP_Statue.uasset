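; Puzzle statue that the player aims at its linked crystal as part of the prism crystal puzzle.
; Overlapping its box registers it with the player; interacting toggles a looping timer that turns it to face the player and sets its eye material from the crystal's color.
; Each tick traces toward the player; when the linked crystal blocks that line, the statue locks facing it and notifies BP_Prism.
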(event `self.ReceiveBeginPlay`
  (bind _returnvalue (`GameplayStatics.GetActorOfClass` "/Game/BP/Character/Player/BP_MasterPlayer.BP_MasterPlayer_C"))
  (set `self.Player` _returnvalue)
  (bind _returnvalue_2 (`GameplayStatics.GetActorOfClass` "/Game/BP/World/PuzzlePrism/BP_Prism.BP_Prism_C"))
  (set `self.Prism` _returnvalue_2)
  (set `self.Crystal Color` (`/Game/BP/World/PuzzlePrism/puzzleCrystal/BP_Crystal.CrystalColor` (`self.LinkCrystal`))))

(event `/Game/BP/Interface/BPI_Interaction.Interaction`
  (params (Player :type "/Game/BP/Character/Player/BP_MasterPlayer Object Reference") (displayUI :type Boolean))
  (bind _oeil__ (`self.oeil  `))
  (if (not (`self.Lock`))
    (`/Engine/EditorBlueprintResources/StandardMacros.FlipFlop`
      (:`A`
        (bind _returnvalue (`KismetSystemLibrary.K2_SetTimer` null "LookAtPlayer" 0.01 true))
        (set `self.TH_LookAt` _returnvalue)
        (switch `/Game/BP/Enum/E_Color` (`self.Crystal Color`)
          (:`NewEnumerator0`
            (`PrimitiveComponent.SetMaterial` _oeil__ 0 "/Game/BP/World/TestMaterials/M_AltarDesactivate.M_AltarDesactivate"))
          (:`NewEnumerator1`
            (`PrimitiveComponent.SetMaterial` _oeil__ 0 "/Game/BP/World/TestMaterials/M_AltarActivate.M_AltarActivate"))
          (:`NewEnumerator4`
            (`PrimitiveComponent.SetMaterial` _oeil__ 0 "/Game/BP/World/TestMaterials/M_IAPatrol.M_IAPatrol"))
          (:`NewEnumerator2`
            (`PrimitiveComponent.SetMaterial` _oeil__ 0 "/Game/BP/World/TestMaterials/M_IALookingAround.M_IALookingAround"))
          (:`NewEnumerator3`
            (`PrimitiveComponent.SetMaterial` _oeil__ 0 "/Game/BP/World/TestMaterials/MI_BaseColor_RespawnAltar.MI_BaseColor_RespawnAltar"))))
      (:`B`
        (`KismetSystemLibrary.K2_PauseTimerHandle` (`self.TH_LookAt`))))))

(event `self.Box.OnComponentBeginOverlap`
  (params (OverlappedComponent :type "PrimitiveComponent Object Reference") (OtherActor :type "Actor Object Reference") (OtherComp :type "PrimitiveComponent Object Reference") (OtherBodyIndex :type Integer) (bFromSweep :type Boolean) (SweepResult :type "HitResult Structure (by ref)"))
  (bind _player (`self.Player`))
  (if (`ActorComponent.ComponentHasTag` OtherComp "interact")
    (set `/Game/BP/Character/Player/BP_MasterPlayer.TriggerCrystalStatue` self _player)
    (`/Game/BP/Widget/WBP_HUD.SetInteractionVisibility` (`/Game/BP/Character/Player/BP_MasterPlayer.HUD` _player))))

(event `self.Box.OnComponentEndOverlap`
  (params (OverlappedComponent :type "PrimitiveComponent Object Reference") (OtherActor :type "Actor Object Reference") (OtherComp :type "PrimitiveComponent Object Reference") (OtherBodyIndex :type Integer))
  (bind _player (`self.Player`))
  (if (`ActorComponent.ComponentHasTag` OtherComp "interact")
    (set `/Game/BP/Character/Player/BP_MasterPlayer.TriggerCrystalStatue` null _player)
    (`/Game/BP/Widget/WBP_HUD.SetInteractionVisibility` (`/Game/BP/Character/Player/BP_MasterPlayer.HUD` _player))))

(fn `LockStatue`
  (set `self.Lock` true))

(fn `LookAtPlayer`
  (bind (_returnvalue_roll _returnvalue_pitch _returnvalue_yaw) (`KismetMathLibrary.BreakRotator` (`KismetMathLibrary.FindLookAtRotation` (`self.K2_GetActorLocation`) (`self.K2_GetActorLocation` (`self.LinkCrystal`)))))
  (bind (_returnvalue_roll_2 _returnvalue_pitch_2 _returnvalue_yaw_2) (`KismetMathLibrary.BreakRotator` (`KismetMathLibrary.FindLookAtRotation` (`self.K2_GetActorLocation`) (`self.K2_GetActorLocation` (`self.Player`)))))
  (`self.K2_SetActorRotation` (`KismetMathLibrary.MakeRotator` _returnvalue_roll_2 0.0 _returnvalue_yaw_2))
  (bind (_outhit _returnvalue) (`KismetSystemLibrary.LineTraceSingle` (`KismetMathLibrary.MakeVector` (.x (`self.K2_GetActorLocation`)) (.y (`self.K2_GetActorLocation`)) (+ (.z (`self.K2_GetActorLocation`)) 1.0)) (`self.K2_GetActorLocation` (`self.Player`)) "TraceTypeQuery2" false (`|MakeArray` self (`self.Player`) :!type "Actor Object Reference") "ForDuration"))
  (if _returnvalue
    (if (== (`.HitActor` (`GameplayStatics.BreakHitResult` _outhit)) (`self.LinkCrystal`))
      (`KismetSystemLibrary.K2_PauseTimerHandle` (`self.TH_LookAt`))
      (`self.LockStatue`)
      (`self.K2_SetActorRotation` (`KismetMathLibrary.MakeRotator` _returnvalue_roll 0.0 _returnvalue_yaw))
      (`/Game/BP/World/PuzzlePrism/BP_Prism.Resolve Cystal Puzzle1` (`self.Prism`) self))))

(fn `reset current statue color`
  (if (== (`self.currentStatueColorIndex`) 4)
    (set `self.currentStatueColorIndex` -1)))

(fn `UserConstructionScript`
  (set `self.Crystal Color` (`/Game/BP/World/PuzzlePrism/puzzleCrystal/BP_Crystal.CrystalColor` (`self.LinkCrystal`))))