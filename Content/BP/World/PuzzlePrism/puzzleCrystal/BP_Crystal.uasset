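; BP_Crystal is a colored crystal actor, filed under the prism puzzle assets.
; Its construction script switches on CrystalColor (red, green, blue, yellow or pink) and sets the first material slot of the Crystal component to match.
; The colors borrow existing altar and AI-state materials rather than crystal-specific ones.
; It has no runtime logic, as the event graph holds only disabled placeholder events.
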(fn `UserConstructionScript`
  (switch `/Game/BP/Enum/E_Color` (`self.CrystalColor`)
    (:`NewEnumerator0`
      (`PrimitiveComponent.SetMaterial` (`self.Crystal`) 0 "/Game/BP/World/TestMaterials/M_AltarDesactivate.M_AltarDesactivate"))
    (:`NewEnumerator1`
      (`PrimitiveComponent.SetMaterial` (`self.Crystal`) 0 "/Game/BP/World/TestMaterials/M_AltarActivate.M_AltarActivate"))
    (:`NewEnumerator4`
      (`PrimitiveComponent.SetMaterial` (`self.Crystal`) 0 "/Game/BP/World/TestMaterials/M_IAPatrol.M_IAPatrol"))
    (:`NewEnumerator2`
      (`PrimitiveComponent.SetMaterial` (`self.Crystal`) 0 "/Game/BP/World/TestMaterials/M_IALookingAround.M_IALookingAround"))
    (:`NewEnumerator3`
      (`PrimitiveComponent.SetMaterial` (`self.Crystal`) 0 "/Game/BP/World/TestMaterials/MI_BaseColor_RespawnAltar.MI_BaseColor_RespawnAltar"))))