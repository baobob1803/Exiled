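; BP_Symbol is a world actor in the prism puzzle's lantern set that displays a colored text symbol.
; Its construction script switches on the EColor variable and tints the TextRender component red, green or blue.
; The event graph holds only disabled default events, so the Blueprint adds no runtime logic.
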(fn `UserConstructionScript`
  (switch `/Game/BP/Enum/E_Color` (`self.E_Color`)
    (:`NewEnumerator0`
      (`TextRenderComponent.SetTextRenderColor` (`self.TextRender`) (make `Color` 0 0 255)))
    (:`NewEnumerator1`
      (`TextRenderComponent.SetTextRenderColor` (`self.TextRender`) (make `Color` 0 255)))
    (:`NewEnumerator4`
      (`TextRenderComponent.SetTextRenderColor` (`self.TextRender`) (make `Color` 255)))))