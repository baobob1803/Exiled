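; BP_Prism is the hub for a three-part world puzzle of bells, colored lanterns and idol statues with crystals, activating the prism once all three are solved.
; It gathers statues and lanterns at BeginPlay, tracks each in parallel completion arrays and locks them when solved.
; Bell input builds a string checked against a code, resetting on a wrong full-length entry.
; Completion swaps the prism material and saves to the GameInstance, which restores it on load.
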(event `self.ReceiveBeginPlay`
  (bind _outactors (`GameplayStatics.GetAllActorsOfClass` "/Game/BP/World/PuzzlePrism/puzzleCrystal/BP_Statue.BP_Statue_C"))
  (for _array_element _outactors
    (`KismetArrayLibrary.Array_Add` (`self.BP_Statues`) _array_element)
    (`KismetArrayLibrary.Array_Add` (`self.StatueComplete`)))
  (bind _outactors_2 (`GameplayStatics.GetAllActorsOfClass` "/Game/BP/World/PuzzlePrism/puzzleLantern/BP_Lantern.BP_Lantern_C"))
  (for _array_element_2 _outactors_2
    (`KismetArrayLibrary.Array_Add` (`self.BP_Lanterns`) _array_element_2)
    (`KismetArrayLibrary.Array_Add` (`self.LanternsComplete`)))
  (`KismetSystemLibrary.Delay` 0.2)
  (bind _value (message `/Game/BP/Interface/BPI_Save.GetPrismPuzzleComplete` (`GameplayStatics.GetGameInstance`)))
  (if _value
    (`self.CompletePuzzle` "NewEnumerator0")
    (`self.CompletePuzzle` "NewEnumerator1")
    (`self.CompletePuzzle` "NewEnumerator2")))

(event `self.CompletePuzzle`
  (params (Puzzle :type "/Game/BP/Enum/E_puzzle Enum" :default "NewEnumerator0"))
  (bind _color (make `Color` 0 255))
  (switch `/Game/BP/Enum/E_puzzle` Puzzle
    (:`NewEnumerator0`
      (`TextRenderComponent.SetTextRenderColor` (`self.Bells`) _color)
      (set `self.BellsPuzzleComplete` true))
    (:`NewEnumerator1`
      (`TextRenderComponent.SetTextRenderColor` (`self.Lantern`) _color)
      (set `self.LanternPuzzleComplete` true))
    (:`NewEnumerator2`
      (`TextRenderComponent.SetTextRenderColor` (`self.Crystal`) _color)
      (set `self.puzzleCrystalComplete` true)))
  (`self.CompletePrism`))

(event `self.Bell's code`
  (params (input :type Integer))
  (bind _output_get (set `self.currentBells code` (`KismetStringLibrary.Concat_StrStr` (`self.currentBells code`) (`KismetStringLibrary.Conv_IntToString` input))))
  (`KismetSystemLibrary.PrintString` _output_get)
  (if (`KismetStringLibrary.EqualEqual_StrStr` _output_get (`self.BellsCode`))
    (`KismetSystemLibrary.PrintString` "complete" true true (struct :`G` 1.0 :`B` 0.053216 :`A` 1.0))
    (`self.CompletePuzzle` "NewEnumerator0")
    (elif (== (`KismetStringLibrary.Len` (`self.currentBells code`)) (`KismetStringLibrary.Len` (`self.BellsCode`)))
      (`KismetSystemLibrary.PrintString` "False" true true (struct :`R` 1.0 :`B` 0.041492 :`A` 1.0))
      (`self.Reset Puzzle` "NewEnumerator0"))))

(event `self.Reset Puzzle`
  (params (Puzzle :type "/Game/BP/Enum/E_puzzle Enum" :default "NewEnumerator0"))
  (switch `/Game/BP/Enum/E_puzzle` Puzzle
    (:`NewEnumerator0`
      (set `self.currentBells code` "")
      (bind _outactors (`GameplayStatics.GetAllActorsOfClass` "/Game/BP/World/PuzzlePrism/puzzleBell/BP_Bells.BP_Bells_C"))
      (for _array_element _outactors
        (`/Game/BP/World/PuzzlePrism/puzzleBell/BP_Bells.reset` _array_element)))))

(fn `CompletePrism`
  (if (`self.LanternPuzzleComplete`)
    (if (`self.BellsPuzzleComplete`)
      (if (`self.puzzleCrystalComplete`)
        (`PrimitiveComponent.SetMaterial` (`self.Prisme`) 0 "/Game/BP/World/TestMaterials/M_AltarActivate.M_AltarActivate")
        (bind _output_get (set `self.PrismComplete` true))
        (message `/Game/BP/Interface/BPI_Save.SetPrismPuzzleComplete` (`GameplayStatics.GetGameInstance`) _output_get)))))

(fn `Resolve Cystal Puzzle`
  (params (Statue :type "/Game/BP/World/PuzzlePrism/puzzleCrystal/BP_Statue Object Reference"))
  (locals (L_Statue :type "/Game/BP/World/PuzzlePrism/puzzleCrystal/BP_Statue Object Reference"))
  (set `local.L_Statue` Statue)
  (for (_array_element _array_index) (`self.BP_Statues`)
    (if (== _array_element (`local.L_Statue`))
      (`KismetArrayLibrary.Array_Set` (`self.StatueComplete`) _array_index true)))
  (for _array_element_2 (`self.StatueComplete`)
    (`KismetSystemLibrary.PrintString` (`KismetStringLibrary.Conv_BoolToString` _array_element_2))
    (if _array_element_2
      (set `self.puzzleCrystalComplete` true)
      (else
        (set `self.puzzleCrystalComplete` false)
        (break))))
  (if (`self.puzzleCrystalComplete`)
    (for _array_element_3 (`self.BP_Statues`)
      (`/Game/BP/World/PuzzlePrism/puzzleCrystal/BP_Statue.LockStatue` _array_element_3))
    (`self.CompletePuzzle` "NewEnumerator2")))

(fn `Resolve Lantern Puzzle`
  (params (Lantern :type "/Game/BP/World/PuzzlePrism/puzzleLantern/BP_Lantern Object Reference"))
  (locals (L_Statue :type "/Game/BP/World/PuzzlePrism/puzzleCrystal/BP_Statue Object Reference") (L_Lantern :type "/Game/BP/World/PuzzlePrism/puzzleLantern/BP_Lantern Object Reference"))
  (bind _lanternscomplete (`self.LanternsComplete`))
  (bind _l_lantern (`local.L_Lantern`))
  (set `local.L_Lantern` Lantern)
  (for (_array_element _array_index) (`self.BP_Lanterns`)
    (if (== _array_element (`local.L_Lantern`))
      (if (`|EnumEquality` (`/Game/BP/World/PuzzlePrism/puzzleLantern/BP_Symbol.E_Color` (`/Game/BP/World/PuzzlePrism/puzzleLantern/BP_Lantern.LinkedSymbol` _l_lantern)) (`/Game/BP/World/PuzzlePrism/puzzleLantern/BP_Lantern.E_Color` _l_lantern))
        (`KismetArrayLibrary.Array_Set` _lanternscomplete _array_index true)
        (else
          (`KismetArrayLibrary.Array_Set` _lanternscomplete _array_index)))))
  (for _array_element_2 (`self.LanternsComplete`)
    (`KismetSystemLibrary.PrintString` (`KismetStringLibrary.Conv_BoolToString` _array_element_2))
    (if _array_element_2
      (set `self.LanternPuzzleComplete` true)
      (else
        (set `self.LanternPuzzleComplete` false)
        (break))))
  (if (`self.LanternPuzzleComplete`)
    (for _array_element_3 (`self.BP_Lanterns`)
      (`/Game/BP/World/PuzzlePrism/puzzleLantern/BP_Lantern.LockLantern` _array_element_3))
    (`self.CompletePuzzle` "NewEnumerator1")))

(fn `UserConstructionScript`)