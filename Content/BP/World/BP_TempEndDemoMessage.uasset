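; Temporary world trigger actor that shows an end-of-demo message while the player stands inside its box.
; On BeginPlay it creates a WBP_TempEndDemo widget, adds it to the viewport and keeps it hidden.
; Box overlap begin and end events toggle the widget's visibility, filtered to actors derived from BP_MasterPlayer.
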(event `self.ReceiveBeginPlay`
  (bind _returnvalue (`|CreateWidget` "/Game/BP/Widget/WBP_TempEndDemo.WBP_TempEndDemo_C"))
  (bind _output_get (set `self.WBP_EndDemoRef` _returnvalue))
  (`UserWidget.AddToViewport` _output_get 3)
  (`Widget.SetVisibility` _output_get "Hidden"))

(event `self.Box.OnComponentBeginOverlap`
  (params (OverlappedComponent :type "PrimitiveComponent Object Reference") (OtherActor :type "Actor Object Reference") (OtherComp :type "PrimitiveComponent Object Reference") (OtherBodyIndex :type Integer) (bFromSweep :type Boolean) (SweepResult :type "HitResult Structure (by ref)"))
  (if (`KismetMathLibrary.ClassIsChildOf` (`GameplayStatics.GetObjectClass` OtherActor) "/Game/BP/Character/Player/BP_MasterPlayer.BP_MasterPlayer_C")
    (`Widget.SetVisibility` (`self.WBP_EndDemoRef`) "Visible")))

(event `self.Box.OnComponentEndOverlap`
  (params (OverlappedComponent :type "PrimitiveComponent Object Reference") (OtherActor :type "Actor Object Reference") (OtherComp :type "PrimitiveComponent Object Reference") (OtherBodyIndex :type Integer))
  (if (`KismetMathLibrary.ClassIsChildOf` (`GameplayStatics.GetObjectClass` OtherActor) "/Game/BP/Character/Player/BP_MasterPlayer.BP_MasterPlayer_C")
    (`Widget.SetVisibility` (`self.WBP_EndDemoRef`) "Hidden")))

(fn `UserConstructionScript`)