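; BP_Rune is a rune in the oracle puzzle, identified by a data table row handle.
; The construction script and UpdateMaterial apply that row's texture material to its cube, while getters expose the handle, key name and empty flag.
; SetRuneInfo only stores a new handle without refreshing the material, whereas ResetRuneInfo switches to the "Nothing" row of BDD_PuzzleRunes and updates the visual.
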(event `self.UpdateMaterial`
  (bind (_datatable _rowname) (break `DataTableRowHandle` (`self.RuneInfo`)))
  (bind _returnvalue (`|GetDataTableRow` _datatable _rowname)
    (:`then`
      (`PrimitiveComponent.SetMaterial` (`self.Cube`) 0 (`.Texture_6_76A06D70413A24439496E8AAD9970F32` (break `/Game/BP/Structure/ST_PuzzleRuneInfo` _returnvalue))))))

(event `self.SetRuneInfo`
  (params (RuneInfo :type "DataTableRowHandle Structure"))
  (set `self.RuneInfo` RuneInfo))

(event `self.ResetRuneInfo`
  (`KismetSystemLibrary.PrintString` "Reset")
  (set `self.RuneInfo` (make `DataTableRowHandle` "/Game/BP/BDD/BDD_PuzzleRunes.BDD_PuzzleRunes" "Nothing"))
  (`self.UpdateMaterial`))

(fn `GetIsEmpty`
  (returns (isEmpty :type Boolean))
  (bind (_datatable _rowname) (break `DataTableRowHandle` (`self.RuneInfo`)))
  (bind _returnvalue (`|GetDataTableRow` _datatable _rowname)
    (:`then`
      (return (`.isEmpty_8_5D362692484F57B5A0D0B4B8E70DCEB1` (break `/Game/BP/Structure/ST_PuzzleRuneInfo` _returnvalue))))))

(fn `GetKey`
  (returns (key :type Name))
  (bind (_datatable _rowname) (break `DataTableRowHandle` (`self.RuneInfo`)))
  (bind _returnvalue (`|GetDataTableRow` _datatable _rowname)
    (:`then`
      (return (`.Name_2_44D87AA84925D95D5CD72D9439F1E008` (break `/Game/BP/Structure/ST_PuzzleRuneInfo` _returnvalue))))))

(fn `GetRuneInfo`
  (returns (RuneInfo :type "DataTableRowHandle Structure"))
  (return (`self.RuneInfo`)))

(fn `UserConstructionScript`
  (`self.UpdateMaterial`))