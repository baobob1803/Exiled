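; BP_OracleDoor is a double door for the Oracle puzzle that swings open when its OpenIt event is called.
; It records both leaf rotations at BeginPlay, then an Open timeline lerps each leaf's world yaw 90 degrees in opposite directions from that start.
; When the timeline finishes, it sets IsOpen; the file shows no closing logic.
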(event `self.ReceiveBeginPlay`
  (set `self.LeftDoorStartRotation` (`SceneComponent.K2_GetComponentRotation` (`self.DoorLeft_Scene`)))
  (set `self.RightDoorStartRotation` (`SceneComponent.K2_GetComponentRotation` (`self.DoorRightScene`))))

(event `OpenIt`
  (bind (_leftdoorstartrotation_roll _leftdoorstartrotation_pitch _leftdoorstartrotation_yaw) (`KismetMathLibrary.BreakRotator` (`self.LeftDoorStartRotation`)))
  (bind (_rightdoorstartrotation_roll _rightdoorstartrotation_pitch _rightdoorstartrotation_yaw) (`KismetMathLibrary.BreakRotator` (`self.RightDoorStartRotation`)))
  (bind (_direction _0_1) (`Timeline|Open`)
    (:`Update`
      (`SceneComponent.K2_SetWorldRotation` (`self.DoorLeft_Scene`) (`KismetMathLibrary.RLerp` (`self.LeftDoorStartRotation`) (`KismetMathLibrary.MakeRotator` _leftdoorstartrotation_roll _leftdoorstartrotation_pitch (+ _leftdoorstartrotation_yaw 90.0)) _0_1) false false)
      (`SceneComponent.K2_SetWorldRotation` (`self.DoorRightScene`) (`KismetMathLibrary.RLerp` (`self.RightDoorStartRotation`) (`KismetMathLibrary.MakeRotator` _rightdoorstartrotation_roll _rightdoorstartrotation_pitch (+ _rightdoorstartrotation_yaw -90.0)) _0_1) false false))
    (:`Finished`
      (set `self.isOpen` true))))

(fn `UserConstructionScript`)