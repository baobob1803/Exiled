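; World actor for a rune-code puzzle that opens a door when four slots hold the wanted combination.
; Interaction blends a spawned camera to the puzzle view and possesses PawnPuzzle, reversing on exit.
; Slot overlaps set the pawn's target, while UpdateKey joins slot keys, opening the door on a match or restoring runes via a key map when full but wrong.
; A GameInstance flag disables interaction at BeginPlay.
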(event `self.ReceiveBeginPlay`
  (bind _returnvalue (`GameplayStatics.GetActorOfClass` "/Game/BP/Character/Player/BP_MasterPlayer.BP_MasterPlayer_C"))
  (set `self.player` _returnvalue)
  (set `/Game/BP/Character/Player/BP_PlayerPuzzle.RunicReceptacle` self (`self.PawnPuzzle`))
  (`self.AddRuneToDict` (`self.Rune_a`))
  (`self.AddRuneToDict` (`self.Rune_b`))
  (`self.AddRuneToDict` (`self.Rune_c`))
  (`self.AddRuneToDict` (`self.Rune_d`))
  (`self.AddRuneToDict` (`self.Rune_e`))
  (`self.AddRuneToDict` (`self.Rune_f`))
  (`self.AddRuneToDict` (`self.Rune_g`))
  (`self.AddRuneToDict` (`self.Rune_h`))
  (`self.AddRuneToDict` (`self.Rune_i`))
  (`self.AddRuneToDict` (`self.Rune_j`))
  (`self.AddRuneToDict` (`self.Rune_k`))
  (`self.AddRuneToDict` (`self.Rune_l`))
  (bind _value (message `/Game/BP/Interface/BPI_Save.GetOracleGraveUsed` (`GameplayStatics.GetGameInstance`)))
  (if _value
    (`PrimitiveComponent.SetCollisionEnabled` (`self.Box`) "NoCollision")))

(event `/Game/BP/Interface/BPI_Interaction.Interaction`
  (params (Player :type "/Game/BP/Character/Player/BP_MasterPlayer Object Reference") (displayUI :type Boolean))
  (bind _returnvalue (`|SpawnActorFromClass` "/Script/Engine.CameraActor" (`SceneComponent.K2_GetComponentToWorld` (`/Game/BP/Character/Player/BP_MasterPlayer.Camera` (`self.player`))) "Undefined" "OverrideRootScale" null null))
  (set `self.Cam` _returnvalue)
  (`PlayerController.SetViewTargetWithBlend` (`GameplayStatics.GetPlayerController` 0) _returnvalue 0.0 "VTBlend_Linear" 0.0 false)
  (`self.GoToPuzzle`))

(event `GoToPuzzle`
  (bind _returnvalue (`GameplayStatics.GetPlayerController` 0))
  (`/Engine/EditorBlueprintResources/StandardMacros.DoOnce` false :!label _label
    (:`Completed`
      (`/Game/BP/Widget/WBP_HUD.SetInteractionVisibility` (`/Game/BP/Character/Player/BP_MasterPlayer.HUD` (`self.player`)))
      (bind (_direction _0_1) (`Timeline|CamTransition` :!label _label_2)
        (:`Update`
          (`SceneComponent.K2_SetWorldTransform` (`CameraActor.SceneComponent` (`self.Cam`)) (`KismetMathLibrary.TLerp` (`SceneComponent.K2_GetComponentToWorld` (`/Game/BP/Character/Player/BP_MasterPlayer.Camera` (`self.player`))) (`SceneComponent.K2_GetComponentToWorld` (`/Game/BP/Character/Player/BP_PlayerPuzzle.Camera` (`self.PawnPuzzle`))) _0_1) false false))
        (:`Finished`
          (`Controller.Possess` (`GameplayStatics.GetPlayerController` 0) (select `bool` (`self.inChara`) :`false` (`self.player`) :`true` (`self.PawnPuzzle`) :!type "Pawn Object Reference"))
          (set `self.inChara` (select `bool` (`self.inChara`) :`false` true))
          (if (`self.inChara`)
            (`self.K2_DestroyActor` (`self.Cam`))
            (`WidgetBlueprintLibrary.SetInputMode_GameOnly` _returnvalue)
            (set `PlayerController.bShowMouseCursor` false (`GameplayStatics.GetPlayerController` 0))
            (`/Game/BP/Widget/WBP_HUD.SetInteractionVisibility` (`/Game/BP/Character/Player/BP_MasterPlayer.HUD` (`self.player`)))
            (goto _label :!via `Reset`)
            (else
              (`WidgetBlueprintLibrary.SetInputMode_GameAndUIEx` _returnvalue null "DoNotLock" false)
              (set `PlayerController.bShowMouseCursor` true (`GameplayStatics.GetPlayerController` 0))
              (goto _label_3 :!via `Reset`))))))))

(event `self.Box.OnComponentBeginOverlap`
  (params (OverlappedComponent :type "PrimitiveComponent Object Reference") (OtherActor :type "Actor Object Reference") (OtherComp :type "PrimitiveComponent Object Reference") (OtherBodyIndex :type Integer) (bFromSweep :type Boolean) (SweepResult :type "HitResult Structure (by ref)"))
  (bind _player (`self.player`))
  (if (`ActorComponent.ComponentHasTag` OtherComp "interact")
    (set `/Game/BP/Character/Player/BP_MasterPlayer.triggerRunicReceptacle` self _player)
    (`/Game/BP/Widget/WBP_HUD.SetInteractionVisibility` (`/Game/BP/Character/Player/BP_MasterPlayer.HUD` _player))))

(event `ReturnToChara`
  (`/Engine/EditorBlueprintResources/StandardMacros.DoOnce` true :!label _label_3
    (:`Completed`
      (`PlayerController.SetViewTargetWithBlend` (`GameplayStatics.GetPlayerController` 0) (`self.Cam`) 0.0 "VTBlend_Linear" 0.0 false)
      (goto _label_2 :!via `ReverseFromEnd`))))

(event `self.Box.OnComponentEndOverlap`
  (params (OverlappedComponent :type "PrimitiveComponent Object Reference") (OtherActor :type "Actor Object Reference") (OtherComp :type "PrimitiveComponent Object Reference") (OtherBodyIndex :type Integer))
  (bind _player (`self.player`))
  (if (`ActorComponent.ComponentHasTag` OtherComp "interact")
    (set `/Game/BP/Character/Player/BP_MasterPlayer.triggerRunicReceptacle` null _player)
    (`/Game/BP/Widget/WBP_HUD.SetInteractionVisibility` (`/Game/BP/Character/Player/BP_MasterPlayer.HUD` _player))))

(event `self.RuneSlotBox.OnComponentBeginOverlap`
  (params (OverlappedComponent :type "PrimitiveComponent Object Reference") (OtherActor :type "Actor Object Reference") (OtherComp :type "PrimitiveComponent Object Reference") (OtherBodyIndex :type Integer) (bFromSweep :type Boolean) (SweepResult :type "HitResult Structure (by ref)"))
  (`self.PlaceRuneInSlot` OtherActor (`self.RuneSlotA`)))

(event `self.RuneSlotBox.OnComponentEndOverlap`
  (params (OverlappedComponent :type "PrimitiveComponent Object Reference") (OtherActor :type "Actor Object Reference") (OtherComp :type "PrimitiveComponent Object Reference") (OtherBodyIndex :type Integer))
  (`self.CancelPlacement` OtherActor (`self.RuneSlotA`)))

(event `self.RuneSlotBox1.OnComponentBeginOverlap`
  (params (OverlappedComponent :type "PrimitiveComponent Object Reference") (OtherActor :type "Actor Object Reference") (OtherComp :type "PrimitiveComponent Object Reference") (OtherBodyIndex :type Integer) (bFromSweep :type Boolean) (SweepResult :type "HitResult Structure (by ref)"))
  (`self.PlaceRuneInSlot` OtherActor (`self.RuneSlotB`)))

(event `self.RuneSlotBox1.OnComponentEndOverlap`
  (params (OverlappedComponent :type "PrimitiveComponent Object Reference") (OtherActor :type "Actor Object Reference") (OtherComp :type "PrimitiveComponent Object Reference") (OtherBodyIndex :type Integer))
  (`self.CancelPlacement` OtherActor (`self.RuneSlotB`)))

(event `self.RuneSlotBox2.OnComponentBeginOverlap`
  (params (OverlappedComponent :type "PrimitiveComponent Object Reference") (OtherActor :type "Actor Object Reference") (OtherComp :type "PrimitiveComponent Object Reference") (OtherBodyIndex :type Integer) (bFromSweep :type Boolean) (SweepResult :type "HitResult Structure (by ref)"))
  (`self.PlaceRuneInSlot` OtherActor (`self.RuneSlotC`)))

(event `self.RuneSlotBox2.OnComponentEndOverlap`
  (params (OverlappedComponent :type "PrimitiveComponent Object Reference") (OtherActor :type "Actor Object Reference") (OtherComp :type "PrimitiveComponent Object Reference") (OtherBodyIndex :type Integer))
  (`self.CancelPlacement` OtherActor (`self.RuneSlotC`)))

(event `self.RuneSlotBox3.OnComponentBeginOverlap`
  (params (OverlappedComponent :type "PrimitiveComponent Object Reference") (OtherActor :type "Actor Object Reference") (OtherComp :type "PrimitiveComponent Object Reference") (OtherBodyIndex :type Integer) (bFromSweep :type Boolean) (SweepResult :type "HitResult Structure (by ref)"))
  (`self.PlaceRuneInSlot` OtherActor (`self.RuneSlotD`)))

(event `self.RuneSlotBox3.OnComponentEndOverlap`
  (params (OverlappedComponent :type "PrimitiveComponent Object Reference") (OtherActor :type "Actor Object Reference") (OtherComp :type "PrimitiveComponent Object Reference") (OtherBodyIndex :type Integer))
  (`self.CancelPlacement` OtherActor (`self.RuneSlotD`)))

(fn `AddRuneToDict`
  (params (Rune :type "ChildActorComponent Object Reference (by ref)"))
  (bind _key (message `/Game/BP/Interface/BPI_PuzzleRune.GetKey` (`ChildActorComponent.ChildActor` Rune)))
  (`BlueprintMapLibrary.Map_Add` (`self.Runes`) _key Rune))

(fn `CancelPlacement`
  (params (OtherActor :type "Actor Object Reference") (RuneSlot :type "Object Object Reference"))
  (if (and (`self.ActorHasTag` OtherActor "Rune") (== (`/Game/BP/Character/Player/BP_PlayerPuzzle.targetChildActor` (`self.PawnPuzzle`)) RuneSlot))
    (set `/Game/BP/Character/Player/BP_PlayerPuzzle.targetChildActor` null (`self.PawnPuzzle`))
    (else
      (`KismetSystemLibrary.PrintString` "J'suis parti"))))

(fn `PlaceRuneInSlot`
  (params (otherActor :type "Actor Object Reference") (runeSlot :type "ChildActorComponent Object Reference"))
  (if (`self.ActorHasTag` otherActor "Rune")
    (`KismetSystemLibrary.PrintString` "Hello")
    (set `/Game/BP/Character/Player/BP_PlayerPuzzle.targetChildActor` runeSlot (`self.PawnPuzzle`))))

(fn `SetRuneVisibility`
  (params (Key :type "Name (by ref)") (NewHidden :type Boolean :default false) (bNewActorEnableCollision :type Boolean))
  (bind (_value _returnvalue) (`BlueprintMapLibrary.Map_Find` (`self.Runes`) Key))
  (if _returnvalue
    (`self.SetActorEnableCollision` (`ChildActorComponent.ChildActor` _value) bNewActorEnableCollision)
    (`SceneComponent.SetHiddenInGame` _value NewHidden false)
    (else
      (`KismetSystemLibrary.PrintString` "NOt  FInd"))))

(fn `UpdateKey`
  (locals (slotA :type Boolean :default false) (slotB :type Boolean :default false) (slotC :type Boolean :default false) (slotD :type Boolean :default false))
  (bind _returnvalue (`GameplayStatics.GetPlayerController` 0))
  (bind _key (message `/Game/BP/Interface/BPI_PuzzleRune.GetKey` (`ChildActorComponent.ChildActor` (`self.RuneSlotA`))))
  (set `self.slotKeyA` _key)
  (bind _key_2 (message `/Game/BP/Interface/BPI_PuzzleRune.GetKey` (`ChildActorComponent.ChildActor` (`self.RuneSlotB`))))
  (set `self.slotKeyB` _key_2)
  (bind _key_3 (message `/Game/BP/Interface/BPI_PuzzleRune.GetKey` (`ChildActorComponent.ChildActor` (`self.RuneSlotC`))))
  (set `self.slotKeyC` _key_3)
  (bind _key_4 (message `/Game/BP/Interface/BPI_PuzzleRune.GetKey` (`ChildActorComponent.ChildActor` (`self.RuneSlotD`))))
  (set `self.slotKeyD` _key_4)
  (bind _output_get (set `self.actualKey` (`KismetStringLibrary.Conv_StringToName` (`KismetStringLibrary.Concat_StrStr` (`KismetStringLibrary.Conv_NameToString` (`self.slotKeyA`)) (`KismetStringLibrary.Conv_NameToString` (`self.slotKeyB`)) (`KismetStringLibrary.Conv_NameToString` (`self.slotKeyC`)) (`KismetStringLibrary.Conv_NameToString` (`self.slotKeyD`))))))
  (if (== _output_get (`self.wantedKey`))
    (`KismetSystemLibrary.PrintString` "You win!!!!")
    (`/Game/BP/World/PuzzleOracle/BP_OracleDoor.OpenIt` (`self.Door`))
    (`Controller.Possess` (`GameplayStatics.GetPlayerController` 0) (`self.player`))
    (`PrimitiveComponent.SetCollisionEnabled` (`self.Box`) "NoCollision")
    (`WidgetBlueprintLibrary.SetInputMode_GameOnly` _returnvalue)
    (set `PlayerController.bShowMouseCursor` false _returnvalue)
    (`/Game/BP/Widget/WBP_HUD.SetInteractionVisibility` (`/Game/BP/Character/Player/BP_MasterPlayer.HUD` (`self.player`)))
    (`PrimitiveComponent.SetCollisionEnabled` (`self.Box`) "NoCollision")
    (else
      (bind _isempty (message `/Game/BP/Interface/BPI_PuzzleRune.GetIsEmpty` (`ChildActorComponent.ChildActor` (`self.RuneSlotA`))))
      (set `local.slotA` _isempty)
      (bind _isempty_2 (message `/Game/BP/Interface/BPI_PuzzleRune.GetIsEmpty` (`ChildActorComponent.ChildActor` (`self.RuneSlotB`))))
      (set `local.slotB` _isempty_2)
      (bind _isempty_3 (message `/Game/BP/Interface/BPI_PuzzleRune.GetIsEmpty` (`ChildActorComponent.ChildActor` (`self.RuneSlotC`))))
      (set `local.slotC` _isempty_3)
      (bind _isempty_4 (message `/Game/BP/Interface/BPI_PuzzleRune.GetIsEmpty` (`ChildActorComponent.ChildActor` (`self.RuneSlotD`))))
      (set `local.slotD` _isempty_4)
      (if (or (`local.slotA`) (`local.slotB`) (`local.slotC`) (`local.slotD`))
        (`KismetSystemLibrary.PrintString` (`KismetStringLibrary.Conv_NameToString` _output_get))
        (else
          (`KismetSystemLibrary.PrintString` "Wrong code!!")
          (`self.SetRuneVisibility` (`self.slotKeyA`) false true)
          (message `/Game/BP/Interface/BPI_PuzzleRune.ResetRuneInfo` (`ChildActorComponent.ChildActor` (`self.RuneSlotA`)))
          (`self.SetRuneVisibility` (`self.slotKeyB`) false true)
          (message `/Game/BP/Interface/BPI_PuzzleRune.ResetRuneInfo` (`ChildActorComponent.ChildActor` (`self.RuneSlotB`)))
          (`self.SetRuneVisibility` (`self.slotKeyC`) false true)
          (message `/Game/BP/Interface/BPI_PuzzleRune.ResetRuneInfo` (`ChildActorComponent.ChildActor` (`self.RuneSlotC`)))
          (`self.SetRuneVisibility` (`self.slotKeyD`) false true)
          (message `/Game/BP/Interface/BPI_PuzzleRune.ResetRuneInfo` (`ChildActorComponent.ChildActor` (`self.RuneSlotD`))))))))

(fn `UserConstructionScript`)