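; BP_EndIntroSetup is a view-target actor that plays the closing camera move of the intro cinematic, gated by the GameInstance's ShowCinematicMessage flag.
; On BeginPlay it takes over the PC_World camera with UI-only input and waits about 30 seconds.
; Two chained timelines then slide it along negative world X and rotate it to zero rotation.
; Finally it returns view and game input to BP_MasterPlayer, shows the HUD and clears the flag.
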(event `self.ReceiveBeginPlay`
  (bind _value (message `/Game/BP/Interface/BPI_Save.GetShowCinematic` (`GameplayStatics.GetGameInstance`)))
  (if _value
    (bind _returnvalue (`GameplayStatics.GetActorOfClass` "/Game/BP/Character/Player/BP_MasterPlayer.BP_MasterPlayer_C"))
    (set `self.Player` _returnvalue)
    (bind _aspc_world (cast `/Game/BP/Data/World/PC_World` (`GameplayStatics.GetPlayerController` 0)))
    (bind _output_get (set `self.As PC World` _aspc_world))
    (`/Game/BP/Data/World/PC_World.Switch Camera` _output_get true self)
    (`WidgetBlueprintLibrary.SetInputMode_UIOnlyEx` (`self.As PC World`) null)
    (`KismetSystemLibrary.Delay` 30.33)
    (`self.Start`)))

(event `Start`
  (bind (_initial_pos_location _initial_pos_rotation) (`KismetMathLibrary.BreakTransform` (`self.initial pos`)))
  (bind _initial_pos_location_2 (`KismetMathLibrary.BreakTransform` (`self.initial pos`)))
  (bind _player (`self.Player`))
  (set `self.initial pos` (`self.GetTransform`))
  (bind (_direction _value) (`Timeline|Timeline_0` :!via `PlayFromStart`)
    (:`Update`
      (`self.K2_SetActorLocation` (`KismetMathLibrary.VLerp` _initial_pos_location_2 (+ _initial_pos_location_2 (-600.0 0.0 0.0)) _value)))
    (:`Finished`
      (bind (_direction_2 _value_2) (`Timeline|Timeline_1` :!via `PlayFromStart`)
        (:`Update`
          (`self.K2_SetActorRotation` (`KismetMathLibrary.RLerp` _initial_pos_rotation (struct) _value_2)))
        (:`Finished`
          (`/Game/BP/Data/World/PC_World.Switch Camera` (`self.As PC World`) true _player)
          (`WidgetBlueprintLibrary.SetInputMode_GameOnly` (`self.As PC World`))
          (`Widget.SetVisibility` (`/Game/BP/Character/Player/BP_MasterPlayer.HUD` _player) "Visible")
          (message `/Game/BP/Interface/BPI_Save.SetShowCinematic` (`GameplayStatics.GetGameInstance`) false))))))

(fn `UserConstructionScript`)