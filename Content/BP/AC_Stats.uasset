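; Stats component that holds a Stats struct and changes individual values, such as health, poise and movement speeds, by enum.
; StatsBehaviour switches on the enum into UpdateStats, forwarding Value only for Health.
; Health and Poise add a clamped delta, while Walk Speed and Sprint Multiplier overwrite, then re-enter StatsBehaviour to recompute sprint speed as their product.
; Block is routed but has no update logic.
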(fn `StatsBehaviour`
  (params (statsEnum :type "/Game/BP/EStats Enum" :default "NewEnumerator0") (Value :type "Float (double-precision)"))
  (switch `/Game/BP/EStats` statsEnum
    (:`NewEnumerator0`
      (`self.UpdateStats` Value :!label _label))
    (:`NewEnumerator1`
      (goto _label :!via `Block`))
    (:`NewEnumerator2`
      (goto _label :!via `Poise`))
    (:`NewEnumerator3`
      (goto _label :!via `Speed`))
    (:`NewEnumerator4`
      (goto _label :!via `SprintMultiplier`))
    (:`NewEnumerator5`
      (goto _label :!via `SpeedSprint`))))